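; Battle actor that tracks an ongoing fight between players and plays its looping battle music.
; AddUnitToBattle records players, keeps each team's last four unit locations and flags that team as active.
; A repeating timer clears those flags, fading music when none were set and destroying the actor after consecutive idle checks.
; Centroid-based arrow placement and battle notifications exist only in disconnected, never-run logic.
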(event Custom|AddUnitToBattle
  (params (UnitLocationA :type Vector%202D%20Structure) (UnitLocationB :type Vector%202D%20Structure) (PlayerA :type Owner%20Structure) (PlayerB :type Owner%20Structure))
  (bind _unitlocations_player4 (Variables|Default|GetUnitLocations_Player4))
  (bind _unitlocations_player3 (Variables|Default|GetUnitLocations_Player3))
  (bind _unitlocations_player2 (Variables|Default|GetUnitLocations_Player2))
  (bind _unitlocations_player1 (Variables|Default|GetUnitLocations_Player1))
  (bind _unitlocations_player1_2 (Variables|Default|GetUnitLocations_Player1))
  (bind _unitlocations_player2_2 (Variables|Default|GetUnitLocations_Player2))
  (bind _unitlocations_player3_2 (Variables|Default|GetUnitLocations_Player3))
  (bind _unitlocations_player4_2 (Variables|Default|GetUnitLocations_Player4))
  (Variables|Default|SetTMP%20Unit%20Location%20A UnitLocationA)
  (Variables|Default|SetTMP%20Unit%20Location%20B UnitLocationB)
  (Variables|Default|SetPlayer%20A PlayerA)
  (Variables|Default|SetPlayer%20B PlayerB)
  (CallFunction|AddPresentPlayer)
  (Utilities|FlowControl|Sequence
    (:then_0
      (switch Utilities|FlowControl|Switch|SwitchonETeam (.Team (Utilities|Struct|BreakOwner (Variables|Default|GetPlayer%20A)))
        (:Team1
          (Utilities|Array|Add _unitlocations_player1_2 (Variables|Default|GetTMP%20Unit%20Location%20A))
          (Variables|Default|SetHasUpdated_Player1 true :!label _label)
          (if (> (Utilities|Array|Length _unitlocations_player1) 4)
            (Utilities|Array|RemoveIndex _unitlocations_player1)))
        (:Team2
          (Utilities|Array|Add _unitlocations_player2_2 (Variables|Default|GetTMP%20Unit%20Location%20A))
          (Variables|Default|SetHasUpdated_Player2 true :!label _label_2)
          (if (> (Utilities|Array|Length _unitlocations_player2) 4)
            (Utilities|Array|RemoveIndex _unitlocations_player2)))
        (:Team3
          (Utilities|Array|Add _unitlocations_player3_2 (Variables|Default|GetTMP%20Unit%20Location%20A))
          (Variables|Default|SetHasUpdated_Player3 true :!label _label_3)
          (if (> (Utilities|Array|Length _unitlocations_player3) 4)
            (Utilities|Array|RemoveIndex _unitlocations_player3)))
        (:Team4
          (Utilities|Array|Add _unitlocations_player4_2 (Variables|Default|GetTMP%20Unit%20Location%20A))
          (Variables|Default|SetHasUpdated_Player4 true :!label _label_4)
          (if (> (Utilities|Array|Length _unitlocations_player4) 4)
            (Utilities|Array|RemoveIndex _unitlocations_player4)))))
    (:then_1
      (switch Utilities|FlowControl|Switch|SwitchonETeam (.Team (Utilities|Struct|BreakOwner (Variables|Default|GetPlayer%20B)))
        (:Team1
          (Utilities|Array|Add _unitlocations_player1_2 (Variables|Default|GetTMP%20Unit%20Location%20B))
          (goto _label))
        (:Team2
          (Utilities|Array|Add _unitlocations_player2_2 (Variables|Default|GetTMP%20Unit%20Location%20B))
          (goto _label_2))
        (:Team3
          (Utilities|Array|Add _unitlocations_player3_2 (Variables|Default|GetTMP%20Unit%20Location%20B))
          (goto _label_3))
        (:Team4
          (Utilities|Array|Add _unitlocations_player4_2 (Variables|Default|GetTMP%20Unit%20Location%20B))
          (goto _label_4))))))

(event Custom|UpdateBattlePosition
  (bind _localbattletheme (Variables|Default|GetLocalBattleTheme))
  (Development|PrintText "UpdateBattlePosition" false false)
  (Variables|Default|SetClosestCentroidPosition "")
  (for (_ _array_index) (Utilities|Array|MakeArray (Variables|Default|GetHasUpdated_Player1) (Variables|Default|GetHasUpdated_Player2) (Variables|Default|GetHasUpdated_Player3) (Variables|Default|GetHasUpdated_Player4))
    (Math|Integer|CompareInt (Math|Conversions|ToInteger(Boolean) (Utilities|Array|Get(acopy) (Utilities|Array|MakeArray (Variables|Default|GetHasUpdated_Player1) (Variables|Default|GetHasUpdated_Player2) (Variables|Default|GetHasUpdated_Player3) (Variables|Default|GetHasUpdated_Player4)) _array_index)) 1
      (:==
        (bind _output_get (Variables|Default|SetNumber%20True (+ (Variables|Default|GetNumber%20True) 1)))
        (Development|PrintString (Utilities|String|Append "NumberTrue: " (Utilities|String|ToString(Integer) _output_get)) false false)
        (switch int _array_index
          (:0
            (Variables|Default|SetHasUpdated_Player1 false))
          (:1
            (Variables|Default|SetHasUpdated_Player2 false))
          (:2
            (Variables|Default|SetHasUpdated_Player3 false))
          (:3
            (Variables|Default|SetHasUpdated_Player4 false))))))
  (if (< (Variables|Default|GetNumber%20True) 1)
    (bind _output_get_2 (Variables|Default|SetFailedBattles (+ (Variables|Default|GetFailedBattles) 1)))
    (Utilities|IsValid _localbattletheme
      (:Is%20Valid
        (Audio|Components|Audio|FadeOut _localbattletheme (* (Variables|/Script/Engine.AudioComponent|GetVolumeMultiplier _localbattletheme) 0.4) 0.0 "Linear" :!class /Script/Engine.AudioComponent)
        (Development|PrintString (Utilities|String|Append (Utilities|String|ToString(Byte) _output_get_2) " failed battles") false false))
      (:Is%20Not%20Valid
        _))
    (if (>= (Variables|Default|GetFailedBattles) 2)
      (Utilities|IsValid 0
        (:Is%20Valid
          (Audio|Components|Audio|FadeOut (Variables|/Game/Blueprints/GameMode/BP_GameInstanceInfernale.BP_GameInstanceInfernale_C|GetBattleTheme_Instances (.AsBP%20Game%20Instance%20Infernale (Utilities|Casting|CastToBP_GameInstanceInfernale (Game|GetGameInstance)))) 5.0 0.0 "Logarithmic" :!class /Script/Engine.AudioComponent))
        (:Is%20Not%20Valid
          (Actor|DestroyActor)
          (Variables|Default|SetNumber%20True 0 :!label _label))))
    (else
      (Variables|Default|SetFailedBattles 0)
      (bind _returnvalue (Class|SoundsDataAsset|GetSoundType (Variables|Default|GetDA%20Sound) "Music" "Ambient Mid - Battle"))
      (Utilities|IsValid _localbattletheme
        (:Is%20Valid
          (Audio|Components|Audio|FadeOut _localbattletheme 3.0 (* (.Volume (Utilities|Struct|BreakSoundType _returnvalue)) (Variables|/Script/InfernaleTesting.GameInstanceInfernale|GetMasterXMusicVolume (.AsBP%20Game%20Instance%20Infernale (Utilities|Casting|CastToBP_GameInstanceInfernale (Game|GetGameInstance))))) "Linear" :!class /Script/Engine.AudioComponent)
          (goto _label))
        (:Is%20Not%20Valid
          (goto _label))))))

(event Custom|AddPresentPlayer
  (bind _listofplayers (Variables|Default|GetListOfPlayers))
  (bind _returnvalue (Utilities|Array|AddUnique _listofplayers (Variables|Default|GetPlayer%20A)))
  (bind _returnvalue_2 (Utilities|Array|AddUnique _listofplayers (Variables|Default|GetPlayer%20B))))

(event EventBeginPlay
  (bind _returnvalue (Transformation|GetActorLocation))
  (bind _returnvalue_2 (Game|GetGameInstance))
  (bind _fadeoutdurationcombat (Variables|Default|GetFadeoutDurationCombat))
  (bind (_x _y _z) (Math|Vector|BreakVector _returnvalue))
  (bind _asbp_game_instance_infernale (Utilities|Casting|CastToBP_GameInstanceInfernale _returnvalue_2))
  (bind _output_get (Variables|Default|SetDA%20Sound (.soundsassets (Utilities|Array|Get(acopy) (Variables|/Script/InfernaleTesting.GameSettingsDataAsset|GetDataAssetsSettings (Class|FunctionLibraryInfernale|GetGameSettingsDataAsset))))))
  (Utilities|FlowControl|Sequence
    (:then_0
      (Variables|Default|SetOwnerLocal (Variables|/Script/InfernaleTesting.PlayerStateInfernale|GetOwnerInfo (.AsBP%20Player%20State%20Infernale (Utilities|Casting|CastToBP_PlayerStateInfernale (Game|GetPlayerState 0)))))
      (Utilities|FlowControl|Delay 1.0)
      (Utilities|FlowControl|Sequence
        (:then_0
          (Development|PrintText "UpdateBattlePosition" false false)
          (Variables|Default|SetClosestCentroidPosition "")
          (for (_ _array_index) (Utilities|Array|MakeArray (Variables|Default|GetHasUpdated_Player1) (Variables|Default|GetHasUpdated_Player2) (Variables|Default|GetHasUpdated_Player3) (Variables|Default|GetHasUpdated_Player4))
            (Math|Integer|CompareInt (Math|Conversions|ToInteger(Boolean) (Utilities|Array|Get(acopy) (Utilities|Array|MakeArray (Variables|Default|GetHasUpdated_Player1) (Variables|Default|GetHasUpdated_Player2) (Variables|Default|GetHasUpdated_Player3) (Variables|Default|GetHasUpdated_Player4)) _array_index)) 1
              (:==
                (bind _output_get_2 (Variables|Default|SetNumber%20True (+ (Variables|Default|GetNumber%20True) 1)))
                (Development|PrintString (Utilities|String|Append "NumberTrue: " (Utilities|String|ToString(Integer) _output_get_2)) false false)
                (switch int _array_index
                  (:0
                    (Variables|Default|SetHasUpdated_Player1 false))
                  (:1
                    (Variables|Default|SetHasUpdated_Player2 false))
                  (:2
                    (Variables|Default|SetHasUpdated_Player3 false))
                  (:3
                    (Variables|Default|SetHasUpdated_Player4 false))))))
          (if (< (Variables|Default|GetNumber%20True) 1)
            (bind _output_get_3 (Variables|Default|SetFailedBattles (+ (Variables|Default|GetFailedBattles) 1)))
            (Utilities|IsValid (Variables|Default|GetLocalBattleTheme)
              (:Is%20Valid
                (Audio|Components|Audio|FadeOut (Variables|Default|GetLocalBattleTheme) (* (Variables|/Script/Engine.AudioComponent|GetVolumeMultiplier (Variables|Default|GetLocalBattleTheme)) 0.4) 0.0 "Linear" :!class /Script/Engine.AudioComponent)
                (Development|PrintString (Utilities|String|Append (Utilities|String|ToString(Byte) _output_get_3) " failed battles") false false))
              (:Is%20Not%20Valid
                _))
            (if (>= (Variables|Default|GetFailedBattles) 2)
              (Utilities|IsValid 0
                (:Is%20Valid
                  (Audio|Components|Audio|FadeOut (Variables|/Game/Blueprints/GameMode/BP_GameInstanceInfernale.BP_GameInstanceInfernale_C|GetBattleTheme_Instances (.AsBP%20Game%20Instance%20Infernale (Utilities|Casting|CastToBP_GameInstanceInfernale (Game|GetGameInstance)))) 5.0 0.0 "Logarithmic" :!class /Script/Engine.AudioComponent))
                (:Is%20Not%20Valid
                  (Actor|DestroyActor)
                  (Variables|Default|SetNumber%20True 0 :!label _label))))
            (else
              (Variables|Default|SetFailedBattles 0)
              (bind _returnvalue_3 (Class|SoundsDataAsset|GetSoundType (Variables|Default|GetDA%20Sound) "Music" "Ambient Mid - Battle"))
              (Utilities|IsValid (Variables|Default|GetLocalBattleTheme)
                (:Is%20Valid
                  (Audio|Components|Audio|FadeOut (Variables|Default|GetLocalBattleTheme) 3.0 (* (.Volume (Utilities|Struct|BreakSoundType _returnvalue_3)) (Variables|/Script/InfernaleTesting.GameInstanceInfernale|GetMasterXMusicVolume (.AsBP%20Game%20Instance%20Infernale (Utilities|Casting|CastToBP_GameInstanceInfernale (Game|GetGameInstance))))) "Linear" :!class /Script/Engine.AudioComponent)
                  (goto _label))
                (:Is%20Not%20Valid
                  (goto _label))))))
        (:then_1
          (Utilities|Time|SetTimerbyEvent (delegate Custom|UpdateBattlePosition) (Variables|Default|GetUpdate%20Period) true))))
    (:then_1
      (bind _returnvalue_4 (Class|SoundsDataAsset|GetSoundType _output_get "Music" "Ambient Mid - Battle" :!label _label_2))
      (Development|PrintString (.SoundName (Utilities|Struct|BreakSoundType _returnvalue_4)) false false)
      (bind _returnvalue_5 (Audio|SpawnSoundatLocation (.Sound (Utilities|Struct|BreakSoundType _returnvalue_4)) (Math|Vector|MakeVector _x _y _z) "90.000000,0.000000,0.000000" (* (.Volume (Utilities|Struct|BreakSoundType _returnvalue_4)) (Variables|/Script/InfernaleTesting.GameInstanceInfernale|GetMasterXMusicVolume _asbp_game_instance_infernale)) 1.0 0.0 0 0))
      (Audio|Components|Audio|FadeIn _returnvalue_5 2.0 (* (.Volume (Utilities|Struct|BreakSoundType _returnvalue_4)) (Variables|/Script/InfernaleTesting.GameInstanceInfernale|GetMasterXMusicVolume _asbp_game_instance_infernale)) 2.0 "Linear" :!class /Script/Engine.AudioComponent)
      (Variables|Default|SetLocalBattleTheme _returnvalue_5)
      (Utilities|Array|Add (Variables|/Game/Blueprints/GameMode/BP_GameInstanceInfernale.BP_GameInstanceInfernale_C|GetBattleTheme_Instances _asbp_game_instance_infernale) _returnvalue_5)
      (Utilities|FlowControl|Delay (- (Variables|/Script/Engine.SoundBase|GetDuration (.Sound (Utilities|Struct|BreakSoundType _returnvalue_4))) _fadeoutdurationcombat))
      (Audio|Components|Audio|FadeOut _returnvalue_5 _fadeoutdurationcombat 0.0 "Linear" :!class /Script/Engine.AudioComponent)
      (goto _label_2))))

(fn ConstructionScript)