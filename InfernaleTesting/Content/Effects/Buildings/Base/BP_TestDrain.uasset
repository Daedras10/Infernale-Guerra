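; Test actor for a drain building effect that stretches the SM_Drain mesh from a default start position to its End component.
; Both the construction script and BeginPlay run the same logic, each adding a thin, X-forward spline mesh component.
; The mesh end follows End's relative location with a strong fixed downward Z tangent, while the Start component is unused.
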(event EventBeginPlay
  (bind _returnvalue (AddComponent|AddSplineMeshComponent false))
  (SplineMesh|SetStartScale _returnvalue "(X=0.010000,Y=0.010000)" true :!class /Script/Engine.SplineMeshComponent)
  (SplineMesh|SetEndScale _returnvalue "(X=0.010000,Y=0.010000)" true :!class /Script/Engine.SplineMeshComponent)
  (SplineMesh|SetForwardAxis _returnvalue "X" true)
  (Components|StaticMesh|SetStaticMesh _returnvalue "/Game/Effects/Buildings/Base/Meshes/SM_Drain.SM_Drain")
  (bind _output_get (Variables|Default|SetTargetPos (Variables|/Script/Engine.SceneComponent|GetRelativeLocation (Variables|Default|GetEnd))))
  (SplineMesh|SetStartandEnd _returnvalue "0, 0, 0" "0, 0, 0" _output_get "0.000000,0.000000,-5000.000000" true :!class /Script/Engine.SplineMeshComponent))

(event Collision|EventActorBeginOverlap
  (params (OtherActor :type Actor%20Object%20Reference)))

(event EventTick
  (params (DeltaSeconds :type Float%20%28single-precision%29)))

(fn ConstructionScript
  (bind _returnvalue (AddComponent|AddSplineMeshComponent false))
  (SplineMesh|SetStartScale _returnvalue "(X=0.010000,Y=0.010000)" true :!class /Script/Engine.SplineMeshComponent)
  (SplineMesh|SetEndScale _returnvalue "(X=0.010000,Y=0.010000)" true :!class /Script/Engine.SplineMeshComponent)
  (SplineMesh|SetForwardAxis _returnvalue "X" true)
  (Components|StaticMesh|SetStaticMesh _returnvalue "/Game/Effects/Buildings/Base/Meshes/SM_Drain.SM_Drain")
  (bind _output_get (Variables|Default|SetTargetPos (Variables|/Script/Engine.SceneComponent|GetRelativeLocation (Variables|Default|GetEnd))))
  (SplineMesh|SetStartandEnd _returnvalue "0, 0, 0" "0, 0, 0" _output_get "0.000000,0.000000,-5000.000000" true :!class /Script/Engine.SplineMeshComponent))