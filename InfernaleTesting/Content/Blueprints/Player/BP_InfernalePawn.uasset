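; BP_InfernalePawn is the player's camera pawn, handling widget clicks, camera jumps to targets and the endgame cinematic.
; Local mouse events from the player controller drive WidgetInteraction, and spawn events manage loading screen and HUD.
; Move events snap or timeline-lerp the pawn, offset behind the camera's flattened forward, notifying AmbianceManager.
; LaunchSequence tints tagged Niagara and meshes with the winning team's color, plays tagged sequences, then flags the GameMode on authority.
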(event Custom|BindWidgetInteraction
  (bind _returnvalue (Game|GetPlayerController 0))
  (bind _asbp_player_controller_infernale (Utilities|Casting|CastToBP_PlayerControllerInfernale _returnvalue))
  (if (Pawn|IsLocallyControlled)
    (EventDispatchers|AssignMousePrimaryStart _asbp_player_controller_infernale (delegate Custom|MousePrimaryStart_Event))
    (EventDispatchers|BindEventtoMousePrimaryEnd _asbp_player_controller_infernale (delegate Custom|MousePrimaryEnd_Event))))

(event Custom|MousePrimaryStart_Event
  (Class|WidgetInteractionComponent|PressPointerKey (Variables|Default|GetWidgetInteraction) "LeftMouseButton"))

(event Custom|MousePrimaryEnd_Event
  (Class|WidgetInteractionComponent|ReleasePointerKey (Variables|Default|GetWidgetInteraction) "LeftMouseButton"))

(event Custom|MovePawnToActor
  (params (New%20Location%20Actor :type Actor%20Object%20Reference))
  (bind _returnvalue (Transformation|GetActorLocation New%20Location%20Actor))
  (bind _cameracomponent (Variables|Default|GetCameraComponent))
  (bind _returnvalue_2 (Math|Vector|GetForwardVector _cameracomponent))
  (bind _returnvalue_3 (* _returnvalue_2 "1.000000,1.000000,0.000000"))
  (bind _returnvalue_4 (Math|Vector|Normalize _returnvalue_3))
  (bind _returnvalue_5 (* _returnvalue_4 5e+03))
  (bind _returnvalue_6 (- _returnvalue _returnvalue_5))
  (bind (_x _y) (Math|Vector|BreakVector _returnvalue_6))
  ;[0 0 0] MovePawnToLocation
  (Utilities|IsValid New%20Location%20Actor
    (:Is%20Valid
      (Transformation|SetActorLocation (Math|Vector|MakeVector _x _y (.Z (Math|Vector|BreakVector (Transformation|GetActorLocation)))) false false))))

(event Custom|MovePawnToLocation
  (params (New%20Location :type Vector))
  (bind _returnvalue (Transformation|GetActorLocation))
  (bind _cameracomponent (Variables|Default|GetCameraComponent))
  (bind _returnvalue_2 (Math|Vector|GetForwardVector _cameracomponent))
  (bind _z (Math|Vector|BreakVector _returnvalue))
  (bind _returnvalue_3 (* _returnvalue_2 "1.000000,1.000000,0.000000"))
  (bind _returnvalue_4 (Math|Vector|Normalize _returnvalue_3))
  (bind _returnvalue_5 (* _returnvalue_4 5e+03))
  (bind _returnvalue_6 (- New%20Location _returnvalue_5))
  (bind (_x _y) (Math|Vector|BreakVector _returnvalue_6))
  (bind _returnvalue_7 (Math|Vector|MakeVector _x _y _z))
  ;[0 0 0] MovePawnToLocation
  (Components|Timeline|SetPlayRate (Variables|Default|GetTimeline) 6.0)
  (bind _value (Timeline|Timeline PlayFromStart)
    (:Update
      (if (Variables|Default|GetbisMoving)
        (Timeline|Timeline Stop)
        (elif (<= (- 1.0 0.0) 0.05)
          (Transformation|SetActorLocation _returnvalue_7 false false)
          (Timeline|Timeline Stop)
          (else
            (Transformation|SetActorLocation (Math|Vector|Lerp(Vector) (Transformation|GetActorLocation) _returnvalue_7 _value) false false)
            (Utilities|IsValid (Variables|Default|GetAmbianceManager) :!label _label
              (:Is%20Valid
                (Class|AmbianceManager|OnPCMoveBP (Variables|Default|GetAmbianceManager)))
              (:Is%20Not%20Valid
                (bind _outactors (Actor|GetAllActorsOfClass "/Script/InfernaleTesting.AmbianceManager"))
                (Variables|Default|SetAmbianceManager (Utilities|Array|Get(acopy) _outactors))
                (Utilities|FlowControl|Delay 0.2)
                (goto _label)))))))))

(event Custom|LaunchSequence
  (params (VictoryPoints :type Victory%20Points%20Structure))
  (bind (_victorypointsnature _victorypointsteam1 _victorypointsteam2 _victorypointsteam3 _victorypointsteam4) (Utilities|Struct|BreakVictoryPoints VictoryPoints))
  (bind _returnvalue (Class|FunctionLibraryInfernale|GetGameSettingsDataAsset))
  (bind _color (CallFunction|GetTeamColor "Team4"))
  (bind _color_2 (CallFunction|GetTeamColor "Team1"))
  (bind _color_3 (CallFunction|GetTeamColor "Team2"))
  (bind _color_4 (CallFunction|GetTeamColor "Team3"))
  (bind _returnvalue_2 (Math|Float|Max(Float) _victorypointsteam1 _victorypointsteam2 _victorypointsteam3 _victorypointsteam4))
  (bind _map (Utilities|Map|MakeMap _victorypointsteam1 _color_2 _victorypointsteam2 _color_3 _victorypointsteam3 _color_4 _victorypointsteam4 _color))
  (bind _dataassetssettings (Variables|/Script/InfernaleTesting.GameSettingsDataAsset|GetDataAssetsSettings _returnvalue))
  (bind _value (Utilities|Map|Find _map _returnvalue_2))
  (bind _output (Utilities|Array|Get(acopy) _dataassetssettings))
  (bind _soundsassets (Utilities|Struct|BreakDataAssetsSettings _output))
  (Default|SwitchVisibilityOfAllWidgets (Variables|/Game/Blueprints/GameMode/Infernale/BP_PlayerControllerInfernale.BP_PlayerControllerInfernale_C|GetBP_UIComponent (.AsBP%20Player%20Controller%20Infernale (Utilities|Casting|CastToBP_PlayerControllerInfernale (Game|GetPlayerController 0)))) false false)
  (Class|InfernalePawn|SetDoCameraEndGameTraving)
  (bind _returnvalue_3 (Class|SoundsDataAsset|GetSoundType _soundsassets "Map" "Endgame Impact"))
  (Class|SoundsDataAsset|PlaySound _soundsassets "Map" (.soundname _returnvalue_3) (Transformation|GetWorldLocation (Variables|Default|GetCameraComponent)))
  (Utilities|FlowControl|Delay 0.5)
  (bind _outactors (Actor|GetAllActorswithTag "EndGameNoColor"))
  (for _array_element _outactors
    (bind _asniagara_actor (Utilities|Casting|CastToNiagaraActor _array_element))
    (Components|Activation|Activate (Variables|/Script/Niagara.NiagaraActor|GetNiagaraComponent _asniagara_actor) false))
  (bind _outactors_2 (Actor|GetAllActorswithTag "EndGameColor"))
  (for _array_element_2 _outactors_2
    (bind _asniagara_actor_2 (Utilities|Casting|CastToNiagaraActor _array_element_2))
    (Niagara|SetNiagaraVariable(LinearColor) (Variables|/Script/Niagara.NiagaraActor|GetNiagaraComponent _asniagara_actor_2) "TeamColor" (.specifiedcolor _value))
    (Components|Activation|Activate (Variables|/Script/Niagara.NiagaraActor|GetNiagaraComponent _asniagara_actor_2) false))
  (bind _outactors_3 (Actor|GetAllActorswithTag "PandemoniumSM"))
  (for _array_element_3 _outactors_3
    (bind _returnvalue_4 (Rendering|Material|CreateDynamicMaterialInstance (Variables|/Script/Engine.StaticMeshActor|GetStaticMeshComponent (.AsStatic%20Mesh%20Actor (Utilities|Casting|CastToStaticMeshActor _array_element_3))) 0 (Rendering|Material|GetMaterial (Variables|/Script/Engine.StaticMeshActor|GetStaticMeshComponent (.AsStatic%20Mesh%20Actor (Utilities|Casting|CastToStaticMeshActor _array_element_3))) 0) "None" :!class /Script/Engine.PrimitiveComponent))
    (bind _returnvalue_5 (Rendering|Material|CreateDynamicMaterialInstance (Variables|/Script/Engine.StaticMeshActor|GetStaticMeshComponent (.AsStatic%20Mesh%20Actor (Utilities|Casting|CastToStaticMeshActor _array_element_3))) 1 (Rendering|Material|GetMaterial (Variables|/Script/Engine.StaticMeshActor|GetStaticMeshComponent (.AsStatic%20Mesh%20Actor (Utilities|Casting|CastToStaticMeshActor _array_element_3))) 1) "None" :!class /Script/Engine.PrimitiveComponent))
    (bind _returnvalue_6 (Rendering|Material|CreateDynamicMaterialInstance (Variables|/Script/Engine.StaticMeshActor|GetStaticMeshComponent (.AsStatic%20Mesh%20Actor (Utilities|Casting|CastToStaticMeshActor _array_element_3))) 2 (Rendering|Material|GetMaterial (Variables|/Script/Engine.StaticMeshActor|GetStaticMeshComponent (.AsStatic%20Mesh%20Actor (Utilities|Casting|CastToStaticMeshActor _array_element_3))) 2) "None" :!class /Script/Engine.PrimitiveComponent))
    (Rendering|Material|SetVectorParameterValue _returnvalue_4 "ColorEmissive" (.specifiedcolor _value) :!class /Script/Engine.MaterialInstanceDynamic))
  (Utilities|FlowControl|Delay 2.0)
  (bind _outactors_4 (Actor|GetAllActorswithTag "EndGame"))
  (for _array_element_4 _outactors_4
    (bind _aslevel_sequence_actor (Utilities|Casting|CastToLevelSequenceActor _array_element_4))
    (Sequencer|Player|Play (Variables|/Script/LevelSequence.LevelSequenceActor|GetSequencePlayer _aslevel_sequence_actor) :!class /Script/MovieScene.MovieSceneSequencePlayer)
    (EventDispatchers|BindEventtoOnFinished (Variables|/Script/LevelSequence.LevelSequenceActor|GetSequencePlayer _aslevel_sequence_actor) (delegate Custom|Sequence%20Finished))
    ;[1 1 1] Progemon
    (Utilities|FlowControl|Delay 3.2)
    (Game|Feedback|ClientStartCameraShake (.AsBP%20Player%20Controller%20Infernale (Utilities|Casting|CastToBP_PlayerControllerInfernale (Pawn|GetController))) "/Game/Blueprints/Camera/BP_Shake.BP_Shake_C" 5.0 "World" "0, 0, 0")
    (Utilities|FlowControl|Delay 0.2)))

(event Custom|Sequence%20Finished
  (Networking|SwitchHasAuthority
    (:Authority
      (Default|SetAnimFinished (.AsBP%20Game%20Mode%20Infernale (Utilities|Casting|CastToBP_GameModeInfernale (Game|GetGameMode))) true))))

(event EventPossessed
  (params (NewController :type Controller%20Object%20Reference))
  (CallFunction|BindWidgetInteraction)
  (bind _outactors (Actor|GetAllActorsOfClass "/Script/InfernaleTesting.AmbianceManager"))
  (Variables|Default|SetAmbianceManager (Utilities|Array|Get(acopy) _outactors)))

(event EventOnPawnSetatSpawnBP
  (Default|DestroyLoadingScreen (Variables|/Game/Blueprints/Component/PlayerController/BP_UIComponent.BP_UIComponent_C|GetLoadingScreen (Variables|/Game/Blueprints/GameMode/Infernale/BP_PlayerControllerInfernale.BP_PlayerControllerInfernale_C|GetBP_UIComponent (.AsBP%20Player%20Controller%20Infernale (Utilities|Casting|CastToBP_PlayerControllerInfernale (Game|GetPlayerController 0)))))))

(event EventOnPawnSpawnTravelFinishedBP
  (Default|SwitchVisibilityOfAllWidgets (Variables|/Game/Blueprints/GameMode/Infernale/BP_PlayerControllerInfernale.BP_PlayerControllerInfernale_C|GetBP_UIComponent (.AsBP%20Player%20Controller%20Infernale (Utilities|Casting|CastToBP_PlayerControllerInfernale (Game|GetPlayerController 0)))) true true))

(event Input|KeyboardEvents|Tab
  (params (Key :type Key%20Structure :default "None")))

(fn ConstructionScript)