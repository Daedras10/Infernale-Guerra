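; Shared function library for Infernale that centralises team visuals and small gameplay, UI and save helpers.
; Team-keyed Selects supply materials, UI colours and Behemoth, Gobborrit and Nerras palettes; overlays show other non-nature teams as hostile.
; Helpers spawn screen-space popup widgets on actors, lazily create player-settings saves, map indices to player/team IDs and format player info.
; IsActorOnScreen actually returns true for off-screen positions; effect formatting and NewFunction are unfinished stubs.
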(fn NewFunction)

(fn GetTeamMaterial
  (params (Owner :type Owner%20Structure%20%28by%20ref%29))
  (return (Utilities|Select :Index (.Team (Utilities|Struct|BreakOwner Owner)) :NatureTeam "/Engine/BasicShapes/BasicShapeMaterial.BasicShapeMaterial" :Team1 "/Engine/MapTemplates/Materials/BasicAsset01.BasicAsset01" :Team2 "/Engine/MapTemplates/Materials/BasicAsset02.BasicAsset02" :Team3 "/Engine/MapTemplates/Materials/BasicAsset03.BasicAsset03" :Team4 "/Engine/BufferVisualization/BaseColor.BaseColor")))

(fn GetTeamColor
  (params (Team :type ETeam%20Enum :default "NatureTeam"))
  (return (Utilities|Select :Index Team :NatureTeam (Utilities|Struct|MakeSlateColor "(R=0.406250,G=0.406250,B=0.406250,A=1.000000)") :Team1 (Utilities|Struct|MakeSlateColor "(R=0.360784,G=1.000000,B=0.121569,A=1.000000)") :Team2 (Utilities|Struct|MakeSlateColor "(R=0.000000,G=0.486275,B=1.000000,A=1.000000)") :Team3 (Utilities|Struct|MakeSlateColor "(R=1.000000,G=0.184314,B=0.000000,A=1.000000)") :Team4 (Utilities|Struct|MakeSlateColor "(R=0.666667,G=0.129412,B=1.000000,A=1.000000)"))))

(fn GetTeamSecondColor
  (params (Team :type ETeam%20Enum :default "NatureTeam"))
  (return (Utilities|Select :Index Team :NatureTeam (Utilities|Struct|MakeSlateColor "(R=0.057292,G=0.057292,B=0.057292,A=1.000000)") :Team1 (Utilities|Struct|MakeSlateColor "(R=0.000000,G=0.656250,B=0.578308,A=1.000000)") :Team2 (Utilities|Struct|MakeSlateColor "(R=0.059408,G=0.076232,B=0.380208,A=16.000000)") :Team3 (Utilities|Struct|MakeSlateColor "(R=1.000000,G=0.035092,B=0.000000,A=1.000000)") :Team4 (Utilities|Struct|MakeSlateColor "(R=0.283593,G=0.070014,B=0.463542,A=1.000000)"))))

(fn GetTeamThirdColor
  (params (Team :type ETeam%20Enum :default "NatureTeam"))
  (return (Utilities|Select :Index Team :NatureTeam (Utilities|Struct|MakeSlateColor "(R=0.348958,G=0.348958,B=0.348958,A=1.000000)") :Team1 (Utilities|Struct|MakeSlateColor "(R=0.152941,G=0.545098,B=0.470588,A=1.000000)") :Team2 (Utilities|Struct|MakeSlateColor "(R=0.227451,G=0.400000,B=0.670588,A=1.000000)") :Team3 (Utilities|Struct|MakeSlateColor "(R=0.764706,G=0.392157,B=0.341176,A=1.000000)") :Team4 (Utilities|Struct|MakeSlateColor "(R=0.235294,G=0.231373,B=0.670588,A=1.000000)"))))

(fn GetTeamVectorColor
  (params (Team :type ETeam%20Enum :default "NatureTeam"))
  (bind ___worldcontext (LocalVariables|Get__WorldContext))
  (bind _color (CallFunction|GetTeamColor Team ___worldcontext))
  (bind _specifiedcolor (Utilities|Struct|BreakSlateColor _color))
  (bind (_r _g _b) (Math|Color|BreakColor _specifiedcolor))
  (return (Math|Vector|MakeVector _r _g _b)))

(fn IsActoronScreen
  (params (Player :type Player%20Controller%20Object%20Reference) (Actor :type Actor%20Object%20Reference))
  (bind _returnvalue (Transformation|GetActorLocation Actor))
  (bind ___worldcontext (LocalVariables|Get__WorldContext))
  (bind _screenposition (Class|GameplayStatics|ProjectWorldtoScreen Player _returnvalue true))
  (bind _returnvalue_2 (Viewport|GetViewportSize ___worldcontext))
  (bind (_x _y) (Math|Vector2D|BreakVector2D _screenposition))
  (bind (_x_2 _y_2) (Math|Vector2D|BreakVector2D _returnvalue_2))
  (return (Math|Boolean|ORBoolean (< _x 0.0) (< _y 0.0) (> _x _x_2) (> _y _y_2))))

(fn GetPosonCircle2D
  (params (R :type Float%20%28double-precision%29) (Teta :type Float%20%28double-precision%29))
  (return (Math|Vector2D|MakeVector2D (* R (Math|Trig|Cos(Degrees) Teta)) (* R (Math|Trig|Sin(Degrees) Teta)))))

(fn GetEffectFormatWIP
  (params (Effect :type Node%20Effect%20Structure))
  (bind (_nodeeffect _value _ispercentage) (Utilities|Struct|BreakNodeEffect Effect))
  (switch Utilities|FlowControl|Switch|SwitchonENodeEffect _nodeeffect
    (:NodeEffectNone
      (return ""))
    (:NodeEffectDamageToBuilding
      (return (select _ispercentage "" "")))
    (:NodeEffectDamageToMonster
      (return ""))
    (:NodeEffectDamageToUnit
      (return ""))
    (:NodeEffectHealthUnit
      (return ""))
    (:NodeEffectHealthBuilding
      (return ""))
    (:NodeEffectFluxRange
      (return ""))
    (:NodeEffectUnitSight
      (return ""))
    (:NodeEffectUnitSpeed
      (return ""))
    (:NodeEffectBuildingSight
      (return ""))
    (:NodeEffectBuildingRecycleSouls
      (return ""))
    (:NodeEffectBuildingOverclockDuration
      (return ""))
    (:NodeEffectBuildingConstructionTime
      (return ""))
    (:NodeEffectBuildingConstructionCost
      (return ""))))

(fn CreatePopUp
  (params (CallerActor :type Actor%20Object%20Reference) (PopUpText :type Text) (PopUpIcon :type Texture%202D%20Object%20Reference) (PopUpDuration :type Float%20%28double-precision%29))
  (bind _returnvalue (UserInterface|CreateWidget "/Game/UI/InGame/WBP_PopUp.WBP_PopUp_C" (Game|GetPlayerController 0)))
  (bind _returnvalue_2 (Game|AddComponentbyClass CallerActor "/Script/UMG.WidgetComponent" false))
  (Variables|/Script/Engine.ActorComponent|SetComponentTags _returnvalue_2 (Utilities|Array|MakeArray (Utilities|Name|MakeLiteralName "Popup")))
  (Class|WidgetComponent|SetWidgetSpace _returnvalue_2 "Screen")
  (UserInterface|SetWidget _returnvalue_2 _returnvalue)
  (Default|Init _returnvalue PopUpText PopUpDuration PopUpIcon CallerActor))

(fn GetBehemothTeamColor
  (params (Team :type ETeam%20Enum :default "NatureTeam"))
  (return (Utilities|Select :Index Team :NatureTeam (Utilities|Struct|MakeSlateColor "(R=0.406250,G=0.406250,B=0.406250,A=1.000000)") :Team1 (Utilities|Struct|MakeSlateColor "(R=0.019382,G=0.141263,B=0.066626,A=1.000000)") :Team2 (Utilities|Struct|MakeSlateColor "(R=0.000000,G=0.070360,B=0.088656,A=1.000000)") :Team3 (Utilities|Struct|MakeSlateColor "(R=0.191202,G=0.090842,B=0.000000,A=1.000000)") :Team4 (Utilities|Struct|MakeSlateColor "(R=0.097587,G=0.046665,B=0.181164,A=1.000000)"))))

(fn GetBehemothEmissColor
  (params (Team :type ETeam%20Enum :default "NatureTeam"))
  (return (Utilities|Select :Index Team :NatureTeam (Utilities|Struct|MakeSlateColor "(R=0.406250,G=0.406250,B=0.406250,A=1.000000)") :Team1 (Utilities|Struct|MakeSlateColor "(R=0.149960,G=1.000000,B=0.313989,A=1.000000)") :Team2 (Utilities|Struct|MakeSlateColor "(R=0.000000,G=0.181164,B=1.000000,A=1.000000)") :Team3 (Utilities|Struct|MakeSlateColor "(R=1.000000,G=0.274677,B=0.000000,A=1.000000)") :Team4 (Utilities|Struct|MakeSlateColor "(R=0.177888,G=0.000000,B=1.000000,A=1.000000)"))))

(fn GetGobborritEmissColor
  (params (Team :type ETeam%20Enum :default "NatureTeam"))
  (return (Utilities|Select :Index Team :NatureTeam (Utilities|Struct|MakeSlateColor "(R=0.406250,G=0.406250,B=0.406250,A=1.000000)") :Team1 (Utilities|Struct|MakeSlateColor "(R=0.070360,G=1.000000,B=0.000000,A=1.000000)") :Team2 (Utilities|Struct|MakeSlateColor "(R=0.000000,G=0.799103,B=1.000000,A=1.000000)") :Team3 (Utilities|Struct|MakeSlateColor "(R=1.000000,G=0.571125,B=0.000000,A=1.000000)") :Team4 (Utilities|Struct|MakeSlateColor "(R=0.291771,G=0.086500,B=1.000000,A=1.000000)"))))

(fn GetGobborritTeamColor
  (params (Team :type ETeam%20Enum :default "NatureTeam"))
  (return (Utilities|Select :Index Team :NatureTeam (Utilities|Struct|MakeSlateColor "(R=0.406250,G=0.406250,B=0.406250,A=1.000000)") :Team1 (Utilities|Struct|MakeSlateColor "(R=0.076185,G=0.230740,B=0.114435,A=1.000000)") :Team2 (Utilities|Struct|MakeSlateColor "(R=0.165132,G=0.584078,B=0.571125,A=1.000000)") :Team3 (Utilities|Struct|MakeSlateColor "(R=1.000000,G=0.479320,B=0.000000,A=1.000000)") :Team4 (Utilities|Struct|MakeSlateColor "(R=0.168269,G=0.040915,B=0.323143,A=1.000000)"))))

(fn GetNerrasTeamColor
  (params (Team :type ETeam%20Enum :default "NatureTeam"))
  (return (Utilities|Select :Index Team :NatureTeam (Utilities|Struct|MakeSlateColor "(R=0.406250,G=0.406250,B=0.406250,A=1.000000)") :Team1 (Utilities|Struct|MakeSlateColor "(R=0.116971,G=0.254152,B=0.109462,A=1.000000)") :Team2 (Utilities|Struct|MakeSlateColor "(R=0.337164,G=0.730461,B=1.000000,A=1.000000)") :Team3 (Utilities|Struct|MakeSlateColor "(R=0.300544,G=0.149960,B=0.051269,A=1.000000)") :Team4 (Utilities|Struct|MakeSlateColor "(R=0.351533,G=0.064803,B=0.356400,A=1.000000)"))))

(fn GetNerrasEmissColor
  (params (Team :type ETeam%20Enum :default "NatureTeam"))
  (return (Utilities|Select :Index Team :NatureTeam (Utilities|Struct|MakeSlateColor "(R=0.406250,G=0.406250,B=0.406250,A=1.000000)") :Team1 (Utilities|Struct|MakeSlateColor "(R=0.396755,G=1.000000,B=0.401978,A=1.000000)") :Team2 (Utilities|Struct|MakeSlateColor "(R=0.246201,G=0.672443,B=1.000000,A=1.000000)") :Team3 (Utilities|Struct|MakeSlateColor "(R=1.000000,G=0.520996,B=0.124772,A=1.000000)") :Team4 (Utilities|Struct|MakeSlateColor "(R=0.637597,G=0.291771,B=1.000000,A=1.000000)"))))

(fn GetOverlayTeamColor
  (params (TargetTeam :type ETeam%20Enum :default "NatureTeam") (YourTeam :type ETeam%20Enum :default "NatureTeam"))
  (LocalVariables|SetSelectedColor (Utilities|Select :Index TargetTeam :NatureTeam "/Game/_Draft/Philemon/MOI_BaseNature.MOI_BaseNature" :Team1 "/Game/_Draft/Philemon/MOI_Base_1.MOI_Base_1" :Team2 "/Game/_Draft/Philemon/MOI_Base_2.MOI_Base_2" :Team3 "/Game/_Draft/Philemon/MOI_Base_3.MOI_Base_3" :Team4 "/Game/_Draft/Philemon/MOI_Base_4.MOI_Base_4"))
  (if (Utilities|Enum|Equal(Enum) TargetTeam "NatureTeam")
    _
    (elif (Utilities|Enum|Equal(Enum) TargetTeam YourTeam)
      _
      (else
        (bind _output_get (LocalVariables|SetSelectedColor "/Game/_Draft/Philemon/MOI_Base_Hostile.MOI_Base_Hostile")))))
  (return _output_get))

(fn GetSaveGameObject
  (params (GameInstanceInfernale :type Game%20Instance%20Infernale%20Object%20Reference))
  (Class|GameInstanceInfernale|SetupPlayerSettings GameInstanceInfernale)
  (Utilities|IsValid (Variables|/Script/InfernaleTesting.GameInstanceInfernale|GetPlayerSettingSave GameInstanceInfernale)
    (:Is%20Valid
      (return (Variables|/Script/InfernaleTesting.GameInstanceInfernale|GetPlayerSettingSave GameInstanceInfernale)))
    (:Is%20Not%20Valid
      (bind _returnvalue (SaveGame|CreateSaveGameObject "/Script/InfernaleTesting.PlayerSettingSave"))
      (bind _output_get (Variables|/Script/InfernaleTesting.GameInstanceInfernale|SetPlayerSettingSave GameInstanceInfernale _returnvalue))
      (return _output_get))))

(fn PlayerInfotoText
  (params (PlayerInfo :type Player%20Info%20Structure))
  (bind (_playerid _playername _playerownerinfo _playercontroller _playerisready _isinroom) (Utilities|Struct|BreakPlayerInfo PlayerInfo))
  (bind (_player _team) (Utilities|Struct|BreakOwner _playerownerinfo))
  (return (Utilities|Text|FormatText "Player ID: {id} 
Player Name: {name} 
Player: {Player} 
Team: {Team} 
Ready ?: {Rdy} 
InRoom?: {Room}" _playerid _playername (Utilities|String|EnumtoString _player) (Utilities|String|EnumtoString _team) _playerisready _isinroom)))

(fn GetPlayerID
  (params (Index :type Integer))
  (return (Utilities|Select :Index Index :Option%200 "Player1" :Option%201 "Player2" :Option%202 "Player3" :Option%203 "Player4")))

(fn GetTeamID
  (params (Index :type Integer))
  (return (Utilities|Select :Index Index :Option%200 "Team1" :Option%201 "Team2" :Option%202 "Team3" :Option%203 "Team4")))