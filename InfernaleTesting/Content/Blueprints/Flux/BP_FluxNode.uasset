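; Blueprint for a flux node: the hoverable, selectable in-world marker for points on a player's Flux.
; NodeTypeRefresh sets mesh, team-colored dynamic materials and visibility by node type and team, retrying until the player's controller, state and team are ready.
; Hover and selection events drive sounds, cursor, scale, selection cone and owning Flux highlight.
; Two chained timelines bob the node and animate its glow, varying with Flux active state.
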(event Custom|Redraw
  (params (Target :type Flux%20Object%20Reference) (Condition :type Boolean))
  (bind _returnvalue (Class|Flux|GetOwnerInfo Target))
  (bind _returnvalue_2 (Game|GetPlayerController 0))
  (bind _nodevisual (Variables|Default|GetNodeVisual))
  (bind (_player _team) (Utilities|Struct|BreakOwner _returnvalue))
  (bind _asbp_player_controller_infernale (Utilities|Casting|CastToBP_PlayerControllerInfernale _returnvalue_2))
  (bind _relativelocation (Variables|/Script/Engine.SceneComponent|GetRelativeLocation _nodevisual))
  (bind (_x _y) (Math|Vector|BreakVector _relativelocation))
  (bind _playerstate (Variables|/Script/Engine.Controller|GetPlayerState _asbp_player_controller_infernale))
  (bind _asbp_player_state_infernale (Utilities|Casting|CastToBP_PlayerStateInfernale _playerstate))
  (bind _ownerinfo (Variables|/Script/InfernaleTesting.PlayerStateInfernale|GetOwnerInfo _asbp_player_state_infernale))
  (bind (_player_2 _team_2) (Utilities|Struct|BreakOwner _ownerinfo))
  ;[1 1 1] Redraw
  (CallFunction|CreateMaterials)
  (Variables|Default|SetIsFluxActive (Class|Flux|IsFluxActive Target))
  (Variables|Default|SetFluxTeam _team)
  (if Condition
    (if (and (Utilities|Enum|Equal(Enum) _player _player_2) (Utilities|Enum|Equal(Enum) _team _team_2))
      (Rendering|SetVisibility (Variables|Default|GetNodeVisual) (Utilities|Enum|NotEqual(Enum) (Variables|Default|GetFluxNodeType) "StartNode") false)
      (Transformation|SetRelativeLocation _nodevisual (Math|Vector|MakeVector _x _y (Variables|Default|GetHoverVisualOffset_Low)) false false)
      (Rendering|Material|SetVectorParameterValue (Variables|Default|GetPinMaterial) "TeamColor" (Variables|Default|GetPlayerColor) :!class /Script/Engine.MaterialInstanceDynamic)
      (else
        (Rendering|SetVisibility (Variables|Default|GetNodeVisual) false false)
        (Rendering|SetVisibility (Variables|Default|GetSelectedCone) false false)))
    (else
      (Rendering|SetVisibility (Variables|Transformation|GetRootComponent) false true)
      (Collision|SetCollisionEnabled (Variables|Default|GetCollisionSphereLow) "NoCollision")
      ;[1 1 1] Show/Hide FakeNodes
      (Rendering|SetVisibility (Variables|Default|GetCube) false false))))

(event Custom|NodeTypeRefresh
  (bind _nodevisual (Variables|Default|GetNodeVisual))
  (bind _nodevisual_2 (Variables|Default|GetNodeVisual))
  (bind _fluxowner (Variables|Default|GetFluxOwner))
  (bind _nodevisual_3 (Variables|Default|GetNodeVisual))
  ;[1 1 1] NodeTypeRefresh
  (CallFunction|CreateMaterials)
  (bind _asbp_player_controller_infernale (Utilities|Casting|CastToBP_PlayerControllerInfernale (Game|GetPlayerController 0) :!label _label)
    (:then
      (bind _asbp_player_state_infernale (Utilities|Casting|CastToBP_PlayerStateInfernale (Variables|/Script/Engine.Controller|GetPlayerState _asbp_player_controller_infernale) :!label _label_2)
        (:then
          (if (Utilities|Enum|NotEqual(Enum) (.Team (Utilities|Struct|BreakOwner (Variables|/Script/InfernaleTesting.PlayerStateInfernale|GetOwnerInfo _asbp_player_state_infernale))) "NatureTeam") :!label _label_3
            (if (Variables|Default|GetbIsReal)
              (switch Utilities|FlowControl|Switch|SwitchonEFluxNodeType (Variables|Default|GetFluxNodeType)
                (:None
                  (Rendering|SetVisibility (Variables|Default|GetNodeVisual) false false :!label _label_4))
                (:BaseNode
                  (goto _label_4))
                (:StartNode
                  (Components|StaticMesh|SetStaticMesh (Variables|Default|GetNodeVisual) "/Game/UI/Meshes/SM_StartPortal.SM_StartPortal")
                  (Rendering|SetVisibility _nodevisual false false)
                  (Transformation|SetRelativeScale3D _nodevisual (Variables|Default|GetBaseScale))
                  (CallFunction|VisualLoopUpDown)
                  (Rendering|Material|SetMaterial _nodevisual_2 0 "/Game/UI/Meshes/M_ArrowIcon_Center.M_ArrowIcon_Center" :!label _label_5)
                  (bind _returnvalue (Rendering|Material|CreateDynamicMaterialInstance _nodevisual_2 0 "/Game/UI/Meshes/M_ArrowIcon_Center.M_ArrowIcon_Center" "None" :!class /Script/Engine.PrimitiveComponent))
                  (bind _output_get (Variables|Default|SetPinMaterial _returnvalue))
                  (Rendering|Material|SetMaterial _nodevisual_2 1 "/Game/UI/Meshes/M_ArrowIcon_Flat.M_ArrowIcon_Flat")
                  (bind _returnvalue_2 (Rendering|Material|CreateDynamicMaterialInstance _nodevisual_2 1 "/Game/UI/Meshes/M_ArrowIcon_Flat.M_ArrowIcon_Flat" "None" :!class /Script/Engine.PrimitiveComponent))
                  (Utilities|IsValid _returnvalue_2
                    (:Is%20Valid
                      (bind _output_get_2 (Variables|Default|SetPin%20Material%201 _returnvalue_2)))
                    (:Is%20Not%20Valid
                      _))
                  (Rendering|Material|SetMaterial _nodevisual_2 2 "/Game/UI/Meshes/M_ArrowIcon.M_ArrowIcon")
                  (bind _returnvalue_3 (Rendering|Material|CreateDynamicMaterialInstance _nodevisual_2 2 "/Game/UI/Meshes/M_ArrowIcon.M_ArrowIcon" "None" :!class /Script/Engine.PrimitiveComponent))
                  (Utilities|IsValid _returnvalue_3
                    (:Is%20Valid
                      (bind _output_get_3 (Variables|Default|SetPin%20Material%202 _returnvalue_3)))
                    (:Is%20Not%20Valid
                      _))
                  (Rendering|Material|SetVectorParameterValue _output_get "TeamColor" (.SpecifiedColor (Utilities|Struct|BreakSlateColor (CallFunction|GetTeamColor (.Team (Utilities|Struct|BreakOwner (Variables|/Script/InfernaleTesting.PlayerStateInfernale|GetOwnerInfo _asbp_player_state_infernale)))))) :!class /Script/Engine.MaterialInstanceDynamic))
                (:EndNode
                  (Components|StaticMesh|SetStaticMesh (Variables|Default|GetNodeVisual) (Variables|Default|GetEndMesh))
                  (Rendering|SetVisibility _nodevisual_3 (Utilities|Enum|Equal(Enum) (.Team (Utilities|Struct|BreakOwner (Variables|/Script/InfernaleTesting.PlayerStateInfernale|GetOwnerInfo _asbp_player_state_infernale))) (.Team (Utilities|Struct|BreakOwner (Class|Flux|GetOwnerInfo _fluxowner)))) false)
                  (Transformation|SetRelativeScale3D _nodevisual_3 (Variables|Default|GetBaseScaleEnd))
                  (CallFunction|VisualLoopUpDown)
                  (goto _label_5))
                (:FakeNode
                  (goto _label_4))
                (:TmpNode
                  (Components|StaticMesh|SetStaticMesh (Variables|Default|GetNodeVisual) "/Game/UI/Meshes/SM_Arrowpoint.SM_Arrowpoint" :!label _label_6)
                  (Rendering|SetVisibility (Variables|Default|GetNodeVisual) (and (Class|Flux|IsFluxActive _fluxowner) (Utilities|Enum|Equal(Enum) (.Team (Utilities|Struct|BreakOwner (Variables|/Script/InfernaleTesting.PlayerStateInfernale|GetOwnerInfo _asbp_player_state_infernale))) (.Team (Utilities|Struct|BreakOwner (Class|Flux|GetOwnerInfo _fluxowner))))) false)
                  (CallFunction|VisualLoopUpDown)
                  (Rendering|Material|SetMaterial _nodevisual_2 0 "/Game/UI/Meshes/M_ArrowIcon_Center.M_ArrowIcon_Center")
                  (bind _returnvalue_4 (Rendering|Material|CreateDynamicMaterialInstance _nodevisual_2 0 "/Game/UI/Meshes/M_ArrowIcon_Center.M_ArrowIcon_Center" "None" :!class /Script/Engine.PrimitiveComponent))
                  (bind _output_get_4 (Variables|Default|SetPinMaterial _returnvalue_4))
                  (Rendering|Material|SetMaterial _nodevisual_2 1 "/Game/UI/Meshes/M_ArrowIcon_Flat.M_ArrowIcon_Flat")
                  (bind _returnvalue_5 (Rendering|Material|CreateDynamicMaterialInstance _nodevisual_2 1 "/Game/UI/Meshes/M_ArrowIcon_Flat.M_ArrowIcon_Flat" "None" :!class /Script/Engine.PrimitiveComponent))
                  (Utilities|IsValid _returnvalue_5
                    (:Is%20Valid
                      (bind _output_get_5 (Variables|Default|SetPin%20Material%201 _returnvalue_5)))
                    (:Is%20Not%20Valid
                      _))
                  (Rendering|Material|SetVectorParameterValue _output_get_4 "TeamColor" (.SpecifiedColor (Utilities|Struct|BreakSlateColor (CallFunction|GetTeamColor (.Team (Utilities|Struct|BreakOwner (Variables|/Script/InfernaleTesting.PlayerStateInfernale|GetOwnerInfo _asbp_player_state_infernale)))))) :!class /Script/Engine.MaterialInstanceDynamic))
                (:PathNode
                  (goto _label_6)))
              (else
                (goto _label_4)))
            (else
              (Utilities|FlowControl|Delay 0.1)
              (goto _label_3))))
        (:CastFailed
          (Utilities|FlowControl|Delay 0.1)
          (goto _label_2))))
    (:CastFailed
      (Utilities|FlowControl|Delay 0.1)
      (goto _label))))

(event Custom|PutNodeHigh
  (bind _fluxnodetype (Variables|Default|GetFluxNodeType))
  (bind _returnvalue (Utilities|Enum|NotEqual(Enum) _fluxnodetype "EndNode"))
  ;[1 1 1] PutNodeHigh
  (bind _scale (Timeline|Timeline_3 PlayFromStart)
    (:Update
      (Transformation|SetRelativeScale3D (Variables|Default|GetNodeVisual) (Math|Vector|Lerp(Vector) (Math|Vector|SelectVector (Variables|Default|GetBaseScale) (Variables|Default|GetBaseScaleEnd) _returnvalue) (Math|Vector|SelectVector (Variables|Default|GetHoverScale) (Variables|Default|GetHoverScaleEnd) _returnvalue) _scale)))))

(event Custom|PutNodeLow
  (bind _fluxnodetype (Variables|Default|GetFluxNodeType))
  (bind _returnvalue (Utilities|Enum|NotEqual(Enum) _fluxnodetype "EndNode"))
  ;[1 1 1] PutNodeLow
  (bind _scale (Timeline|Timeline_2 ReverseFromEnd)
    (:Update
      (Rendering|SetVisibility (Variables|Default|GetPlaneGroundCircle) true false)
      (Transformation|SetRelativeScale3D (Variables|Default|GetNodeVisual) (Math|Vector|Lerp(Vector) (Math|Vector|SelectVector (Variables|Default|GetBaseScale) (Variables|Default|GetBaseScaleEnd) _returnvalue) (Math|Vector|SelectVector (Variables|Default|GetHoverScale) (Variables|Default|GetHoverScaleEnd) _returnvalue) _scale)))))

(event Custom|VisualLoopUpDown
  (bind _isfluxactive (Variables|Default|GetIsFluxActive))
  (bind _isfluxactive_2 (Variables|Default|GetIsFluxActive))
  (bind _pin_material_2 (Variables|Default|GetPin%20Material%202))
  (bind _isfluxactive_3 (Variables|Default|GetIsFluxActive))
  (bind _pin_material_2_2 (Variables|Default|GetPin%20Material%202))
  (bind _isfluxactive_4 (Variables|Default|GetIsFluxActive))
  ;[1 1 1] LoopUpDown
  (bind _scale (Timeline|Timeline_0 PlayFromStart)
    (:Update
      (if (Variables|Default|GetHovered)
        (Variables|Default|SetUpOrDown true)
        (Timeline|Timeline_0 Stop)
        (else
          (Transformation|SetRelativeLocation (Variables|Default|GetCollisionSphereHigh) (Math|Vector|Lerp(Vector) "0.000000,0.000000,400.000000" (Math|Vector|SelectVector "0.000000,0.000000,600.000000" "0.000000,0.000000,700.000000" _isfluxactive) _scale) false false)
          (Rendering|Material|SetScalarParameterValue (Variables|Default|GetPinMaterial) "Desaturation" (Math|Float|SelectFloat 0.5 (Math|Float|Lerp 0.4 -0.2 _scale) _isfluxactive_4) :!class /Script/Engine.MaterialInstanceDynamic)
          (Utilities|IsValid _pin_material_2_2
            (:Is%20Valid
              (Rendering|Material|SetScalarParameterValue _pin_material_2_2 "Intensity" (Math|Float|SelectFloat 6.0 (Math|Float|Lerp 2e+01 4.0 _scale) _isfluxactive_2) :!class /Script/Engine.MaterialInstanceDynamic)
              (Rendering|Material|SetScalarParameterValue (Variables|Default|GetPinMaterial) "Brightness" (Math|Float|SelectFloat 1.5 (Math|Float|Lerp 5.0 0.1 _scale) _isfluxactive_3) :!class /Script/Engine.MaterialInstanceDynamic))))))
    (:Finished
      (bind _scale_2 (Timeline|Timeline_1 ReverseFromEnd)
        (:Update
          (if (Variables|Default|GetHovered)
            (Variables|Default|SetUpOrDown false)
            (Timeline|Timeline_1 Stop)
            (else
              (Transformation|SetRelativeLocation (Variables|Default|GetCollisionSphereHigh) (Math|Vector|Lerp(Vector) "0.000000,0.000000,400.000000" (Math|Vector|SelectVector "0.000000,0.000000,600.000000" "0.000000,0.000000,700.000000" _isfluxactive) _scale_2) false false)
              (Rendering|Material|SetScalarParameterValue (Variables|Default|GetPinMaterial) "Desaturation" (Math|Float|SelectFloat 0.5 (Math|Float|Lerp 0.4 -0.2 _scale_2) _isfluxactive_4) :!class /Script/Engine.MaterialInstanceDynamic)
              (Utilities|IsValid _pin_material_2
                (:Is%20Valid
                  (Rendering|Material|SetScalarParameterValue _pin_material_2 "Intensity" (Math|Float|SelectFloat 6.0 (Math|Float|Lerp 2e+01 4.0 _scale_2) _isfluxactive_2) :!class /Script/Engine.MaterialInstanceDynamic)
                  (Rendering|Material|SetScalarParameterValue (Variables|Default|GetPinMaterial) "Brightness" (Math|Float|SelectFloat 1.5 (Math|Float|Lerp 5.0 0.1 _scale_2) _isfluxactive_3) :!class /Script/Engine.MaterialInstanceDynamic))))))
        (:Finished
          (Timeline|Timeline_0 PlayFromStart))))))

(event Custom|CreateMaterials
  ;[1 1 1] BeginPlay
  (if (not (Variables|Default|GetMaterialCreated))
    (bind _returnvalue (Rendering|Material|CreateDynamicMaterialInstance (Variables|Default|GetNodeVisual) 0 "/Game/UI/Materials/MI_Pin.MI_Pin" "None" :!class /Script/Engine.PrimitiveComponent))
    (Variables|Default|SetPinMaterial _returnvalue)
    (bind _returnvalue_2 (Rendering|Material|CreateDynamicMaterialInstance (Variables|Default|GetPlaneGroundCircle) 0 "/Game/_Draft/Benjamin/M_GroundIndicatorMaterial.M_GroundIndicatorMaterial" "None" :!class /Script/Engine.PrimitiveComponent))
    (Variables|Default|SetGround%20Radius%20Material _returnvalue_2)
    (Variables|Default|SetMaterialCreated true)))

(event Custom|ResumeUpDown
  (bind _isfluxactive (Variables|Default|GetIsFluxActive))
  (bind _isfluxactive_2 (Variables|Default|GetIsFluxActive))
  (bind _pin_material_2 (Variables|Default|GetPin%20Material%202))
  (bind _isfluxactive_3 (Variables|Default|GetIsFluxActive))
  (bind _pin_material_2_2 (Variables|Default|GetPin%20Material%202))
  (bind _isfluxactive_4 (Variables|Default|GetIsFluxActive))
  ;[1 1 1] LoopUpDown
  (if (Variables|Default|GetUpOrDown)
    (bind _scale (Timeline|Timeline_0 Play)
      (:Update
        (if (Variables|Default|GetHovered)
          (Variables|Default|SetUpOrDown true)
          (Timeline|Timeline_0 Stop)
          (else
            (Transformation|SetRelativeLocation (Variables|Default|GetCollisionSphereHigh) (Math|Vector|Lerp(Vector) "0.000000,0.000000,400.000000" (Math|Vector|SelectVector "0.000000,0.000000,600.000000" "0.000000,0.000000,700.000000" _isfluxactive) _scale) false false)
            (Rendering|Material|SetScalarParameterValue (Variables|Default|GetPinMaterial) "Desaturation" (Math|Float|SelectFloat 0.5 (Math|Float|Lerp 0.4 -0.2 _scale) _isfluxactive_4) :!class /Script/Engine.MaterialInstanceDynamic)
            (Utilities|IsValid _pin_material_2_2
              (:Is%20Valid
                (Rendering|Material|SetScalarParameterValue _pin_material_2_2 "Intensity" (Math|Float|SelectFloat 6.0 (Math|Float|Lerp 2e+01 4.0 _scale) _isfluxactive_2) :!class /Script/Engine.MaterialInstanceDynamic)
                (Rendering|Material|SetScalarParameterValue (Variables|Default|GetPinMaterial) "Brightness" (Math|Float|SelectFloat 1.5 (Math|Float|Lerp 5.0 0.1 _scale) _isfluxactive_3) :!class /Script/Engine.MaterialInstanceDynamic))))))
      (:Finished
        (bind _scale_2 (Timeline|Timeline_1 ReverseFromEnd)
          (:Update
            (if (Variables|Default|GetHovered)
              (Variables|Default|SetUpOrDown false)
              (Timeline|Timeline_1 Stop)
              (else
                (Transformation|SetRelativeLocation (Variables|Default|GetCollisionSphereHigh) (Math|Vector|Lerp(Vector) "0.000000,0.000000,400.000000" (Math|Vector|SelectVector "0.000000,0.000000,600.000000" "0.000000,0.000000,700.000000" _isfluxactive) _scale_2) false false)
                (Rendering|Material|SetScalarParameterValue (Variables|Default|GetPinMaterial) "Desaturation" (Math|Float|SelectFloat 0.5 (Math|Float|Lerp 0.4 -0.2 _scale_2) _isfluxactive_4) :!class /Script/Engine.MaterialInstanceDynamic)
                (Utilities|IsValid _pin_material_2
                  (:Is%20Valid
                    (Rendering|Material|SetScalarParameterValue _pin_material_2 "Intensity" (Math|Float|SelectFloat 6.0 (Math|Float|Lerp 2e+01 4.0 _scale_2) _isfluxactive_2) :!class /Script/Engine.MaterialInstanceDynamic)
                    (Rendering|Material|SetScalarParameterValue (Variables|Default|GetPinMaterial) "Brightness" (Math|Float|SelectFloat 1.5 (Math|Float|Lerp 5.0 0.1 _scale_2) _isfluxactive_3) :!class /Script/Engine.MaterialInstanceDynamic))))))
          (:Finished
            (Timeline|Timeline_0 PlayFromStart)))))
    (else
      (Timeline|Timeline_1 Reverse))))

(event EventBeginPlay
  ;[1 1 1] BeginPlay
  (Rendering|SetVisibility (Variables|Default|GetSelectedCone) false false)
  (CallFunction|CreateMaterials)
  (bind _asbp_player_controller_infernale (Utilities|Casting|CastToBP_PlayerControllerInfernale (Game|GetPlayerController 0) :!label _label)
    (:then
      (bind _asbp_player_state_infernale (Utilities|Casting|CastToBP_PlayerStateInfernale (Variables|/Script/Engine.Controller|GetPlayerState _asbp_player_controller_infernale) :!label _label_2)
        (:then
          (if (Utilities|Enum|NotEqual(Enum) (.Team (Utilities|Struct|BreakOwner (Variables|/Script/InfernaleTesting.PlayerStateInfernale|GetOwnerInfo _asbp_player_state_infernale))) "NatureTeam") :!label _label_3
            (bind _output_get (Variables|Default|SetPlayerColor (.SpecifiedColor (Utilities|Struct|BreakSlateColor (CallFunction|GetTeamColor (.Team (Utilities|Struct|BreakOwner (Variables|/Script/InfernaleTesting.PlayerStateInfernale|GetOwnerInfo _asbp_player_state_infernale))))))))
            (Rendering|Material|SetVectorParameterValue (Variables|Default|GetGround%20Radius%20Material) "TeamColor" _output_get :!class /Script/Engine.MaterialInstanceDynamic)
            (CallFunction|NodeTypeRefresh)
            (else
              (Utilities|FlowControl|Delay 0.1)
              (goto _label_3))))
        (:CastFailed
          (Utilities|FlowControl|Delay 0.1)
          (goto _label_2))))
    (:CastFailed
      (Utilities|FlowControl|Delay 0.1)
      (goto _label))))

(event EventOnSelectedforFlux
  ;[1 1 1] (De)Selected for flux
  (Rendering|SetVisibility (Variables|Default|GetSelectedCone) true false)
  (if (Utilities|Enum|Equal(Enum) (Variables|Default|GetFluxNodeType) "EndNode")
    (bind _output_get (Variables|Default|SetSFX_Select "Creating"))
    (else
      (Variables|Default|SetSFX_Select "Edit")))
  (Class|SoundsDataAsset|PlaySound (Utilities|GetSoundDataAsset) "Flux" (Utilities|String|Append "Start " _output_get " Flux") (Transformation|GetActorLocation))
  (Rendering|Material|SetScalarParameterValue (Variables|Default|GetPinMaterial) "IsHovered" 1.0 :!class /Script/Engine.MaterialInstanceDynamic)
  (Variables|Default|SetIsFluxActive (Class|Flux|IsFluxActive (Variables|Default|GetFluxReference))))

(event EventNodeInitBP
  (params (Flux :type Flux%20Object%20Reference) (IsReal :type Boolean))
  ;[1 1 1] NodeInitBP
  (bind _output_get (Variables|Default|SetFluxReference Flux))
  (CallFunction|Redraw _output_get IsReal)
  (CallFunction|NodeTypeRefresh))

(event EventOnDeselectedforFlux
  ;[1 1 1] (De)Selected for flux
  (Rendering|SetVisibility (Variables|Default|GetSelectedCone) false false)
  (if (Utilities|Enum|Equal(Enum) (Variables|Default|GetFluxNodeType) "EndNode")
    (bind _output_get (Variables|Default|SetSFX_Select "Creating"))
    (else
      (Variables|Default|SetSFX_Select "Edit")))
  (Class|SoundsDataAsset|PlaySound (Utilities|GetSoundDataAsset) "Flux" (Utilities|String|Append "Finish " _output_get " Flux") (Transformation|GetActorLocation))
  (Rendering|Material|SetScalarParameterValue (Variables|Default|GetPinMaterial) "IsHovered" 0.0 :!class /Script/Engine.MaterialInstanceDynamic)
  (Variables|Default|SetIsFluxActive (Class|Flux|IsFluxActive (Variables|Default|GetFluxReference))))

(event EventOnHovered
  ;[1 1 1] Hovered
  (Variables|Default|SetHovered true)
  (Class|SoundsDataAsset|PlaySound (.soundsassets (Utilities|Array|Get(acopy) (Variables|/Script/InfernaleTesting.GameSettingsDataAsset|GetDataAssetsSettings (Class|FunctionLibraryInfernale|GetGameSettingsDataAsset)))) "Flux" "Hover FluxNode" (Transformation|GetActorLocation))
  (Default|SetCursorModeCustom (Variables|/Game/Blueprints/GameMode/Infernale/BP_PlayerControllerInfernale.BP_PlayerControllerInfernale_C|GetBP_UIComponent (.AsBP%20Player%20Controller%20Infernale (Utilities|Casting|CastToBP_PlayerControllerInfernale (Game|GetPlayerController 0)))) "Hand")
  (Class|SoundsDataAsset|PlaySound (Utilities|GetSoundDataAsset) "Flux" "Hover FluxNode" (Transformation|GetActorLocation))
  (CallFunction|PutNodeHigh)
  (Rendering|Material|SetScalarParameterValue (Variables|Default|GetPinMaterial) "IsHovered" 1.0 :!class /Script/Engine.MaterialInstanceDynamic)
  (Default|SimpleHoverFlux (.AsBP%20Flux (Utilities|Casting|CastToBP_Flux (Variables|Default|GetFluxOwner))))
  ;[1 1 1] Unhover
  (Utilities|IsValid (Variables|Default|GetPin%20Material%201)
    (:Is%20Valid
      (Utilities|IsValid (Variables|Default|GetPin%20Material%202)
        (:Is%20Valid
          (Rendering|Material|SetVectorParameterValue (Variables|Default|GetPinMaterial) "TeamColor" (Variables|Default|GetPlayerColor) :!class /Script/Engine.MaterialInstanceDynamic))
        (:Is%20Not%20Valid
          _)))
    (:Is%20Not%20Valid
      _))
  (CallFunction|ResumeUpDown))

(event EventOnUnHovered
  ;[1 1 1] Unhover
  (Variables|Default|SetHovered false)
  (Default|SetCursorModeCustom (Variables|/Game/Blueprints/GameMode/Infernale/BP_PlayerControllerInfernale.BP_PlayerControllerInfernale_C|GetBP_UIComponent (.AsBP%20Player%20Controller%20Infernale (Utilities|Casting|CastToBP_PlayerControllerInfernale (Game|GetPlayerController 0)))) "Default")
  (CallFunction|PutNodeLow)
  (Rendering|Material|SetScalarParameterValue (Variables|Default|GetPinMaterial) "IsHovered" 0.0 :!class /Script/Engine.MaterialInstanceDynamic)
  (Default|SimpleUnHoverFLux (.AsBP%20Flux (Utilities|Casting|CastToBP_Flux (Variables|Default|GetFluxOwner))))
  (Utilities|IsValid (Variables|Default|GetPin%20Material%201)
    (:Is%20Valid
      (Utilities|IsValid (Variables|Default|GetPin%20Material%202)
        (:Is%20Valid
          (Rendering|Material|SetVectorParameterValue (Variables|Default|GetPinMaterial) "TeamColor" (Variables|Default|GetPlayerColor) :!class /Script/Engine.MaterialInstanceDynamic))
        (:Is%20Not%20Valid
          _)))
    (:Is%20Not%20Valid
      _))
  (CallFunction|ResumeUpDown))

(event EventNodeTypeUpdatedBP
  (bind _nodevisual (Variables|Default|GetNodeVisual))
  (bind _nodevisual_2 (Variables|Default|GetNodeVisual))
  (bind _fluxowner (Variables|Default|GetFluxOwner))
  (bind _nodevisual_3 (Variables|Default|GetNodeVisual))
  ;[1 1 1] NodeTypeRefresh
  (CallFunction|CreateMaterials)
  (bind _asbp_player_controller_infernale (Utilities|Casting|CastToBP_PlayerControllerInfernale (Game|GetPlayerController 0) :!label _label)
    (:then
      (bind _asbp_player_state_infernale (Utilities|Casting|CastToBP_PlayerStateInfernale (Variables|/Script/Engine.Controller|GetPlayerState _asbp_player_controller_infernale) :!label _label_2)
        (:then
          (if (Utilities|Enum|NotEqual(Enum) (.Team (Utilities|Struct|BreakOwner (Variables|/Script/InfernaleTesting.PlayerStateInfernale|GetOwnerInfo _asbp_player_state_infernale))) "NatureTeam") :!label _label_3
            (if (Variables|Default|GetbIsReal)
              (switch Utilities|FlowControl|Switch|SwitchonEFluxNodeType (Variables|Default|GetFluxNodeType)
                (:None
                  (Rendering|SetVisibility (Variables|Default|GetNodeVisual) false false :!label _label_4))
                (:BaseNode
                  (goto _label_4))
                (:StartNode
                  (Components|StaticMesh|SetStaticMesh (Variables|Default|GetNodeVisual) "/Game/UI/Meshes/SM_StartPortal.SM_StartPortal")
                  (Rendering|SetVisibility _nodevisual false false)
                  (Transformation|SetRelativeScale3D _nodevisual (Variables|Default|GetBaseScale))
                  (CallFunction|VisualLoopUpDown)
                  (Rendering|Material|SetMaterial _nodevisual_2 0 "/Game/UI/Meshes/M_ArrowIcon_Center.M_ArrowIcon_Center" :!label _label_5)
                  (bind _returnvalue (Rendering|Material|CreateDynamicMaterialInstance _nodevisual_2 0 "/Game/UI/Meshes/M_ArrowIcon_Center.M_ArrowIcon_Center" "None" :!class /Script/Engine.PrimitiveComponent))
                  (bind _output_get (Variables|Default|SetPinMaterial _returnvalue))
                  (Rendering|Material|SetMaterial _nodevisual_2 1 "/Game/UI/Meshes/M_ArrowIcon_Flat.M_ArrowIcon_Flat")
                  (bind _returnvalue_2 (Rendering|Material|CreateDynamicMaterialInstance _nodevisual_2 1 "/Game/UI/Meshes/M_ArrowIcon_Flat.M_ArrowIcon_Flat" "None" :!class /Script/Engine.PrimitiveComponent))
                  (Utilities|IsValid _returnvalue_2
                    (:Is%20Valid
                      (bind _output_get_2 (Variables|Default|SetPin%20Material%201 _returnvalue_2)))
                    (:Is%20Not%20Valid
                      _))
                  (Rendering|Material|SetMaterial _nodevisual_2 2 "/Game/UI/Meshes/M_ArrowIcon.M_ArrowIcon")
                  (bind _returnvalue_3 (Rendering|Material|CreateDynamicMaterialInstance _nodevisual_2 2 "/Game/UI/Meshes/M_ArrowIcon.M_ArrowIcon" "None" :!class /Script/Engine.PrimitiveComponent))
                  (Utilities|IsValid _returnvalue_3
                    (:Is%20Valid
                      (bind _output_get_3 (Variables|Default|SetPin%20Material%202 _returnvalue_3)))
                    (:Is%20Not%20Valid
                      _))
                  (Rendering|Material|SetVectorParameterValue _output_get "TeamColor" (.SpecifiedColor (Utilities|Struct|BreakSlateColor (CallFunction|GetTeamColor (.Team (Utilities|Struct|BreakOwner (Variables|/Script/InfernaleTesting.PlayerStateInfernale|GetOwnerInfo _asbp_player_state_infernale)))))) :!class /Script/Engine.MaterialInstanceDynamic))
                (:EndNode
                  (Components|StaticMesh|SetStaticMesh (Variables|Default|GetNodeVisual) (Variables|Default|GetEndMesh))
                  (Rendering|SetVisibility _nodevisual_3 (Utilities|Enum|Equal(Enum) (.Team (Utilities|Struct|BreakOwner (Variables|/Script/InfernaleTesting.PlayerStateInfernale|GetOwnerInfo _asbp_player_state_infernale))) (.Team (Utilities|Struct|BreakOwner (Class|Flux|GetOwnerInfo _fluxowner)))) false)
                  (Transformation|SetRelativeScale3D _nodevisual_3 (Variables|Default|GetBaseScaleEnd))
                  (CallFunction|VisualLoopUpDown)
                  (goto _label_5))
                (:FakeNode
                  (goto _label_4))
                (:TmpNode
                  (Components|StaticMesh|SetStaticMesh (Variables|Default|GetNodeVisual) "/Game/UI/Meshes/SM_Arrowpoint.SM_Arrowpoint" :!label _label_6)
                  (Rendering|SetVisibility (Variables|Default|GetNodeVisual) (and (Class|Flux|IsFluxActive _fluxowner) (Utilities|Enum|Equal(Enum) (.Team (Utilities|Struct|BreakOwner (Variables|/Script/InfernaleTesting.PlayerStateInfernale|GetOwnerInfo _asbp_player_state_infernale))) (.Team (Utilities|Struct|BreakOwner (Class|Flux|GetOwnerInfo _fluxowner))))) false)
                  (CallFunction|VisualLoopUpDown)
                  (Rendering|Material|SetMaterial _nodevisual_2 0 "/Game/UI/Meshes/M_ArrowIcon_Center.M_ArrowIcon_Center")
                  (bind _returnvalue_4 (Rendering|Material|CreateDynamicMaterialInstance _nodevisual_2 0 "/Game/UI/Meshes/M_ArrowIcon_Center.M_ArrowIcon_Center" "None" :!class /Script/Engine.PrimitiveComponent))
                  (bind _output_get_4 (Variables|Default|SetPinMaterial _returnvalue_4))
                  (Rendering|Material|SetMaterial _nodevisual_2 1 "/Game/UI/Meshes/M_ArrowIcon_Flat.M_ArrowIcon_Flat")
                  (bind _returnvalue_5 (Rendering|Material|CreateDynamicMaterialInstance _nodevisual_2 1 "/Game/UI/Meshes/M_ArrowIcon_Flat.M_ArrowIcon_Flat" "None" :!class /Script/Engine.PrimitiveComponent))
                  (Utilities|IsValid _returnvalue_5
                    (:Is%20Valid
                      (bind _output_get_5 (Variables|Default|SetPin%20Material%201 _returnvalue_5)))
                    (:Is%20Not%20Valid
                      _))
                  (Rendering|Material|SetVectorParameterValue _output_get_4 "TeamColor" (.SpecifiedColor (Utilities|Struct|BreakSlateColor (CallFunction|GetTeamColor (.Team (Utilities|Struct|BreakOwner (Variables|/Script/InfernaleTesting.PlayerStateInfernale|GetOwnerInfo _asbp_player_state_infernale)))))) :!class /Script/Engine.MaterialInstanceDynamic))
                (:PathNode
                  (goto _label_6)))
              (else
                (goto _label_4)))
            (else
              (Utilities|FlowControl|Delay 0.1)
              (goto _label_3))))
        (:CastFailed
          (Utilities|FlowControl|Delay 0.1)
          (goto _label_2))))
    (:CastFailed
      (Utilities|FlowControl|Delay 0.1)
      (goto _label))))

(event EventSetNodeVisibilityBP
  (params (bVisible :type Boolean))
  ;[1 1 1] SetNodeVisibilityBP
  (Rendering|SetVisibility (Variables|Default|GetNodeVisual) bVisible false))

(event EventEnableCollisionsBP
  (params (bEnabled :type Boolean))
  ;[1 1 1] EnableCollisionsBP
  (Collision|SetCollisionEnabled (Variables|Default|GetCollisionSphereLow) (select bEnabled "QueryOnly" "NoCollision")))

(event EventRefreshNodeVisibilityBP
  (params (NewVisibility :type Boolean))
  ;[1 1 1] Event Refresh Node Visibility BP
  (CallFunction|NodeTypeRefresh)
  (if NewVisibility
    (Rendering|SetVisibility (Variables|Default|GetNodeVisual) (Utilities|Enum|NotEqual(Enum) (Variables|Default|GetFluxNodeType) "StartNode") false)
    (else
      (Rendering|SetVisibility (Variables|Default|GetNodeVisual) false false)
      (Rendering|SetVisibility (Variables|Default|GetSelectedCone) false false))))

(fn ConstructionScript)