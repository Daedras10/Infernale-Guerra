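; Strategic view component intended to react to domination, power and souls layer changes from the strategic view UI.
; On BeginPlay it retries every 0.2 seconds until the player controller's UI component has a valid UIStrategicView.
; The following sequence is empty, and the nodes binding the three layer-change events are disconnected, so they never run.
; The three handlers are placeholders that only print debug strings.
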(event Custom|Bind
  (Utilities|IsValid (Variables|/Game/Blueprints/Component/PlayerController/BP_UIComponent.BP_UIComponent_C|GetUIStrategicView (Actor|GetComponentbyClass (Game|GetPlayerController 0) "/Game/Blueprints/Component/PlayerController/BP_UIComponent.BP_UIComponent_C"))
    (:Is%20Valid
      (Utilities|FlowControl|Sequence))
    (:Is%20Not%20Valid
      (Utilities|FlowControl|Delay 0.2)
      (CallFunction|Bind))))

(event Custom|DisplayDominationInfo
  (Development|PrintString "Domination Info"))

(event Custom|DisplayPowerInfo
  (Development|PrintString "Power Info"))

(event Custom|DisplaySoulsInfo
  (Development|PrintString "Souls Info"))

(event EventBeginPlay
  (CallFunction|Bind))