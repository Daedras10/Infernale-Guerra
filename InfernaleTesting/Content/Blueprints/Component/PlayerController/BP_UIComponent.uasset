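; Player controller component that creates and manages the local player's UI, from HUD and menus to transmutation tree, end screen and cursors.
; BeginPlay retries until controller and player state are ready, then builds the widgets and gathers world widgets from buildings, bosses and camps.
; Events forward game state to those widgets, while Tick manually advances transmutation nodes, popups and notifications.
; A global visibility switch saves and restores each widget's previous state.
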(event Custom|CreateDebugHUD
  (bind _returnvalue (Game|GetGameInstance))
  (bind _bp_player_state_infernale (Variables|Default|GetBP%20Player%20State%20Infernale))
  (bind _asbp_game_instance_infernale (Utilities|Casting|CastToBP_GameInstanceInfernale _returnvalue))
  ;[1 1 1] CreateDebugHUD
  (bind _returnvalue_2 (UserInterface|CreateWidget "/Game/UI/InGame/WBP_DebugHUD.WBP_DebugHUD_C" (Variables|Default|GetPlayerControllerInfernale)))
  (bind _output_get (Variables|Default|SetHUD%20Widget _returnvalue_2))
  (UserInterface|Viewport|AddtoViewport _output_get 0)
  (Default|Init _output_get _bp_player_state_infernale)
  (Default|SetPC (Variables|Default|GetHUD%20Widget) (Variables|Default|GetBP%20Player%20Controller%20Infernale))
  (bind _returnvalue_3 (Class|GameInstanceInfernale|GetCustomGameMode _asbp_game_instance_infernale))
  (if (or (== _returnvalue_3 3) (not (Variables|/Script/InfernaleTesting.GameInstanceInfernale|GetbIsPhilosophicallyAccurateGame _asbp_game_instance_infernale)))
    (Default|ResetReadyState _asbp_game_instance_infernale)
    (Widget|SetVisibility (Variables|Default|GetHUD%20Widget) "Hidden")
    (bind _returnvalue_4 (UserInterface|CreateWidget "/Game/UI/InGame/WBP_HUDSandBox.WBP_HUDSandBox_C" (Variables|Default|GetPlayerControllerInfernale)))
    (bind _output_get_2 (Variables|Default|SetHUD%20Sandbox _returnvalue_4))
    (UserInterface|Viewport|AddtoViewport _output_get_2 0)
    (Default|Init _output_get_2 _bp_player_state_infernale)
    (Default|SetPC _output_get_2 (Variables|Default|GetBP%20Player%20Controller%20Infernale))))

(event Custom|CreateWidgets
  ;[1 1 1] CreateWidgets
  (CallFunction|CreateDebugHUD)
  (CallFunction|CreateGameElements)
  (CallFunction|CreateBreachUI)
  (CallFunction|CreateTooltip)
  (CallFunction|CreateDraftUI)
  (CallFunction|CreateEndGame)
  (CallFunction|CreateStratgicView)
  (CallFunction|CreateNotificationTray)
  (CallFunction|CreateConstructionMenu)
  (CallFunction|CreateCursorWidgets)
  (CallFunction|CreateOptionsMenu)
  (CallFunction|CreateCloseAll)
  (CallFunction|CreateNvidiaWidget))

(event Custom|Create%20TransmutationTree
  (params (TransmutationNodesOwned :type Array%20of%20Transmutation%20Node%20Owned%20Structures) (TransmutationNodesSettings :type Transmutation%20Settings%20Structure))
  ;[1 1 1] CreateTransmutationTree
  (bind _returnvalue (UserInterface|CreateWidget "/Game/UI/InGame/Transmutation/WBP_TransmutationTree.WBP_TransmutationTree_C" (Variables|Default|GetPlayerControllerInfernale)))
  (bind _output_get (Variables|Default|SetWBP%20TransmutationTree _returnvalue))
  (Default|Init _output_get TransmutationNodesOwned TransmutationNodesSettings self)
  (UserInterface|Viewport|AddtoViewport _output_get 10)
  (Widget|SetVisibility _output_get "Hidden"))

(event Custom|CreateStratgicView
  ;[1 1 1] StrategicView
  (bind _returnvalue (UserInterface|CreateWidget "/Game/UI/InGame/WBP_StrategicView.WBP_StrategicView_C" (Variables|Default|GetBP%20Player%20Controller%20Infernale)))
  (bind _output_get (Variables|Default|SetUIStrategicView _returnvalue))
  (Default|Init _output_get)
  (UserInterface|Viewport|AddtoViewport _returnvalue 0))

(event Custom|CreateConstructionMenu
  ;[1 1 1] CreateConstructionMenu
  (bind _returnvalue (UserInterface|CreateWidget "/Game/UI/BuildingMenu/WBP_BuildingMenu.WBP_BuildingMenu_C" (Variables|Default|GetBP%20Player%20Controller%20Infernale)))
  (bind _output_get (Variables|Default|SetConstructionMenu _returnvalue))
  (UserInterface|Viewport|AddtoViewport _output_get 1)
  (Widget|SetVisibility _output_get "Hidden"))

(event Custom|Create%20Notification%20Tray
  ;[1 1 1] Notification Tray
  (bind _returnvalue (UserInterface|CreateWidget "/Game/UI/InGame/WBP_NotificationTray.WBP_NotificationTray_C" (Variables|Default|GetBP%20Player%20Controller%20Infernale)))
  (bind _output_get (Variables|Default|SetNotificationTray _returnvalue))
  (UserInterface|Viewport|AddtoViewport _output_get 0))

(event Custom|CreateCursorWidgets
  ;[1 1 1] CreateCursorWidgets
  (bind _returnvalue (UserInterface|CreateWidget "/Game/UI/InGame/Cursor/WBP_Cursor_Main.WBP_Cursor_Main_C"))
  (bind _output_get (Variables|Default|SetCursorMain _returnvalue))
  (Class|PlayerController|SetMouseCursorWidget (Variables|Default|GetPlayerControllerInfernale) "Default" _output_get)
  (bind _returnvalue_2 (UserInterface|CreateWidget "/Game/UI/InGame/Cursor/WBP_Cursor_Hovering.WBP_Cursor_Hovering_C"))
  (bind _output_get_2 (Variables|Default|SetCursorHovering _returnvalue_2))
  (Class|PlayerController|SetMouseCursorWidget (Variables|Default|GetPlayerControllerInfernale) "Hand" _output_get_2))

(event Custom|ShowConstructionMenu
  (params (Show :type Boolean) (MainBuilding :type Main%20Building%20Object%20Reference))
  (bind _constructionmenu (Variables|Default|GetConstructionMenu))
  ;[1 1 1] ShowConstructionMenu
  (if (not (Variables|Default|GetisHiddenForStart))
    (Class|UIComponent|SetConstructionMenuVisible Show)
    (Default|SetBuildingMode (Variables|Default|GetWBP_CloseAll) Show)
    (Widget|SetVisibility (Variables|Default|GetConstructionMenu) (select Show "SelfHitTestInvisible" "Hidden"))
    (if Show
      (Default|Init _constructionmenu MainBuilding)
      (Class|SoundsDataAsset|PlaySound (.soundsassets (Utilities|Array|Get(acopy) (Variables|/Script/InfernaleTesting.GameSettingsDataAsset|GetDataAssetsSettings (Class|FunctionLibraryInfernale|GetGameSettingsDataAsset)))) "Building" "Open Building Menu/Select Base" (Transformation|GetActorLocation (Game|Player|GetPlayerPawn 0)))
      (else
        (Default|Closed _constructionmenu)))))

(event Custom|SetCursorModeCustom
  (params (Cursor :type EMouseCursor%20Enum :default "None"))
  (Class|PlayerController|SetMouseCursorWidget (Variables|Default|GetPlayerControllerInfernale) "Default" (Utilities|Select :Index Cursor :None 0 :Default (Variables|Default|GetCursorMain) :TextEditBeam 0 :ResizeLeftRight 0 :ResizeUpDown 0 :ResizeSouthEast 0 :ResizeSouthWest 0 :CardinalCross 0 :Crosshairs 0 :Hand (Variables|Default|GetCursorHovering) :GrabHand 0 :GrabHandClosed 0 :SlashedCircle 0 :EyeDropper 0)))

(event Custom|SwitchVisibilityOfAllWidgets
  (params (Show :type Boolean) (AtStart :type Boolean))
  (bind _visibilitystates (Variables|Default|GetVisibilityStates))
  ;[1 0 0.8268] SwitchVisibilityOfAllWidgets
  (if AtStart
    (Variables|Default|SetisHiddenForStart (not (Variables|Default|GetisHiddenForStart)))
    (bind _output_get (Variables|Default|SetWidgetsArray (Utilities|Array|MakeArray (Variables|Default|GetHUD%20Widget) (Variables|Default|GetGameElements) (Variables|Default|GetBreachUI) (Variables|Default|GetWBP%20TransmutationTree) (Variables|Default|GetWBP_Tooltip) (Variables|Default|GetUIDraft) (Variables|Default|GetWBP_EndGame) (Variables|Default|GetUIStrategicView) (Variables|Default|GetUIStrategicView) (Variables|Default|GetNotificationTray) (Variables|Default|GetConstructionMenu) (Variables|Default|GetCursorMain) (Variables|Default|GetCursorHovering) (Variables|Default|GetHUD%20Sandbox) (Variables|Default|GetOptionsMenu)) :!label _label))
    (for _array_element _output_get
      (Utilities|IsValid _array_element
        (:Is%20Not%20Valid
          (Utilities|Array|RemoveItem (Variables|Default|GetWidgetsArray) _array_element))))
    (for _array_element_2 (Variables|Default|GetPopUps)
      (Utilities|Array|Add (Variables|Default|GetWidgetsArray) _array_element_2))
    (for _array_element_3 (Variables|Default|GetBuildingWidgets)
      (Utilities|Array|Add (Variables|Default|GetWidgetsArray) _array_element_3))
    (if Show
      (for _array_element_4 (Variables|Default|GetWidgetsArray)
        (Utilities|IsValid _array_element_4
          (:Is%20Valid
            (if (.ReturnValue (Utilities|Map|Find _visibilitystates _array_element_4))
              (Widget|SetVisibility _array_element_4 (.Value (Utilities|Map|Find _visibilitystates _array_element_4)))
              (Utilities|Map|Remove _visibilitystates _array_element_4)))))
      (else
        (for _array_element_5 (Variables|Default|GetWidgetsArray)
          (Utilities|IsValid _array_element_5
            (:Is%20Valid
              (Utilities|Map|Add _visibilitystates _array_element_5 (Widget|GetVisibility _array_element_5))
              (Widget|SetVisibility _array_element_5 "Hidden"))))))
    (elif (not (Variables|Default|GetisHiddenForStart))
      (goto _label))))

(event Custom|TriggerConseillerServer
  (params (Index :type String))
  ;[0 0 0] Trigger Conseiller with Index for Server
  (for _array_element (Class|GameModeInfernale|GetPlayerControllers (.AsBP%20Game%20Mode%20Infernale (Utilities|Casting|CastToBP_GameModeInfernale (Game|GetGameMode))))
    (CallFunction|CheckConseillerOwner (.AsBP%20UIComponent (Utilities|Casting|CastToBP_UIComponent (Variables|/Script/InfernaleTesting.PlayerControllerInfernale|GetUIComponent _array_element))) Index)))

(event Custom|CreateOptionsMenu
  (bind _returnvalue (UserInterface|CreateWidget "/Game/UI/InGame/Options/WBP_Escape.WBP_Escape_C" (Variables|Default|GetBP%20Player%20Controller%20Infernale)))
  (bind _output_get (Variables|Default|SetOptionsMenu _returnvalue))
  (UserInterface|Viewport|AddtoViewport _output_get 0)
  (Widget|SetVisibility _output_get "Hidden")
  (Variables|/Game/UI/InGame/Options/WBP_Escape.WBP_Escape_C|SetPlayerControllerInfernale _output_get (Variables|Default|GetBP%20Player%20Controller%20Infernale)))

(event Custom|FluxModeStart_Event
  ;[1 1 1] LocalController
  (Utilities|FlowControl|DelayUntilNextTick)
  (Default|ChangeFluxMode (Variables|Default|GetHUD%20Widget) (Class|FluxComponent|IsFluxMode (Variables|/Script/InfernaleTesting.PlayerControllerInfernale|GetFluxComponent (Variables|Default|GetBP%20Player%20Controller%20Infernale)))))

(event Custom|CheckConseillerOwner
  (params (Index :type String))
  ;[0 0 0] Trigger Conseiller with Index for Server
  (Default|CheckConseillerwithIndex (Variables|Default|GetHUD%20Widget) Index))

(event Custom|CreateLoadingOnClient
  ;[1 1 1] CreateLoadingUI BP
  (bind _returnvalue (UserInterface|CreateWidget "/Game/UI/StartGameLobby/WBP_LoadingScreen.WBP_LoadingScreen_C" (Variables|Default|GetPlayerControllerInfernale)))
  (bind _output_get (Variables|Default|SetLoadingScreen _returnvalue))
  (UserInterface|Viewport|AddtoViewport _output_get 10000))

(event Custom|ShowHideOptionsMenu
  (params (Index :type Boolean))
  (bind _returnvalue (Game|GetPlayerController 0))
  (bind _optionsmenu (Variables|Default|GetOptionsMenu))
  (if (not (Variables|Default|GetisHiddenForStart))
    (Widget|SetVisibility _optionsmenu (select Index "Hidden" "Visible"))
    (if Index
      (Input|SetInputModeGameandUI _returnvalue 0 "LockInFullscreen" false false)
      (else
        (Input|SetInputModeUIOnly _returnvalue _optionsmenu "LockInFullscreen" false)))))

(event Custom|CreateBreachUI
  ;[1 1 1] CreateBreachUI
  (bind _returnvalue (UserInterface|CreateWidget "/Game/UI/InGame/WBP_BreachUI.WBP_BreachUI_C" (Variables|Default|GetPlayerControllerInfernale)))
  (bind _output_get (Variables|Default|SetBreachUI _returnvalue))
  (UserInterface|Viewport|AddtoViewport _output_get 0)
  (Default|Init (Variables|Default|GetBreachUI) 0 (Variables|Default|GetBP%20Player%20State%20Infernale) (Variables|Default|GetBP%20Player%20Controller%20Infernale))
  (Default|ActivateBackground (Variables|Default|GetBreachUI) false))

(event Custom|CreateNvidiaWidget)

(event Custom|LocalController
  (bind _bp_player_controller_infernale (Variables|Default|GetBP%20Player%20Controller%20Infernale))
  ;[1 1 1] LocalController
  (if (Pawn|IsLocalController (Variables|Default|GetPlayerControllerInfernale))
    (CallFunction|CreateWidgets)
    (EventDispatchers|AssignFluxModeStart _bp_player_controller_infernale (delegate Custom|FluxModeStart_Event))
    (bind _returnvalue (Class|PlayerControllerInfernale|UseFluxMode _bp_player_controller_infernale))
    (if _returnvalue
      _)))

(event Custom|CreateGameElements
  ;[1 1 1] CreateGameElements
  (bind _returnvalue (UserInterface|CreateWidget "/Game/UI/InGame/WBP_GameElements.WBP_GameElements_C" (Variables|Default|GetPlayerControllerInfernale)))
  (bind _output_get (Variables|Default|SetGameElements _returnvalue))
  (UserInterface|Viewport|AddtoViewport _output_get 1)
  (Default|Init _output_get (Variables|Default|GetBP%20Player%20Controller%20Infernale)))

(event Custom|CreateCloseAll
  ;[1 1 1] CreateCloseAll
  (bind _returnvalue (UserInterface|CreateWidget "/Game/UI/InGame/WBP_CloseAll.WBP_CloseAll_C" (Variables|Default|GetPlayerControllerInfernale)))
  (Variables|Default|SetWBP_CloseAll _returnvalue)
  (UserInterface|Viewport|AddtoViewport _returnvalue -1))

(event Custom|ShowBreach
  (params (Show :type Boolean) (Breach :type BP%20Breach%20Object%20Reference) (UseCateogry :type Boolean))
  (bind _breachui (Variables|Default|GetBreachUI))
  ;[1 1 1] ShowBreach
  (Widget|SetVisibility (Variables|Default|GetBreachUI) (select Show "Visible" "Hidden"))
  (Default|ActivateBackground (Variables|Default|GetBreachUI) Show)
  (if Show
    (Default|Init (Variables|Default|GetBreachUI) Breach (Variables|Default|GetBP%20Player%20State%20Infernale) (Variables|Default|GetBP%20Player%20Controller%20Infernale))
    (if UseCateogry
      (Default|RefreshListCategory _breachui)
      (else
        (Default|RefreshListBuildingsWithoutCategory _breachui)))))

(event Custom|CreateTooltip
  ;[1 1 1] CreateToolTips
  (bind _returnvalue (UserInterface|CreateWidget "/Game/UI/InGame/WBP_Tooltip.WBP_Tooltip_C" (Variables|Default|GetPlayerControllerInfernale)))
  (bind _output_get (Variables|Default|SetWBP_Tooltip _returnvalue))
  (UserInterface|Viewport|AddtoViewport _output_get 100)
  (Default|Init _output_get))

(event Custom|TransmutationNodeTooltip
  (params (Node :type Transmutation%20Node%20Owned%20Structure) (Location :type WBP%20Transmutation%20Node%20Object%20Reference) (Hovered :type Boolean))
  (Default|TransmutationNodeTooltip (Variables|Default|GetWBP_Tooltip) Node Location Hovered (Variables|/Game/UI/InGame/Transmutation/WBP_TransmutationTree.WBP_TransmutationTree_C|GetTransmutation%20Component (Variables|Default|GetWBP%20TransmutationTree))))

(event Custom|Create%20DraftUI
  ;[1 1 1] Create DraftUI
  (bind _returnvalue (Class|GameInstanceInfernale|GetCustomGameMode (.AsGame%20Instance%20Infernale (Utilities|Casting|CastToGameInstanceInfernale (Game|GetGameInstance)))))
  (if (== _returnvalue 3)
    (bind _returnvalue_2 (UserInterface|CreateWidget "/Game/UI/InGame/WBP_UIDraft.WBP_UIDraft_C" (Variables|Default|GetPlayerControllerInfernale)))
    (bind _output_get (Variables|Default|SetUIDraft _returnvalue_2))
    (UserInterface|Viewport|AddtoViewport _output_get 897)))

(event Custom|CreateEndGame
  ;[1 1 1] CreateEndGame
  (bind _returnvalue (UserInterface|CreateWidget "/Game/UI/InGame/EndGame/WBP_EndGame.WBP_EndGame_C" (Variables|Default|GetPlayerControllerInfernale)))
  (bind _output_get (Variables|Default|SetWBP_EndGame _returnvalue))
  (UserInterface|Viewport|AddtoViewport _output_get 100)
  (Widget|SetVisibility _output_get "Hidden"))

(event EventBeginPlay
  (bind _buildingwidgets (Variables|Default|GetBuildingWidgets))
  (bind _playercontrollerinfernale (Variables|Default|GetPlayerControllerInfernale))
  ;[1 1 1] BeginPlay
  (Utilities|IsValid _playercontrollerinfernale :!label _label
    (:Is%20Valid
      (bind _asbp_player_state_infernale (Utilities|Casting|CastToBP_PlayerStateInfernale (Variables|/Script/Engine.Controller|GetPlayerState _playercontrollerinfernale))
        (:then
          (Variables|Default|SetBP%20Player%20State%20Infernale _asbp_player_state_infernale)
          (Variables|Default|SetBP%20Player%20Controller%20Infernale (.AsBP%20Player%20Controller%20Infernale (Utilities|Casting|CastToBP_PlayerControllerInfernale _playercontrollerinfernale)))
          (CallFunction|LocalController)
          (bind _outactors (Actor|GetAllActorsOfClass "/Game/Blueprints/LD/Buildings/BP_MainBuilding.BP_MainBuilding_C"))
          (for _array_element _outactors
            (bind _asbp_main_building (Utilities|Casting|CastToBP_MainBuilding _array_element))
            (Utilities|Array|Add _buildingwidgets (UserInterface|GetWidget (Variables|/Game/Blueprints/LD/Buildings/BP_MainBuilding.BP_MainBuilding_C|GetIconRessources1 _asbp_main_building))))
          (bind _outactors_2 (Actor|GetAllActorsOfClass "/Game/Blueprints/LD/Buildings/BP_PandemoniumMainBuilding.BP_PandemoniumMainBuilding_C"))
          (for _array_element_2 _outactors_2
            (bind _asbp_pandemonium_main_building (Utilities|Casting|CastToBP_PandemoniumMainBuilding _array_element_2))
            (Utilities|Array|Add _buildingwidgets (UserInterface|GetWidget (Variables|/Game/Blueprints/LD/Buildings/BP_PandemoniumMainBuilding.BP_PandemoniumMainBuilding_C|GetIconRessources1 _asbp_pandemonium_main_building))))
          (bind _outactors_3 (Actor|GetAllActorsOfClass "/Game/Blueprints/LD/LDElements/BP_SoulBeacon.BP_SoulBeacon_C"))
          (for _array_element_3 _outactors_3
            (bind _asbp_soul_beacon (Utilities|Casting|CastToBP_SoulBeacon _array_element_3))
            (Utilities|Array|Add _buildingwidgets (UserInterface|GetWidget (Variables|/Game/Blueprints/LD/LDElements/BP_SoulBeacon.BP_SoulBeacon_C|GetIconRessources _asbp_soul_beacon))))
          (bind _outactors_4 (Actor|GetAllActorsOfClass "/Game/Blueprints/LD/LDElements/BP_Boss.BP_Boss_C"))
          (for _array_element_4 _outactors_4
            (bind _asbp_boss (Utilities|Casting|CastToBP_Boss _array_element_4))
            (Utilities|Array|Add _buildingwidgets (Variables|/Game/Blueprints/LD/LDElements/BP_Boss.BP_Boss_C|GetHigh_Altar_Widget _asbp_boss))
            (Utilities|Array|Add _buildingwidgets (Variables|/Game/Blueprints/LD/LDElements/BP_Boss.BP_Boss_C|GetLow_Altar_Widget _asbp_boss)))
          (bind _outactors_5 (Actor|GetAllActorsOfClass "/Game/Blueprints/LD/LDElements/BP_NeutralCamp_Small.BP_NeutralCamp_Small_C"))
          (for _array_element_5 _outactors_5
            (bind _asbp_neutral_camp_small (Utilities|Casting|CastToBP_NeutralCamp_Small _array_element_5))
            (Utilities|Array|Add _buildingwidgets (Variables|/Game/Blueprints/LD/LDElements/BP_NeutralCamp_Small.BP_NeutralCamp_Small_C|GetHighWidget _asbp_neutral_camp_small))
            (Utilities|Array|Add _buildingwidgets (Variables|/Game/Blueprints/LD/LDElements/BP_NeutralCamp_Small.BP_NeutralCamp_Small_C|GetLowWidget _asbp_neutral_camp_small)))
          (bind _outactors_6 (Actor|GetAllActorsOfClass "/Game/Blueprints/LD/LDElements/BP_NeutralCamp_Big.BP_NeutralCamp_Big_C"))
          (for _array_element_6 _outactors_6
            (bind _asbp_neutral_camp_big (Utilities|Casting|CastToBP_NeutralCamp_Big _array_element_6))
            (Utilities|Array|Add _buildingwidgets (Variables|/Game/Blueprints/LD/LDElements/BP_NeutralCamp_Big.BP_NeutralCamp_Big_C|GetHigh%20Widget _asbp_neutral_camp_big))
            (Utilities|Array|Add _buildingwidgets (Variables|/Game/Blueprints/LD/LDElements/BP_NeutralCamp_Big.BP_NeutralCamp_Big_C|GetLow%20Widget _asbp_neutral_camp_big))))
        (:CastFailed
          (Utilities|FlowControl|Delay 0.1 :!label _label_2)
          (goto _label))))
    (:Is%20Not%20Valid
      (goto _label_2))))

(event EventUpdateTimeRemainingBP
  (params (TimeRemaining :type Time%20Remaining%20Structure))
  (bind _hud_widget (Variables|Default|GetHUD%20Widget))
  ;[1 1 1] OnTimeRemainingBP
  (Utilities|IsValid _hud_widget
    (:Is%20Valid
      (Default|SetTimeRemaining _hud_widget TimeRemaining))
    (:Is%20Not%20Valid
      (Development|PrintString "hud widget not valid"))))

(event EventTick
  (params (DeltaSeconds :type Float%20%28single-precision%29))
  (bind _wbp_transmutationtree (Variables|Default|GetWBP%20TransmutationTree))
  ;[1 1 1] EventTick
  (Utilities|IsValid _wbp_transmutationtree
    (:Is%20Valid
      (for _array_element (Variables|/Game/UI/InGame/Transmutation/WBP_TransmutationTree.WBP_TransmutationTree_C|GetNodes _wbp_transmutationtree)
        (if (Variables|/Game/UI/InGame/Transmutation/WBP_TransmutationNode.WBP_TransmutationNode_C|GetShouldProgress _array_element)
          (Default|CustomTick _array_element DeltaSeconds)))
      (for _array_element_2 (Variables|Default|GetPopUps)
        (Default|CustomTick _array_element_2 DeltaSeconds))
      (Default|NotificationTick (Variables|Default|GetNotificationTray) DeltaSeconds))))

(event EventOnLocalPlayerLostBP
  (params (VictoryInfo :type Victory%20Info%20Map%20Structure))
  (bind _wbp_endgame (Variables|Default|GetWBP_EndGame))
  ;[1 1 1] On Local Player Lost BP
  (Widget|SetVisibility _wbp_endgame "Visible")
  (Default|PlayerKilled _wbp_endgame VictoryInfo (.Team (Utilities|Struct|BreakOwner (Variables|/Script/InfernaleTesting.PlayerStateInfernale|GetOwnerInfo (Variables|Default|GetBP%20Player%20State%20Infernale)))) self))

(event EventOnTransmutationQueueAlteredBP
  (params (TransmutationQueue :type Transmutation%20Queue%20Structure))
  ;[1 1 1] OnTransmutationQueueAltered
  (Default|TransmutationQueueAltered (Variables|Default|GetWBP%20TransmutationTree) TransmutationQueue))

(event EventOnLaunchSequenceBP
  (params (VictoryPoints :type Victory%20Points%20Structure%20%28by%20ref%29) (Team :type ETeam%20Enum :default "NatureTeam"))
  ;[1 1 1] On Launch Sequence BP
  (Default|LaunchSequence (.AsBP%20Infernale%20Pawn (Utilities|Casting|CastToBP_InfernalePawn (Game|Player|GetPlayerPawn 0))) VictoryPoints))

(event EventOnSimpleNodeOwnedAlteredBP
  (params (NodeID :type String) (TransmutationQueue :type Simple%20Transmutation%20Queue%20Structure))
  ;[1 1 1] TransmutationAlteredV2
  (Default|NodeAlteredV2 (Variables|Default|GetWBP%20TransmutationTree) NodeID TransmutationQueue))

(event EventOnSimpleTransmutationQueueAlteredBP
  (params (TransmutationQueue :type Simple%20Transmutation%20Queue%20Structure))
  ;[1 1 1] TransmutationAlteredV2
  (Default|QueueAlteredV2 (Variables|Default|GetWBP%20TransmutationTree) TransmutationQueue))

(event EventOnFluxModeRemovingBP
  (params (Start :type Boolean) (FluxModeState :type EFluxModeState%20Enum :default "FMSNone") (Duration :type Float%20%28single-precision%29))
  ;[1 1 1] OnFluxModeRemovingBP
  (Class|SoundsDataAsset|PlaySound (.soundsassets (Utilities|Array|Get(acopy) (Variables|/Script/InfernaleTesting.GameSettingsDataAsset|GetDataAssetsSettings (Class|FunctionLibraryInfernale|GetGameSettingsDataAsset)))) "Flux" "FluxNode Deleted" (Transformation|GetActorLocation (Game|Player|GetPlayerPawn 0)))
  (Default|ShowFillImages (Variables|Default|GetGameElements) Start))

(event EventOnVictoryPointChangedBP
  (params (VictoryInfo :type Victory%20Info%20Map%20Structure) (VictoryPointReason :type EVictoryPointReason%20Enum :default "EVPNone") (TeamPointChanged :type ETeam%20Enum :default "NatureTeam") (Score :type Integer))
  ;[1 1 1] OnVictoryPointChangedBP
  (Default|SetPlayersScores (Variables|Default|GetHUD%20Widget) VictoryInfo VictoryPointReason TeamPointChanged Score))

(event EventOnFluxRemovingBP
  (params (FluxModeState :type EFluxModeState%20Enum :default "FMSNone") (CurrentTimer :type Float%20%28single-precision%29) (MaxTimer :type Float%20%28single-precision%29))
  ;[1 1 1] OnFluxRemovingBP
  (Default|Advance (Variables|Default|GetGameElements) (/ CurrentTimer MaxTimer))
  (Default|MoveFillImages (Variables|Default|GetGameElements)))

(event EventCreateLoadingUIBP
  ;[1 1 1] CreateLoadingUI BP
  (bind _returnvalue (UserInterface|CreateWidget "/Game/UI/StartGameLobby/WBP_LoadingScreen.WBP_LoadingScreen_C" (Variables|Default|GetPlayerControllerInfernale)))
  (bind _output_get (Variables|Default|SetLoadingScreen _returnvalue))
  (UserInterface|Viewport|AddtoViewport _output_get 10000))

(event EventCreateTransmutationNodesBP
  (params (TransmutationNodesOwned :type Array%20of%20Transmutation%20Node%20Owned%20Structures) (TransmutationSettings :type Transmutation%20Settings%20Structure))
  ;[1 1 1] CreateTransmutationNodeBP
  (CallFunction|CreateTransmutationTree TransmutationNodesOwned TransmutationSettings))

(event EventOnTransmutationModeBP
  (params (bTransmutationMode :type Boolean))
  (bind _hud_sandbox (Variables|Default|GetHUD%20Sandbox))
  ;[1 1 1] OnTransmutationMode
  (Default|SetTransmutationMode (Variables|Default|GetWBP_CloseAll) bTransmutationMode)
  (Class|UIComponent|SetTransmutationVisible bTransmutationMode)
  (Default|SetTransmutationToogled (Variables|Default|GetHUD%20Widget) bTransmutationMode)
  (Widget|SetVisibility (Variables|Default|GetWBP%20TransmutationTree) (select bTransmutationMode "SelfHitTestInvisible" "Hidden"))
  (Utilities|IsValid _hud_sandbox
    (:Is%20Valid
      (Widget|SetFocus _hud_sandbox)
      (Default|ShowBlur _hud_sandbox bTransmutationMode))
    (:Is%20Not%20Valid
      (Widget|SetFocus (Variables|Default|GetHUD%20Widget))))
  (Class|SoundsDataAsset|PlaySound (.soundsassets (Utilities|Array|Get(acopy) (Variables|/Script/InfernaleTesting.GameSettingsDataAsset|GetDataAssetsSettings (Class|FunctionLibraryInfernale|GetGameSettingsDataAsset)))) "Transmutation Tree" (Utilities|String|Append (Utilities|String|SelectString "Open" "Close" bTransmutationMode) " Transmutation Tree") (Transformation|GetActorLocation (Game|Player|GetPlayerPawn 0))))

(event EventOnNodeOwnedAlteredBP
  (params (NodeID :type String) (TransmutationQueue :type Transmutation%20Queue%20Structure))
  ;[1 1 1] OnNodeOwnedAlteredBP
  (Development|PrintString NodeID false false "(R=0.000000,G=1.000000,B=0.063770,A=1.000000)" 2e+03)
  (Default|NodeAltered (Variables|Default|GetWBP%20TransmutationTree) NodeID TransmutationQueue))

(fn BloodCostHovered
  (params (Hovered :type Boolean) (Cost :type Float%20%28single-precision%29))
  (Default|BloodCost (Variables|Default|GetHUD%20Widget) Hovered Cost))

(fn SoulsCostHovered
  (params (Hovered :type Boolean) (Cost :type Float%20%28single-precision%29))
  (|CallParentFunction Hovered Cost)
  (Default|BloodCost (Variables|Default|GetHUD%20Widget) Hovered Cost))

(fn RemoveLoadingScreen
  (params (bRemove :type Boolean))
  (Default|RemoveLoadingScreen (.AsBP%20Game%20Instance%20Infernale (Utilities|Casting|CastToBP_GameInstanceInfernale (Game|GetGameInstance)))))

(fn FluxEntityHoveredBP
  (params (InfoType :type EFluxHoverInfoType%20Enum :default "FluxHoverInfoTypeNone"))
  (bind _hud_widget (Variables|Default|GetHUD%20Widget))
  (Utilities|IsValid _hud_widget
    (:Is%20Valid
      (Default|FluxEntityHovered _hud_widget InfoType))))

(fn OnAllPlayersSpawnedBP
  (params (Players :type Integer))
  (Default|InitPlayerScores (Variables|Default|GetHUD%20Widget) Players))

(fn TryCloseMenu
  (Default|CloseAll (Variables|Default|GetWBP_CloseAll))
  (|CallParentFunction))