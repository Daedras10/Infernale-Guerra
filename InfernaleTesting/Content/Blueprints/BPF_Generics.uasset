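; BPF_Generics is a Blueprint function set with a single helper, PolarArray, that builds transforms arranged in a circle.
; It loops over Count indices, placing each on the XY plane at Radius using degree sine and cosine, with uniform Scale and no rotation.
; The angle step divides 360 by Count minus one, so the last transform lands on the first.
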(fn PolarArray
  (params (Count :type Integer) (Radius :type Float%20%28double-precision%29) (Scale :type Float%20%28double-precision%29))
  (bind _returnvalue (Math|Float|MakeLiteralFloat Scale))
  (bind _returnvalue_2 (- Count 1))
  (for _index (range 0 _returnvalue_2)
    (Utilities|Array|Add (LocalVariables|GetInstancesTransforms) (Math|Transform|MakeTransform (Math|Vector|MakeVector (* (Math|Trig|Sin(Degrees) (* (Math|Conversions|ToFloat(Integer) _index) (/ 3.6e+02 (Math|Conversions|ToFloat(Integer) _returnvalue_2)))) Radius) (* (Math|Trig|Cos(Degrees) (* (Math|Conversions|ToFloat(Integer) _index) (/ 3.6e+02 (Math|Conversions|ToFloat(Integer) _returnvalue_2)))) Radius) 0.0) "0, 0, 0" (Math|Vector|MakeVector _returnvalue _returnvalue _returnvalue))))
  (return (LocalVariables|GetInstancesTransforms)))