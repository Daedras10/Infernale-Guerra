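; BP_GRFluxVISU is a flow visualizer that keeps a stream of static meshes moving from a spawn box toward a Finish point.
; BeginPlay calls Spawn to create mesh components at random points inside SpawnBox.
; Tick lerps each mesh toward Finish by delta time times MoveSpeed and rotates it to face that point.
; Meshes entering KillBox are destroyed, then removed from the array and replaced through Spawn.
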(event EventTick
  (params (DeltaSeconds :type Float%20%28single-precision%29))
  (bind _killbox (Variables|Default|GetKillBox))
  (bind _meshs (Variables|Default|GetMeshs))
  (bind _returnvalue (Components|Box|GetScaledBoxExtent _killbox))
  (bind _relativelocation (Variables|/Script/Engine.SceneComponent|GetRelativeLocation _killbox))
  (for _array_element (Variables|Default|GetMeshs)
    (Utilities|IsValid _array_element
      (:Is%20Valid
        (Transformation|SetRelativeLocation _array_element (Math|Vector|Lerp(Vector) (Variables|/Script/Engine.SceneComponent|GetRelativeLocation _array_element) (Variables|/Script/Engine.SceneComponent|GetRelativeLocation (Variables|Default|GetFinish)) (* DeltaSeconds (Variables|Default|GetMoveSpeed))) false false)
        (Transformation|SetWorldRotation _array_element (Math|Rotator|FindLookatRotation (Transformation|GetWorldLocation _array_element) (Transformation|GetWorldLocation (Variables|Default|GetFinish))) false false)
        (if (Class|KismetMathLibrary|BoxIsPointInside (Math|Box|MakeBox (- _relativelocation _returnvalue) (+ _relativelocation _returnvalue)) (Variables|/Script/Engine.SceneComponent|GetRelativeLocation _array_element))
          (Components|DestroyComponent _array_element)))))
  (for _array_element_2 _meshs
    (Utilities|IsValid _array_element_2
      (:Is%20Not%20Valid
        (Utilities|Array|RemoveItem _meshs _array_element_2)
        (CallFunction|Spawn)
        (for _array_element_3 _meshs
          (Utilities|IsValid _array_element_3
            (:Is%20Not%20Valid
              (Utilities|Array|RemoveItem (Variables|Default|GetMeshs) _array_element_3))))))))

(event EventBeginPlay
  (bind _meshs (Variables|Default|GetMeshs))
  (for _index (range 0 (Variables|Default|GetNbrMeshs))
    (CallFunction|Spawn))
  (for _array_element _meshs
    (Utilities|IsValid _array_element
      (:Is%20Not%20Valid
        (Utilities|Array|RemoveItem _meshs _array_element)))))

(fn ConstructionScript)

(fn Spawn
  (bind _spawnbox (Variables|Default|GetSpawnBox))
  (bind _returnvalue (Components|Box|GetScaledBoxExtent _spawnbox))
  (bind _relativelocation (Variables|/Script/Engine.SceneComponent|GetRelativeLocation _spawnbox))
  (bind _returnvalue_2 (/ _returnvalue 2.0))
  (bind _returnvalue_3 (AddComponent|AddStaticMeshComponent false (Math|Conversions|ToTransform(Vector) (Class|KismetMathLibrary|RandomPointinBoundingBoxBox (Math|Box|MakeBox (- _relativelocation _returnvalue_2) (+ _relativelocation _returnvalue_2))))))
  (Transformation|SetWorldScale3D _returnvalue_3 (Variables|Default|GetScaleMesh))
  (Components|StaticMesh|SetStaticMesh _returnvalue_3 (Variables|Default|GetMesh))
  (Utilities|Array|Add (Variables|Default|GetMeshs) _returnvalue_3)
  (Transformation|SetMobility _returnvalue_3 "Movable"))