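; Gray-room prototype actor that draws an editable flux path as a spline, along which army units spawned from an origin travel.
; A flux node actor sits at each spline point; inserts are placed by distance along the spline, and inserts or removals reindex nodes and update units.
; Node selection is forwarded to the player controller's flux component by direct cast.
; A text label at the middle node shows the clamped flux width.
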(event Custom|BuildSpline
  (params (Origin :type BP%20GR%20Base%20Object%20Reference))
  (bind _points (Variables|Default|GetPoints))
  (bind _points_2 (Variables|Default|GetPoints))
  (bind _output (Utilities|Array|Get(acopy) _points 1))
  (bind _output_2 (Utilities|Array|Get(acopy) _points_2))
  ;[1 1 1] BuildSpline
  (Spline|SetLocationatSplinePoint (Variables|Default|GetSpline) 0 _output_2 "Local" true)
  (bind _fluxnode (CallFunction|SpawnFluxNode (Math|Transform|MakeTransform _output_2) true false))
  (CallFunction|SetupFluxNode _fluxnode)
  (Variables|/Game/Blueprints/0_GrayRoom/AlexMess/Grayroom_Flux/Blueprint/BP_GRFluxNode.BP_GRFluxNode_C|SetNodeIndex _fluxnode 0)
  (Utilities|Array|Add (Variables|Default|GetNodes) _fluxnode)
  (Spline|SetLocationatSplinePoint (Variables|Default|GetSpline) 1 _output "Local" true)
  (bind _fluxnode_2 (CallFunction|SpawnFluxNode (Math|Transform|MakeTransform _output) false true))
  (CallFunction|SetupFluxNode _fluxnode_2)
  (Variables|/Game/Blueprints/0_GrayRoom/AlexMess/Grayroom_Flux/Blueprint/BP_GRFluxNode.BP_GRFluxNode_C|SetNodeIndex _fluxnode_2 1)
  (Utilities|Array|Add (Variables|Default|GetNodes) _fluxnode_2)
  (CallFunction|HideEndPoints)
  (Variables|Default|SetOrigin Origin)
  (CallFunction|UpdateText))

(event Custom|UpdateNode
  (params (NodeIndex :type Integer) (NewPosition :type Vector))
  ;[1 1 1] UpdateNode
  (Spline|SetLocationatSplinePoint (Variables|Default|GetSpline) NodeIndex NewPosition "Local" true)
  (CallFunction|UpdateText))

(event Custom|OnFluxNodeSelected
  (params (Selected :type Boolean) (Node :type BP%20GR%20Flux%20Node%20Object%20Reference))
  (bind _self self)
  (Default|CallFluxSelectedbyNode Selected Node _self)
  ;[1 1 1] For now, direct ref
  (bind _asbp_player_controller_infernale (Utilities|Casting|CastToBP_GRPlayerControllerInfernale (Game|GetPlayerController 0)))
  (Default|NodeSelected (Variables|/Game/Blueprints/0_GrayRoom/InfernaleAssets/Blueprint/GameMode/Game/BP_GRPlayerControllerInfernale.BP_GRPlayerControllerInfernale_C|GetFluxComponent _asbp_player_controller_infernale) Selected Node _self))

(event Custom|OnModified
  (for _index (range 0 (Utilities|Array|Length (Variables|Default|GetUnits)))
    _))

(event Custom|FluxNodeRemoved_Event
  (params (FluxNode :type BP%20GR%20Flux%20Node%20Object%20Reference))
  (CallFunction|RemoveNode (Variables|/Game/Blueprints/0_GrayRoom/AlexMess/Grayroom_Flux/Blueprint/BP_GRFluxNode.BP_GRFluxNode_C|GetNodeIndex FluxNode)))

(event Custom|AddNode
  (params (InputPosition :type Vector))
  (bind _units (Variables|Default|GetUnits))
  ;[1 1 1] AddNode
  (bind _returnvalue (Game|SpawnActorfromClass "/Game/Blueprints/0_GrayRoom/AlexMess/Grayroom_Flux/Blueprint/BP_GRFluxNode.BP_GRFluxNode_C" (Math|Transform|MakeTransform InputPosition) "Undefined" "MultiplyWithRoot" 0 0))
  (CallFunction|SetupFluxNode _returnvalue)
  (bind _returnindex (CallFunction|InsertNewNode _returnvalue InputPosition))
  (CallFunction|ReordertoIndex _returnindex)
  (CallFunction|ReorderfromIndex _returnindex)
  (CallFunction|UpdateText)
  (for _index (range 0 (Utilities|Array|Length (Variables|Default|GetUnits)))
    (Utilities|IsValid 0
      (:Is%20Valid
        (Default|CallUpdateArmyUnits (Utilities|Array|Get(acopy) _units _index)))
      (:Is%20Not%20Valid
        (Utilities|Array|RemoveItem _units (Utilities|Array|Get(acopy) _units _index))))))

(event Custom|HideEndPoints
  (bind _nodes (Variables|Default|GetNodes))
  (bind _output (Utilities|Array|Get(acopy) _nodes))
  ;[1 1 1] HideEndPoints
  (Rendering|SetActorHiddenInGame _output true)
  (Collision|SetCollisionEnabled (Variables|/Game/Blueprints/0_GrayRoom/AlexMess/Grayroom_Flux/Blueprint/BP_GRFluxNode.BP_GRFluxNode_C|GetCylinder _output) "NoCollision"))

(event Custom|ReorderToIndex
  (params (Index :type Integer))
  ;[1 1 1] ReorderToIndex
  (for _index (range 0 Index)
    (bind _output_get (Variables|/Game/Blueprints/0_GrayRoom/AlexMess/Grayroom_Flux/Blueprint/BP_GRFluxNode.BP_GRFluxNode_C|SetNodeIndex (Utilities|Array|Get(acopy) (Variables|Default|GetNodes) _index) _index))
    (CallFunction|UpdateNode _output_get (Transformation|GetActorLocation (Utilities|Array|Get(acopy) (Variables|Default|GetNodes) _index)))))

(event Custom|RemoveNode
  (params (Index :type Integer))
  (bind _nodes (Variables|Default|GetNodes))
  (bind _output (Utilities|Array|Get(acopy) _nodes Index))
  ;[1 1 1] RemoveNode
  (Spline|RemoveSplinePoint (Variables|Default|GetSpline) Index true)
  (Utilities|Array|RemoveIndex (Variables|Default|GetPoints) Index)
  (Actor|DestroyActor _output)
  (Utilities|Array|RemoveItem _nodes _output)
  (CallFunction|ReorderfromIndex Index)
  (CallFunction|UpdateText)
  (for _index (range 0 (Utilities|Array|Length (Variables|Default|GetUnits)))
    (Utilities|IsValid (Utilities|Array|Get(acopy) (Variables|Default|GetUnits) _index)
      (:Is%20Valid
        (Default|CallUpdateArmyUnits (Utilities|Array|Get(acopy) (Variables|Default|GetUnits) _index))))))

(event Custom|UpdateText
  (bind _nodes (Variables|Default|GetNodes))
  ;[1 1 1] UpdateText
  (Transformation|SetWorldLocation (Variables|Default|GetTextRender) (Transformation|GetActorLocation (Utilities|Array|Get(acopy) _nodes (/ (Utilities|Array|Length _nodes) 2))) false false)
  (Variables|Default|SetFluxWidth (Math|Float|Clamp(Float) (Variables|Default|GetFluxWidth) (Variables|Default|GetMinWidth) (Variables|Default|GetMaxWidth)))
  (Rendering|Components|TextRender|SetText (Variables|Default|GetTextRender) (Utilities|Text|ToText(Float) (Variables|Default|GetFluxWidth) "HalfToEven")))

(event Custom|ReorderFromIndex
  (params (Index :type Integer))
  ;[1 1 1] ReorderFromIndex
  (for _index (range Index (- (Utilities|Array|Length (Variables|Default|GetNodes)) 1))
    (bind _output_get (Variables|/Game/Blueprints/0_GrayRoom/AlexMess/Grayroom_Flux/Blueprint/BP_GRFluxNode.BP_GRFluxNode_C|SetNodeIndex (Utilities|Array|Get(acopy) (Variables|Default|GetNodes) _index) _index))
    (CallFunction|UpdateNode _output_get (Transformation|GetActorLocation (Utilities|Array|Get(acopy) (Variables|Default|GetNodes) _index)))))

(event Custom|SpawnUnit
  (bind _returnvalue (Game|SpawnActorfromClass "/Game/Blueprints/0_GrayRoom/AlexMess/Grayroom_Flux/Blueprint/BP_GRArmyUnit.BP_GRArmyUnit_C" (Transformation|GetActorTransform (Variables|Default|GetOrigin)) "Undefined" "MultiplyWithRoot" 0 0))
  (Utilities|Array|Add (Variables|Default|GetUnits) _returnvalue)
  (Default|Initialize _returnvalue (Variables|Default|GetSpline) (.Unit (Utilities|Struct|BreakSTRUCT_GRBaseArmyUnitSelection (Utilities|Array|Get(acopy) (Variables|/Game/Blueprints/0_GrayRoom/AlexMess/Grayroom_Flux/Blueprint/BP_GRBase.BP_GRBase_C|GetUnits (Variables|Default|GetOrigin))))) (Utilities|Array|Length (Variables|Default|GetUnits)))
  (Rendering|Material|SetMaterial (Variables|/Game/Blueprints/0_GrayRoom/AlexMess/Grayroom_Flux/Blueprint/BP_GRArmyUnit.BP_GRArmyUnit_C|GetCone _returnvalue) 0 (Variables|/Game/Blueprints/0_GrayRoom/AlexMess/Grayroom_Flux/Blueprint/BP_GRBase.BP_GRBase_C|GetTeamMaterial (Variables|Default|GetOrigin))))

(event Custom|SetupFluxNode
  (params (FluxNode :type BP%20GR%20Flux%20Node%20Object%20Reference))
  (EventDispatchers|BindEventtoFluxNodeSelected FluxNode (delegate Custom|OnFluxNodeSelected))
  (EventDispatchers|AssignFluxNodeRemoved FluxNode (delegate Custom|FluxNodeRemoved_Event)))

(fn ConstructionScript)

(fn InsertNewNode
  (params (Node :type BP%20GR%20Flux%20Node%20Object%20Reference) (InsertPosition :type Vector))
  (bind _spline (Variables|Default|GetSpline))
  (bind _returnvalue (Spline|GetNumberOfSplinePoints _spline))
  (bind _returnvalue_2 (- _returnvalue 2))
  (bind _returnvalue_3 (- _returnvalue 1))
  (bind _returnvalue_4 (Math|Integer|Clamp(Integer) _returnvalue_2 1 _returnvalue_3))
  (bind _index (Utilities|FlowControl|ForLoopwithBreak 0 (Spline|GetNumberOfSplinePoints (Variables|Default|GetSpline)))
    (:LoopBody
      (if (> (Spline|GetDistanceAlongSplineatSplinePoint (Variables|Default|GetSpline) _index) (Class|SplineComponent|GetDistanceAlongSplineatLocation (Variables|Default|GetSpline) InsertPosition "Local"))
        (Spline|AddSplinePointatIndex (Variables|Default|GetSpline) InsertPosition _index "Local" true)
        (bind _output_get (Variables|/Game/Blueprints/0_GrayRoom/AlexMess/Grayroom_Flux/Blueprint/BP_GRFluxNode.BP_GRFluxNode_C|SetNodeIndex Node _index))
        (Utilities|Array|Insert (Variables|Default|GetNodes) Node _output_get)
        (Development|PrintString (Utilities|String|ToString(Integer) _output_get))
        (return _output_get)
        (elif (>= _index _returnvalue)
          (Spline|AddSplinePointatIndex (Variables|Default|GetSpline) InsertPosition _returnvalue_4 "Local" true)
          (bind _output_get_2 (Variables|/Game/Blueprints/0_GrayRoom/AlexMess/Grayroom_Flux/Blueprint/BP_GRFluxNode.BP_GRFluxNode_C|SetNodeIndex Node _returnvalue_4))
          (Utilities|Array|Insert (Variables|Default|GetNodes) Node _output_get_2)
          (Development|PrintString "Inserted at last point")
          (return _output_get_2))))))

(fn SpawnFluxNode
  (params (Transform :type Transform) (IsStart :type Boolean) (IsEnd :type Boolean))
  (bind _returnvalue (Game|SpawnActorfromClass "/Game/Blueprints/0_GrayRoom/AlexMess/Grayroom_Flux/Blueprint/BP_GRFluxNode.BP_GRFluxNode_C" Transform "Undefined" "MultiplyWithRoot" 0 0))
  (Variables|/Game/Blueprints/0_GrayRoom/AlexMess/Grayroom_Flux/Blueprint/BP_GRFluxNode.BP_GRFluxNode_C|SetIsStart _returnvalue IsStart)
  (Variables|/Game/Blueprints/0_GrayRoom/AlexMess/Grayroom_Flux/Blueprint/BP_GRFluxNode.BP_GRFluxNode_C|SetIsEnd _returnvalue IsEnd)
  (return _returnvalue))