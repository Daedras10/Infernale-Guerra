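; BP_GRArmyUnit is an army unit that marches along a spline, fights opposing units and besieges enemy bases.
; Initialize takes stats and team from unit data, then Tick steps it between spline points until death or path end destroys it.
; A range-sized sphere switches it to Attack, draining the first enemy's health over time.
; Overlapping an enemy base reduces possession, capturing or putting it under siege, and flags the unit for destruction.
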(event OnComponentBeginOverlap(Collider)
  (params (OverlappedComponent :type Primitive%20Component%20Object%20Reference) (OtherActor :type Actor%20Object%20Reference) (OtherComp :type Primitive%20Component%20Object%20Reference) (OtherBodyIndex :type Integer) (bFromSweep :type Boolean) (SweepResult :type Hit%20Result%20Structure%20%28by%20ref%29))
  (bind (_asbp_army_unit _bsuccess) (Utilities|Casting|CastToBP_GRArmyUnit OtherActor))
  (bind _asbp_base (Utilities|Casting|CastToBP_GRBase OtherActor))
  (if (Variables|Default|Get?isInitialized)
    (if _bsuccess
      (if (Variables|BP_GRArmyUnit_C|Get?isInitialized _asbp_army_unit)
        (if (!= (Variables|Default|GetTeam) (Variables|BP_GRArmyUnit_C|GetTeam _asbp_army_unit))
          (Utilities|Array|AddUnique (Variables|Default|GetEnemiesInRange) _asbp_army_unit)
          (Variables|Default|SetState "NewEnumerator2")))
      (else
        (Utilities|IsValid _asbp_base
          (:Is%20Valid
            (if (!= (Variables|Default|GetTeam) (Variables|/Game/Blueprints/0_GrayRoom/AlexMess/Grayroom_Flux/Blueprint/BP_GRBase.BP_GRBase_C|GetTeam _asbp_base))
              (CallFunction|ReducePosession _asbp_base)
              (Variables|Default|Set%20?shouldDestroy true))))))))

(event Custom|Initialize
  (params (Spline :type Spline%20Component%20Object%20Reference) (UnitData :type STRUCT%20GR%20Army%20Amalgam%20Structure) (ID :type Integer))
  (bind (_blueprintunit _damage _health _range _baseref) (Utilities|Struct|BreakSTRUCT_GRArmyAmalgam UnitData))
  (bind _output_get (Variables|Default|SetSpline Spline))
  (Variables|Default|SetTarget (.Position (Utilities|Struct|BreakSplinePoint (Spline|GetSplinePointAt _output_get 0 "Local"))))
  (Variables|Default|SetTargetIndex 0)
  (Variables|Default|SetDamage _damage)
  (Variables|Default|SetHealth _health)
  (Components|Sphere|SetSphereRadius (Variables|Default|GetCollider) _range true)
  (Variables|Default|SetTeam (Variables|/Game/Blueprints/0_GrayRoom/AlexMess/Grayroom_Flux/Blueprint/BP_GRBase.BP_GRBase_C|GetTeam _baseref))
  (Variables|Default|Set?isInitialized true))

(event Custom|SetTargetAtNextPoint
  (bind _output_get (Variables|Default|SetTargetIndex (+ (Variables|Default|GetTargetIndex) 1)))
  (if (!= _output_get (Spline|GetNumberOfSplinePoints (Variables|Default|GetSpline)))
    (Variables|Default|SetTarget (.Position (Utilities|Struct|BreakSplinePoint (Spline|GetSplinePointAt (Variables|Default|GetSpline) _output_get "Local"))))
    (else
      (Variables|Default|Set%20?shouldDestroy true))))

(event Custom|ReducePosession
  (params (TargetBase :type BP%20GR%20Base%20Object%20Reference))
  (bind _output_get (Variables|/Game/Blueprints/0_GrayRoom/AlexMess/Grayroom_Flux/Blueprint/BP_GRBase.BP_GRBase_C|SetPossession TargetBase (- (Variables|/Game/Blueprints/0_GrayRoom/AlexMess/Grayroom_Flux/Blueprint/BP_GRBase.BP_GRBase_C|GetPossession TargetBase) 1.0)))
  (if (<= _output_get 0.0)
    (Default|Capture TargetBase (Variables|Default|GetTeam))
    (else
      (Variables|/Game/Blueprints/0_GrayRoom/AlexMess/Grayroom_Flux/Blueprint/BP_GRBase.BP_GRBase_C|SetBaseState TargetBase "NewEnumerator2")
      (Variables|/Game/Blueprints/0_GrayRoom/AlexMess/Grayroom_Flux/Blueprint/BP_GRBase.BP_GRBase_C|SetSiegeEndTimer TargetBase 0.0))))

(event Custom|UpdateTarget
  (Variables|Default|SetTarget (.Position (Utilities|Struct|BreakSplinePoint (Spline|GetSplinePointAt (Variables|Default|GetSpline) (Variables|Default|GetTargetIndex) "Local")))))

(event EventBeginPlay
  (EventDispatchers|BindEventtoUpdateArmyUnits (delegate Custom|UpdateTarget)))

(event EventTick
  (params (DeltaSeconds :type Float%20%28single-precision%29))
  (bind _returnvalue (Transformation|GetActorLocation))
  (bind _enemiesinrange (Variables|Default|GetEnemiesInRange))
  (bind _target (Variables|Default|GetTarget))
  (bind _output (Utilities|Array|Get(acopy) _enemiesinrange))
  (bind _returnvalue_2 (- _target _returnvalue))
  (if (Variables|Default|Get?isInitialized)
    (if (> (Variables|Default|GetHealth) 0.0)
      (switch Utilities|FlowControl|Switch|SwitchonENUM_GRArmyUnitState (Variables|Default|GetState)
        (:NewEnumerator1
          (if (> (Math|Vector|VectorLength _returnvalue_2) 2.0)
            (Utilities|IsValid self
              (:Is%20Valid
                _))
            (else
              (CallFunction|SetTargetatNextPoint)))
          (Transformation|SetActorLocation self (+ (* (Math|Vector|Normalize _returnvalue_2) DeltaSeconds (Variables|Default|GetSpeed)) (Transformation|GetActorLocation)) false false)
          (if (Variables|Default|Get%20?shouldDestroy)
            (Actor|DestroyActor)))
        (:NewEnumerator2
          (if (Utilities|Array|IsNotEmpty _enemiesinrange)
            (Utilities|IsValid _output
              (:Is%20Valid
                (Variables|BP_GRArmyUnit_C|SetHealth _output (- (Variables|BP_GRArmyUnit_C|GetHealth _output) (* (Variables|Default|GetDamage) DeltaSeconds))))
              (:Is%20Not%20Valid
                (Utilities|Array|RemoveItem _enemiesinrange _output)))
            (else
              (Variables|Default|SetState "NewEnumerator1")))))
      (else
        (Actor|DestroyActor)))))

(fn ConstructionScript)