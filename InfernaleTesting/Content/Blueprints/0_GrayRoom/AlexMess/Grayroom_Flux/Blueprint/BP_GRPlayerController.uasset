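; Gray-room prototype player controller for mouse-driven selection of bases and drawing and editing of the fluxes between them.
; Draw and edit mode flags gate cursor traces that create fluxes from the selected base, then add or drag their nodes.
; Node placement and drags refresh the flux's army units, pruning invalid ones.
; Debug keys handle mode switching, flux cycling, deletion and width adjustment.
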(event Custom|ResetModes
  (bind _selectedbase (Variables|Default|GetSelectedBase))
  ;[1 1 1] Reset Edition Modes
  (Variables|Default|Set?isDrawMode false)
  (Variables|Default|Set?isEditMode false)
  (Utilities|IsValid _selectedbase
    (:Is%20Valid
      (Default|OnDeselected _selectedbase))))

(event EventTick
  (params (DeltaSeconds :type Float%20%28single-precision%29))
  (bind _hitresult (Game|Player|GetHitResultUnderCursorbyChannel "TraceTypeQuery1" true))
  (bind _selectedbase (Variables|Default|GetSelectedBase))
  (bind _fluxindex (Variables|Default|GetFluxIndex))
  (bind _impactpoint (Collision|BreakHitResult _hitresult))
  (bind _fluxarray (Variables|/Game/Blueprints/0_GrayRoom/AlexMess/Grayroom_Flux/Blueprint/BP_GRBase.BP_GRBase_C|GetFluxArray _selectedbase))
  (bind (_x _y) (Math|Vector|BreakVector _impactpoint))
  (bind _output (Utilities|Array|Get(acopy) _fluxarray _fluxindex))
  (bind _units (Variables|/Game/Blueprints/0_GrayRoom/AlexMess/Grayroom_Flux/Blueprint/BP_GRFluxDrawer.BP_GRFluxDrawer_C|GetUnits _output))
  ;[1 1 1] Currently Handles Node Displacement using cursor
  (Utilities|IsValid (Variables|Default|GetGrabbedNode)
    (:Is%20Valid
      (if (Variables|Default|Get?isGrab)
        (Default|UpdateLocation (Variables|Default|GetGrabbedNode) (CallFunction|GetCurrentFlux) (Math|Vector|MakeVector _x _y 0.0))
        (for _index (range 0 (Utilities|Array|Length _units))
          (Utilities|IsValid (Utilities|Array|Get(acopy) _units _index)
            (:Is%20Valid
              (Default|CallUpdateArmyUnits (Utilities|Array|Get(acopy) _units _index)))
            (:Is%20Not%20Valid
              (Utilities|Array|RemoveItem _units (Utilities|Array|Get(acopy) _units _index)))))))))

(event EventBeginPlay
  (Development|ExecuteConsoleCommand "show splines" 0)
  (Variables|Default|SetbShowMouseCursor true))

(event Input|MouseEvents|DebugKeyRightMouseButton
  (params (Key :type Key%20Structure) (ActionValue :type Input%20Action%20Value%20Structure))
  (bind _selectedbase (Variables|Default|GetSelectedBase))
  (bind _selectedbase_2 (Variables|Default|GetSelectedBase))
  (bind _fluxarray (Variables|/Game/Blueprints/0_GrayRoom/AlexMess/Grayroom_Flux/Blueprint/BP_GRBase.BP_GRBase_C|GetFluxArray _selectedbase_2))
  ;[1 1 1] RMB Input - Handles Either Flux Creation or Node Placement
  (:Pressed
    (if (Variables|Default|Get?isDrawMode)
      (bind _asbp_base (Utilities|Casting|CastToBP_GRBase (.HitActor (Collision|BreakHitResult (.HitResult (Game|Player|GetHitResultUnderCursorbyChannel "TraceTypeQuery1" true)))))
        (:then
          (Utilities|IsValid _selectedbase
            (:Is%20Valid
              (Default|CreateFlux _selectedbase _asbp_base)
              (if (Utilities|Array|IsEmpty _fluxarray)
                _
                (else
                  (Default|OnFluxDeselectedbyIndex _selectedbase_2 (Variables|Default|GetFluxIndex))))
              (bind _output_get (Variables|Default|SetFluxIndex (- (Utilities|Array|Length _fluxarray) 1)))
              (Default|OnFluxSelectedbyIndex _selectedbase _output_get)
              (Variables|Default|Set?isDrawMode false)
              (Variables|Default|Set?isEditMode true)
              (Default|EnterEditMode (Variables|Default|GetSelectedBase))
              (for _index (range 0 (Utilities|Array|Length (Variables|/Game/Blueprints/0_GrayRoom/AlexMess/Grayroom_Flux/Blueprint/BP_GRFluxDrawer.BP_GRFluxDrawer_C|GetUnits (Utilities|Array|Get(acopy) (Variables|/Game/Blueprints/0_GrayRoom/AlexMess/Grayroom_Flux/Blueprint/BP_GRBase.BP_GRBase_C|GetFluxArray (Variables|Default|GetSelectedBase)) (Variables|Default|GetFluxIndex)))))
                (Utilities|IsValid (Utilities|Array|Get(acopy) (Variables|/Game/Blueprints/0_GrayRoom/AlexMess/Grayroom_Flux/Blueprint/BP_GRFluxDrawer.BP_GRFluxDrawer_C|GetUnits (Utilities|Array|Get(acopy) (Variables|/Game/Blueprints/0_GrayRoom/AlexMess/Grayroom_Flux/Blueprint/BP_GRBase.BP_GRBase_C|GetFluxArray (Variables|Default|GetSelectedBase)) (Variables|Default|GetFluxIndex))) _index)
                  (:Is%20Valid
                    (Default|CallUpdateArmyUnits (Utilities|Array|Get(acopy) (Variables|/Game/Blueprints/0_GrayRoom/AlexMess/Grayroom_Flux/Blueprint/BP_GRFluxDrawer.BP_GRFluxDrawer_C|GetUnits (Utilities|Array|Get(acopy) (Variables|/Game/Blueprints/0_GrayRoom/AlexMess/Grayroom_Flux/Blueprint/BP_GRBase.BP_GRBase_C|GetFluxArray (Variables|Default|GetSelectedBase)) (Variables|Default|GetFluxIndex))) _index)))
                  (:Is%20Not%20Valid
                    (Utilities|Array|RemoveItem (Variables|/Game/Blueprints/0_GrayRoom/AlexMess/Grayroom_Flux/Blueprint/BP_GRFluxDrawer.BP_GRFluxDrawer_C|GetUnits (Utilities|Array|Get(acopy) (Variables|/Game/Blueprints/0_GrayRoom/AlexMess/Grayroom_Flux/Blueprint/BP_GRBase.BP_GRBase_C|GetFluxArray (Variables|Default|GetSelectedBase)) (Variables|Default|GetFluxIndex))) (Utilities|Array|Get(acopy) (Variables|/Game/Blueprints/0_GrayRoom/AlexMess/Grayroom_Flux/Blueprint/BP_GRFluxDrawer.BP_GRFluxDrawer_C|GetUnits (Utilities|Array|Get(acopy) (Variables|/Game/Blueprints/0_GrayRoom/AlexMess/Grayroom_Flux/Blueprint/BP_GRBase.BP_GRBase_C|GetFluxArray (Variables|Default|GetSelectedBase)) (Variables|Default|GetFluxIndex))) _index))))))))
        (:CastFailed
          (CallFunction|ResetModes)
          (Development|PrintString "Invalid Destination")))
      (elif (Variables|Default|Get?isEditMode)
        (Default|AddNode (CallFunction|GetCurrentFlux) (.ImpactPoint (Collision|BreakHitResult (.HitResult (Game|Player|GetHitResultUnderCursorbyChannel "TraceTypeQuery1" true)))))
        (for _index_2 (range 0 (Utilities|Array|Length (Variables|/Game/Blueprints/0_GrayRoom/AlexMess/Grayroom_Flux/Blueprint/BP_GRFluxDrawer.BP_GRFluxDrawer_C|GetUnits (Utilities|Array|Get(acopy) (Variables|/Game/Blueprints/0_GrayRoom/AlexMess/Grayroom_Flux/Blueprint/BP_GRBase.BP_GRBase_C|GetFluxArray (Variables|Default|GetSelectedBase)) (Variables|Default|GetFluxIndex)))))
          (Utilities|IsValid (Utilities|Array|Get(acopy) (Variables|/Game/Blueprints/0_GrayRoom/AlexMess/Grayroom_Flux/Blueprint/BP_GRFluxDrawer.BP_GRFluxDrawer_C|GetUnits (Utilities|Array|Get(acopy) (Variables|/Game/Blueprints/0_GrayRoom/AlexMess/Grayroom_Flux/Blueprint/BP_GRBase.BP_GRBase_C|GetFluxArray (Variables|Default|GetSelectedBase)) (Variables|Default|GetFluxIndex))) _index_2)
            (:Is%20Valid
              (Default|CallUpdateArmyUnits (Utilities|Array|Get(acopy) (Variables|/Game/Blueprints/0_GrayRoom/AlexMess/Grayroom_Flux/Blueprint/BP_GRFluxDrawer.BP_GRFluxDrawer_C|GetUnits (Utilities|Array|Get(acopy) (Variables|/Game/Blueprints/0_GrayRoom/AlexMess/Grayroom_Flux/Blueprint/BP_GRBase.BP_GRBase_C|GetFluxArray (Variables|Default|GetSelectedBase)) (Variables|Default|GetFluxIndex))) _index_2)))
            (:Is%20Not%20Valid
              (Utilities|Array|RemoveItem (Variables|/Game/Blueprints/0_GrayRoom/AlexMess/Grayroom_Flux/Blueprint/BP_GRFluxDrawer.BP_GRFluxDrawer_C|GetUnits (Utilities|Array|Get(acopy) (Variables|/Game/Blueprints/0_GrayRoom/AlexMess/Grayroom_Flux/Blueprint/BP_GRBase.BP_GRBase_C|GetFluxArray (Variables|Default|GetSelectedBase)) (Variables|Default|GetFluxIndex))) (Utilities|Array|Get(acopy) (Variables|/Game/Blueprints/0_GrayRoom/AlexMess/Grayroom_Flux/Blueprint/BP_GRFluxDrawer.BP_GRFluxDrawer_C|GetUnits (Utilities|Array|Get(acopy) (Variables|/Game/Blueprints/0_GrayRoom/AlexMess/Grayroom_Flux/Blueprint/BP_GRBase.BP_GRBase_C|GetFluxArray (Variables|Default|GetSelectedBase)) (Variables|Default|GetFluxIndex))) _index_2)))))))))

(event Input|KeyboardEvents|DebugKeyF
  (params (Key :type Key%20Structure) (ActionValue :type Input%20Action%20Value%20Structure))
  (bind _selectedbase (Variables|Default|GetSelectedBase))
  ;[1 1 1] F Input - Enters Draw Mode
  (:Pressed
    (Utilities|IsValid (Variables|Default|GetSelectedBase)
      (:Is%20Valid
        (bind _output_get (Variables|Default|Set?isDrawMode (not (Variables|Default|Get?isDrawMode))))
        (if _output_get
          (Default|EnterBuildMode _selectedbase)
          (else
            (Default|OnSelected _selectedbase)))))))

(event Input|KeyboardEvents|DebugKeySubtract
  (params (Key :type Key%20Structure) (ActionValue :type Input%20Action%20Value%20Structure))
  (bind _newparam (CallFunction|GetCurrentFlux))
  ;[1 1 1] Input Num - - Decrease Flux Width
  (:Pressed
    (bind _output_get (Variables|/Game/Blueprints/0_GrayRoom/AlexMess/Grayroom_Flux/Blueprint/BP_GRFluxDrawer.BP_GRFluxDrawer_C|SetFluxWidth _newparam (- (Variables|/Game/Blueprints/0_GrayRoom/AlexMess/Grayroom_Flux/Blueprint/BP_GRFluxDrawer.BP_GRFluxDrawer_C|GetFluxWidth _newparam) 0.5)))
    (Default|UpdateText _newparam)
    (Development|PrintString (Utilities|String|ToString(Float) _output_get))))

(event Input|KeyboardEvents|DebugKeyAdd
  (params (Key :type Key%20Structure) (ActionValue :type Input%20Action%20Value%20Structure))
  (bind _newparam (CallFunction|GetCurrentFlux))
  ;[1 1 1] Input Num + - Incease Flux Width
  (:Pressed
    (bind _output_get (Variables|/Game/Blueprints/0_GrayRoom/AlexMess/Grayroom_Flux/Blueprint/BP_GRFluxDrawer.BP_GRFluxDrawer_C|SetFluxWidth _newparam (+ (Variables|/Game/Blueprints/0_GrayRoom/AlexMess/Grayroom_Flux/Blueprint/BP_GRFluxDrawer.BP_GRFluxDrawer_C|GetFluxWidth _newparam) 0.5)))
    (Default|UpdateText _newparam)
    (Development|PrintString (Utilities|String|ToString(Float) _output_get))))

(event Input|KeyboardEvents|DebugKeyQ
  (params (Key :type Key%20Structure) (ActionValue :type Input%20Action%20Value%20Structure))
  ;[1 1 1] Q Input - Reset Modes
  (:Pressed
    (CallFunction|ResetModes)))

(event Input|MouseEvents|DebugKeyLeftMouseButton
  (params (Key :type Key%20Structure) (ActionValue :type Input%20Action%20Value%20Structure))
  (bind _hitresult (Game|Player|GetHitResultUnderCursorbyChannel "TraceTypeQuery1" true))
  (bind _hitresult_2 (Game|Player|GetHitResultUnderCursorbyChannel "TraceTypeQuery1" true))
  (bind _hitactor (Collision|BreakHitResult _hitresult))
  (bind _hitactor_2 (Collision|BreakHitResult _hitresult_2))
  (bind _asbp_flux_node (Utilities|Casting|CastToBP_GRFluxNode _hitactor_2))
  (bind (_asbp_base _bsuccess) (Utilities|Casting|CastToBP_GRBase _hitactor))
  ;[1 1 1] Left Click Input - Selects Flux Node or Base
  (:Pressed
    (if (Variables|Default|Get?isEditMode)
      (if (Utilities|Array|ContainsItem (Variables|/Game/Blueprints/0_GrayRoom/AlexMess/Grayroom_Flux/Blueprint/BP_GRFluxDrawer.BP_GRFluxDrawer_C|GetNodes (CallFunction|GetCurrentFlux)) _asbp_flux_node)
        (Variables|Default|Set?isGrab true)
        (bind _output_get (Variables|Default|SetGrabbedNode _asbp_flux_node))
        (Default|OnSelected _output_get))
      (else
        (Utilities|IsValid (Variables|Default|GetSelectedBase)
          (:Is%20Valid
            (Default|OnDeselected (Variables|Default|GetSelectedBase)))
          (:Is%20Not%20Valid
            _))
        (if _bsuccess
          (bind _output_get_2 (Variables|Default|SetSelectedBase _asbp_base))
          (Default|OnSelected _output_get_2)
          (Variables|Default|SetFluxIndex 0)
          (else
            (Variables|Default|SetSelectedBase 0))))))
  (:Released
    (Variables|Default|Set?isGrab false)
    (Utilities|IsValid (Variables|Default|GetGrabbedNode)
      (:Is%20Valid
        (Default|OnDeselected (Variables|Default|GetGrabbedNode))
        (Variables|Default|SetGrabbedNode 0)))))

(event Input|KeyboardEvents|DebugKeyR
  (params (Key :type Key%20Structure) (ActionValue :type Input%20Action%20Value%20Structure))
  (bind _grabbednode (Variables|Default|GetGrabbedNode))
  ;[1 1 1] R Input - Delete Selected Flux Node
  (:Pressed
    (Utilities|IsValid _grabbednode
      (:Is%20Valid
        (Default|RemoveNode (CallFunction|GetCurrentFlux) (Variables|/Game/Blueprints/0_GrayRoom/AlexMess/Grayroom_Flux/Blueprint/BP_GRFluxNode.BP_GRFluxNode_C|GetNodeIndex _grabbednode))))))

(event Input|KeyboardEvents|DebugKeyT
  (params (Key :type Key%20Structure) (ActionValue :type Input%20Action%20Value%20Structure))
  (bind _selectedbase (Variables|Default|GetSelectedBase))
  ;[1 1 1] T Input - Delete Flux
  (:Pressed
    (Utilities|IsValid _selectedbase
      (:Is%20Valid
        (Default|DestroyFlux _selectedbase (Variables|Default|GetFluxIndex))
        (Default|OnSelected _selectedbase)))))

(event Input|KeyboardEvents|DebugKeyP
  (params (Key :type Key%20Structure) (ActionValue :type Input%20Action%20Value%20Structure))
  (bind _selectedbase (Variables|Default|GetSelectedBase))
  ;[1 1 1] P Input - Deselect Base
  (:Pressed
    (Utilities|IsValid _selectedbase
      (:Is%20Valid
        (Default|OnDeselected _selectedbase)
        (Default|OnFluxDeselectedbyIndex _selectedbase (Variables|Default|GetFluxIndex))))))

(event Input|KeyboardEvents|DebugKeyNumPadOne
  (params (Key :type Key%20Structure) (ActionValue :type Input%20Action%20Value%20Structure))
  (bind _selectedbase (Variables|Default|GetSelectedBase))
  ;[1 1 1] Input Num1 - Flux Selection
  (:Pressed
    (Utilities|IsValid _selectedbase
      (:Is%20Valid
        (if (not (Utilities|Array|IsEmpty (Variables|/Game/Blueprints/0_GrayRoom/AlexMess/Grayroom_Flux/Blueprint/BP_GRBase.BP_GRBase_C|GetFluxArray (Variables|Default|GetSelectedBase))))
          (Variables|Default|Set?isEditMode true)
          (Default|OnFluxDeselectedbyIndex _selectedbase (Variables|Default|GetFluxIndex))
          (bind _output_get (Variables|Default|SetFluxIndex (Math|Integer|%(Integer) (+ (Variables|Default|GetFluxIndex) 1) (Utilities|Array|Length (Variables|/Game/Blueprints/0_GrayRoom/AlexMess/Grayroom_Flux/Blueprint/BP_GRBase.BP_GRBase_C|GetFluxArray (Variables|Default|GetSelectedBase))))))
          (Default|OnFluxSelectedbyIndex _selectedbase _output_get)
          (Default|EnterEditMode _selectedbase))))))

(fn ConstructionScript)

(fn GetCurrentFlux
  (return (Utilities|Array|Get(acopy) (Variables|/Game/Blueprints/0_GrayRoom/AlexMess/Grayroom_Flux/Blueprint/BP_GRBase.BP_GRBase_C|GetFluxArray (Variables|Default|GetSelectedBase)) (Variables|Default|GetFluxIndex))))