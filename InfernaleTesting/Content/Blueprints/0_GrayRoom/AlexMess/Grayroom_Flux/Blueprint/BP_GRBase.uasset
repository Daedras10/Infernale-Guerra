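; Team-owned base for a gray-room prototype that sends units along player-directed "flux" paths and can be captured.
; Creates and destroys BP_GRFluxDrawer splines, with Tick spawning units round-robin across them on a timer.
; A Tick-driven state machine handles siege timeout and possession recovery, while Capture switches team and clears fluxes.
; Team, selection, build and edit modes show through cube materials; flux selection recolors splines.
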(event Custom|OnSelected
  ;[1 1 1] OnSelected
  (Rendering|Material|SetMaterial (Variables|Default|GetCube) 0 "/Game/Blueprints/0_GrayRoom/AlexMess/Grayroom_Flux/Materials/M_GRSelected.M_GRSelected"))

(event Custom|OnDeselected
  ;[1 1 1] OnDeselected
  (Rendering|Material|SetMaterial (Variables|Default|GetCube) 0 (Variables|Default|GetTeamMaterial))
  (for _index (range 0 (- (Utilities|Array|Length (Variables|Default|GetFluxArray)) 1))
    (CallFunction|OnFluxDeselectedbyIndex _index)))

(event Custom|OnFluxDeselected
  (params (Flux :type BP%20GR%20Flux%20Drawer%20Object%20Reference))
  (bind _returnvalue (Math|Color|MakeColor 0.0 1.0 0.0))
  (bind _spline (Variables|/Game/Blueprints/0_GrayRoom/AlexMess/Grayroom_Flux/Blueprint/BP_GRFluxDrawer.BP_GRFluxDrawer_C|GetSpline Flux))
  (Class|SplineComponent|SetUnselectedSplineSegmentColor _spline _returnvalue)
  (Class|SplineComponent|SetSelectedSplineSegmentColor _spline _returnvalue)
  (Spline|UpdateSpline _spline))

(event Custom|OnFluxSelected
  (params (Flux :type BP%20GR%20Flux%20Drawer%20Object%20Reference))
  (bind _returnvalue (Math|Color|MakeColor 1.0 0.0 0.0))
  (bind _spline (Variables|/Game/Blueprints/0_GrayRoom/AlexMess/Grayroom_Flux/Blueprint/BP_GRFluxDrawer.BP_GRFluxDrawer_C|GetSpline Flux))
  (Class|SplineComponent|SetUnselectedSplineSegmentColor _spline _returnvalue)
  (Class|SplineComponent|SetSelectedSplineSegmentColor _spline _returnvalue)
  (Spline|UpdateSpline _spline))

(event Custom|UpdateFluxesOutput
  ;[1 0.1771 0.1771] UpdateFluxesOutput
)

(event Custom|UpdateTeam
  (params (Team :type Byte))
  (bind _units (Variables|Default|GetUnits))
  (Variables|Default|SetTeam Team)
  (bind _returnvalue (Rendering|Material|CreateDynamicMaterialInstance "/Game/Blueprints/0_GrayRoom/AlexMess/Grayroom_Flux/Materials/M_GRTeam.M_GRTeam" "None" "None" :!class /Script/Engine.KismetMaterialLibrary))
  (bind _output_get (Variables|Default|SetTeamMaterial _returnvalue))
  (Rendering|Material|SetVectorParameterValue _output_get "Base Color" (Utilities|Select :Index (Variables|Default|GetTeam) :Option%200 "(R=1.000000,G=0.021699,B=0.000000,A=1.000000)" :Option%201 "(R=0.009358,G=0.000000,B=1.000000,A=1.000000)" :Option%202 "(R=1.000000,G=0.876216,B=0.000000,A=1.000000)" :Option%203 "(R=0.076735,G=1.000000,B=0.000000,A=1.000000)") :!class /Script/Engine.MaterialInstanceDynamic)
  (Rendering|Material|SetMaterial (Variables|Default|GetCube1) 0 (Variables|Default|GetTeamMaterial))
  (Rendering|Material|SetMaterial (Variables|Default|GetCube2) 0 (Variables|Default|GetTeamMaterial))
  (Rendering|Material|SetMaterial (Variables|Default|GetCube3) 0 (Variables|Default|GetTeamMaterial))
  (Rendering|Material|SetMaterial (Variables|Default|GetCube4) 0 (Variables|Default|GetTeamMaterial))
  (Rendering|Material|SetMaterial (Variables|Default|GetCube5) 0 (Variables|Default|GetTeamMaterial))
  (Rendering|Material|SetMaterial (Variables|Default|GetCube) 0 (Variables|Default|GetTeamMaterial))
  (Variables|Default|SetPossession (Variables|Default|GetPossessionMax))
  (for (_array_element _array_index) _units
    (Utilities|Array|SetArrayElem _units _array_index (Utilities|Struct|MakeSTRUCT_GRBaseArmyUnitSelection (Utilities|Struct|MakeSTRUCT_GRArmyAmalgam (.blueprintunit (.Unit (Utilities|Struct|BreakSTRUCT_GRBaseArmyUnitSelection _array_element))) (.damage (.Unit (Utilities|Struct|BreakSTRUCT_GRBaseArmyUnitSelection _array_element))) (.health (.Unit (Utilities|Struct|BreakSTRUCT_GRBaseArmyUnitSelection _array_element))) (.range (.Unit (Utilities|Struct|BreakSTRUCT_GRBaseArmyUnitSelection _array_element))) self) (.Proportion (Utilities|Struct|BreakSTRUCT_GRBaseArmyUnitSelection _array_element))))))

(event Custom|Capture
  (params (Team :type Byte))
  (bind _fluxarray (Variables|Default|GetFluxArray))
  ;[1 1 1] Captrure
  (bind _output_get (Variables|Default|SetTeam Team))
  (CallFunction|UpdateTeam _output_get)
  (Variables|Default|SetPossession 1.0)
  (Variables|Default|SetBaseState "NewEnumerator3")
  (for _array_element _fluxarray
    (Utilities|Array|RemoveItem _fluxarray _array_element)
    (Actor|DestroyActor _array_element)))

(event Custom|DestroyFluxRef
  (params (Flux :type BP%20GR%20Flux%20Drawer%20Object%20Reference))
  ;[1 1 1] DestroyFluxRef
  (Utilities|IsValid Flux
    (:Is%20Valid
      (for _index (range 0 (- (Utilities|Array|Length (Variables|/Game/Blueprints/0_GrayRoom/AlexMess/Grayroom_Flux/Blueprint/BP_GRFluxDrawer.BP_GRFluxDrawer_C|GetNodes Flux)) 1))
        (Actor|DestroyActor (Utilities|Array|Get(acopy) (Variables|/Game/Blueprints/0_GrayRoom/AlexMess/Grayroom_Flux/Blueprint/BP_GRFluxDrawer.BP_GRFluxDrawer_C|GetNodes Flux) _index)))
      (Actor|DestroyActor Flux)
      (Utilities|Array|RemoveItem (Variables|Default|GetFluxArray) Flux)
      (CallFunction|UpdateFluxesOutput))))

(event Custom|OnFluxSelectedByIndex
  (params (FluxIndex :type Integer))
  (bind _returnvalue (Math|Color|MakeColor 1.0 0.0 0.0))
  (bind _fluxarray (Variables|Default|GetFluxArray))
  (bind _output (Utilities|Array|Get(acopy) _fluxarray FluxIndex))
  (bind _spline (Variables|/Game/Blueprints/0_GrayRoom/AlexMess/Grayroom_Flux/Blueprint/BP_GRFluxDrawer.BP_GRFluxDrawer_C|GetSpline _output))
  ;[1 1 1] OnFluxSelected
  (Class|SplineComponent|SetUnselectedSplineSegmentColor _spline _returnvalue)
  (Class|SplineComponent|SetSelectedSplineSegmentColor _spline _returnvalue)
  (Spline|UpdateSpline _spline))

(event Custom|OnFluxDeselectedByIndex
  (params (FluxIndex :type Integer))
  (bind _returnvalue (Math|Color|MakeColor 0.0 1.0 0.0))
  (bind _fluxarray (Variables|Default|GetFluxArray))
  (bind _output (Utilities|Array|Get(acopy) _fluxarray FluxIndex))
  (bind _spline (Variables|/Game/Blueprints/0_GrayRoom/AlexMess/Grayroom_Flux/Blueprint/BP_GRFluxDrawer.BP_GRFluxDrawer_C|GetSpline _output))
  ;[1 1 1] OnFluxDeselected
  (Class|SplineComponent|SetUnselectedSplineSegmentColor _spline _returnvalue)
  (Class|SplineComponent|SetSelectedSplineSegmentColor _spline _returnvalue)
  (Spline|UpdateSpline _spline))

(event Custom|CreateFluxPos
  (params (Destination :type Vector))
  ;[1 1 1] CreateFluxPos
  (bind _returnvalue (Game|SpawnActorfromClass "/Game/Blueprints/0_GrayRoom/AlexMess/Grayroom_Flux/Blueprint/BP_GRFluxDrawer.BP_GRFluxDrawer_C" (Math|Transform|MakeTransform "0.000000,0.000000,50.000000") "Undefined" "MultiplyWithRoot" 0 0))
  (Utilities|Array|Add (Variables|Default|GetFluxArray) _returnvalue)
  (Utilities|Array|Add (Variables|/Game/Blueprints/0_GrayRoom/AlexMess/Grayroom_Flux/Blueprint/BP_GRFluxDrawer.BP_GRFluxDrawer_C|GetPoints _returnvalue) (Transformation|GetActorLocation))
  (Utilities|Array|Add (Variables|/Game/Blueprints/0_GrayRoom/AlexMess/Grayroom_Flux/Blueprint/BP_GRFluxDrawer.BP_GRFluxDrawer_C|GetPoints _returnvalue) Destination)
  (Default|BuildSpline _returnvalue self)
  (CallFunction|UpdateFluxesOutput))

(event Custom|EnterBuildMode
  ;[1 1 1] EnterBuildMode
  (Rendering|Material|SetMaterial (Variables|Default|GetCube) 0 "/Game/Blueprints/0_GrayRoom/AlexMess/Grayroom_Flux/Materials/M_GRBaseBuildMode.M_GRBaseBuildMode"))

(event Custom|EnterEditMode
  ;[1 1 1] EnterEditMode
  (Rendering|Material|SetMaterial (Variables|Default|GetCube) 0 "/Game/Blueprints/0_GrayRoom/AlexMess/Grayroom_Flux/Materials/M_GRBaseEditMode.M_GRBaseEditMode"))

(event Custom|CreateFlux
  (params (Destination :type BP%20GR%20Base%20Object%20Reference))
  ;[1 1 1] CreateFlux
  (bind _returnvalue (Game|SpawnActorfromClass "/Game/Blueprints/0_GrayRoom/AlexMess/Grayroom_Flux/Blueprint/BP_GRFluxDrawer.BP_GRFluxDrawer_C" (Math|Transform|MakeTransform "0.000000,0.000000,50.000000") "Undefined" "MultiplyWithRoot" 0 0))
  (Utilities|Array|Add (Variables|Default|GetFluxArray) _returnvalue)
  (Utilities|Array|Add (Variables|/Game/Blueprints/0_GrayRoom/AlexMess/Grayroom_Flux/Blueprint/BP_GRFluxDrawer.BP_GRFluxDrawer_C|GetPoints _returnvalue) (Transformation|GetActorLocation))
  (Utilities|Array|Add (Variables|/Game/Blueprints/0_GrayRoom/AlexMess/Grayroom_Flux/Blueprint/BP_GRFluxDrawer.BP_GRFluxDrawer_C|GetPoints _returnvalue) (Transformation|GetActorLocation Destination))
  (Default|BuildSpline _returnvalue self)
  (CallFunction|UpdateFluxesOutput))

(event Custom|DestroyFlux
  (params (FluxIndex :type Integer))
  (bind _fluxarray (Variables|Default|GetFluxArray))
  (bind _fluxarray_2 (Variables|Default|GetFluxArray))
  (bind _output (Utilities|Array|Get(acopy) _fluxarray_2 FluxIndex))
  ;[1 1 1] DestroyFlux
  (Utilities|IsValid _output
    (:Is%20Valid
      (for _index (range 0 (- (Utilities|Array|Length (Variables|/Game/Blueprints/0_GrayRoom/AlexMess/Grayroom_Flux/Blueprint/BP_GRFluxDrawer.BP_GRFluxDrawer_C|GetNodes _output)) 1))
        (Actor|DestroyActor (Utilities|Array|Get(acopy) (Variables|/Game/Blueprints/0_GrayRoom/AlexMess/Grayroom_Flux/Blueprint/BP_GRFluxDrawer.BP_GRFluxDrawer_C|GetNodes (Utilities|Array|Get(acopy) (Variables|Default|GetFluxArray) FluxIndex)) _index)))
      (Actor|DestroyActor (Utilities|Array|Get(acopy) _fluxarray FluxIndex))
      (Utilities|Array|RemoveIndex _fluxarray FluxIndex)
      (CallFunction|UpdateFluxesOutput))
    (:Is%20Not%20Valid
      (Development|PrintString "Hello"))))

(event EventBeginPlay
  (bind _units (Variables|Default|GetUnits))
  (bind _returnvalue (Rendering|Material|CreateDynamicMaterialInstance "/Game/Blueprints/0_GrayRoom/AlexMess/Grayroom_Flux/Materials/M_GRTeam.M_GRTeam" "None" "None" :!class /Script/Engine.KismetMaterialLibrary))
  (bind _output_get (Variables|Default|SetTeamMaterial _returnvalue))
  (Rendering|Material|SetVectorParameterValue _output_get "Base Color" (Utilities|Select :Index (Variables|Default|GetTeam) :Option%200 "(R=1.000000,G=0.021699,B=0.000000,A=1.000000)" :Option%201 "(R=0.009358,G=0.000000,B=1.000000,A=1.000000)" :Option%202 "(R=1.000000,G=0.876216,B=0.000000,A=1.000000)" :Option%203 "(R=0.076735,G=1.000000,B=0.000000,A=1.000000)") :!class /Script/Engine.MaterialInstanceDynamic)
  (Rendering|Material|SetMaterial (Variables|Default|GetCube1) 0 (Variables|Default|GetTeamMaterial))
  (Rendering|Material|SetMaterial (Variables|Default|GetCube2) 0 (Variables|Default|GetTeamMaterial))
  (Rendering|Material|SetMaterial (Variables|Default|GetCube3) 0 (Variables|Default|GetTeamMaterial))
  (Rendering|Material|SetMaterial (Variables|Default|GetCube4) 0 (Variables|Default|GetTeamMaterial))
  (Rendering|Material|SetMaterial (Variables|Default|GetCube5) 0 (Variables|Default|GetTeamMaterial))
  (Rendering|Material|SetMaterial (Variables|Default|GetCube) 0 (Variables|Default|GetTeamMaterial))
  (Variables|Default|SetPossession (Variables|Default|GetPossessionMax))
  (for (_array_element _array_index) _units
    (Utilities|Array|SetArrayElem _units _array_index (Utilities|Struct|MakeSTRUCT_GRBaseArmyUnitSelection (Utilities|Struct|MakeSTRUCT_GRArmyAmalgam (.blueprintunit (.Unit (Utilities|Struct|BreakSTRUCT_GRBaseArmyUnitSelection _array_element))) (.damage (.Unit (Utilities|Struct|BreakSTRUCT_GRBaseArmyUnitSelection _array_element))) (.health (.Unit (Utilities|Struct|BreakSTRUCT_GRBaseArmyUnitSelection _array_element))) (.range (.Unit (Utilities|Struct|BreakSTRUCT_GRBaseArmyUnitSelection _array_element))) self) (.Proportion (Utilities|Struct|BreakSTRUCT_GRBaseArmyUnitSelection _array_element))))))

(event EventTick
  (params (DeltaSeconds :type Float%20%28single-precision%29))
  (bind _fluxarray (Variables|Default|GetFluxArray))
  (bind _returnvalue (Utilities|Array|Length _fluxarray))
  (Utilities|FlowControl|Sequence
    (:then_0
      (if (> (Variables|Default|GetSpawnTimer) (Variables|Default|GetSpawnThreshold))
        (Variables|Default|SetSpawnTimer (+ 0.0 DeltaSeconds))
        (bind _result (Math|Integer|IncrementInt (Variables|Default|GetSpawnCount))
          (:%20%20
            (if (> _returnvalue 0) :!label _label
              (Utilities|IsValid (Utilities|Array|Get(acopy) _fluxarray (Math|Integer|%(Integer) _result _returnvalue))
                (:Is%20Valid
                  (Default|SpawnUnit (Utilities|Array|Get(acopy) _fluxarray (Math|Integer|%(Integer) _result _returnvalue))))
                (:Is%20Not%20Valid
                  (Utilities|Array|RemoveItem _fluxarray (Utilities|Array|Get(acopy) _fluxarray (Math|Integer|%(Integer) _result _returnvalue)))
                  (goto _label))))))
        (else
          (Variables|Default|SetSpawnTimer (+ (Variables|Default|GetSpawnTimer) DeltaSeconds)))))
    (:then_1
      (switch Utilities|FlowControl|Switch|SwitchonENUM_GRBaseState (Variables|Default|GetBaseState)
        (:NewEnumerator0
          (Development|PrintString "Base State is \"None\""))
        (:NewEnumerator3
          ;[1 1 1] Recover Case
          (if (> (Variables|Default|GetPossessionMax) (Variables|Default|GetPossession))
            (Variables|Default|SetPossession (+ (Variables|Default|GetPossession) 0.75))
            (else
              (Variables|Default|SetBaseState "NewEnumerator1"))))
        (:NewEnumerator2
          ;[1 1 1] Siege Case
          (bind _output_get (Variables|Default|SetSiegeEndTimer (+ (Variables|Default|GetSiegeEndTimer) DeltaSeconds)))
          (if (< (Variables|Default|GetSiegeEndThreshold) _output_get)
            (Variables|Default|SetBaseState "NewEnumerator3")))))))

(fn ConstructionScript)

(fn GetSplineRef2
  (return (Variables|/Game/Blueprints/0_GrayRoom/AlexMess/Grayroom_Flux/Blueprint/BP_GRFluxDrawer.BP_GRFluxDrawer_C|GetSpline (Utilities|Array|Get(acopy) (Variables|Default|GetFluxArray)))))