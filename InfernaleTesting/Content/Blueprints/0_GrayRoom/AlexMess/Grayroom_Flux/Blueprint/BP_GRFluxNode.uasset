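; BP_GRFluxNode is a gray-room prototype actor for an editable node in a Flux object.
; UpdateLocation passes its NodeIndex and new position to the given Flux, then moves the actor there.
; Selection swaps the cylinder between an edit-mode material and the basic shape material and fires a FluxNodeSelected dispatcher; selecting also prints its name.
; RemoveNode only fires FluxNodeRemoved, leaving removal to listeners.
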(event Custom|UpdateLocation
  (params (Flux :type BP%20GR%20Flux%20Drawer%20Object%20Reference) (NewPosition :type Vector))
  ;[1 1 1] UpdateLocation
  (Default|UpdateNode Flux (Variables|Default|GetNodeIndex) NewPosition)
  (Transformation|SetActorLocation NewPosition false false))

(event Custom|OnSelected
  (bind _self self)
  ;[1 1 1] OnSelected
  (Rendering|Material|SetMaterial (Variables|Default|GetCylinder) 0 "/Game/Blueprints/0_GrayRoom/AlexMess/Grayroom_Flux/Materials/M_GRBaseEditMode.M_GRBaseEditMode")
  (Default|CallFluxNodeSelected true _self)
  (Development|PrintString (Utilities|GetDisplayName _self) true true "(R=0.000000,G=1.000000,B=0.179567,A=1.000000)"))

(event Custom|OnDeselected
  ;[1 1 1] OnDeselected
  (Rendering|Material|SetMaterial (Variables|Default|GetCylinder) 0 "/Engine/BasicShapes/BasicShapeMaterial.BasicShapeMaterial")
  (Default|CallFluxNodeSelected false self))

(event Custom|RemoveNode
  (Default|CallFluxNodeRemoved self))

(fn ConstructionScript)