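; BP_GRInfernalePawn is a player pawn that lets primary mouse input drive in-world widgets through a Widget Interaction component.
; On BeginPlay it assigns start and end callbacks to the Infernale player controller's primary mouse action.
; These callbacks press and release the left mouse button as a virtual pointer key on the component, so the controller owns input and the pawn only forwards clicks.
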(event Custom|SubscribeWidgetInteractionEvent
  (bind _playercontrollerinfernale (Variables|Default|GetPlayerControllerInfernale))
  (EventDispatchers|AssignMousePrimaryStart _playercontrollerinfernale (delegate Custom|MousePrimaryStart_Event))
  (EventDispatchers|AssignMousePrimaryEnd _playercontrollerinfernale (delegate Custom|MousePrimaryEnd_Event)))

(event Custom|MousePrimaryStart_Event
  (Class|WidgetInteractionComponent|PressPointerKey (Variables|Default|GetWidgetInteraction) "LeftMouseButton"))

(event Custom|MousePrimaryEnd_Event
  (Class|WidgetInteractionComponent|ReleasePointerKey (Variables|Default|GetWidgetInteraction) "LeftMouseButton"))

(event EventBeginPlay
  (CallFunction|SubscribeWidgetInteractionEvent))

(fn ConstructionScript)