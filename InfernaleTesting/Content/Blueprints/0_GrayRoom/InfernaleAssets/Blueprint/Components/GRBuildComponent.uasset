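; Player controller component for selecting and editing build spots, plus debug placement of bases and spots.
; In mode None, right-click toggles or switches the edited BP_GRBuildSpot, and EditCurrent forwards build IDs to it.
; Debug toggles rebind mouse input: left-click spawns or grabs, right-click destroys.
; Dragging follows cursor traces while pawn look is suspended; DebugBuildSpot's modes look inverted, setting None when activated.
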(event Custom|EditCurrent
  (params (BuidId :type Integer))
  (bind _buildspot (Variables|Default|GetBuildSpot))
  (Utilities|IsValid _buildspot
    (:Is%20Valid
      (Default|EditCurrent _buildspot BuidId))))

(event Custom|ChangeBuildMode
  (params (NewMode :type EBuildModeGR%20Enum :default "DebugCreateSpot"))
  ;[1 1 1] ChangeBuildMode
  (Variables|Default|SetCurrentMode NewMode)
  (CallFunction|StopEditing))

(event Custom|BuildBaseSecondary
  (bind (_hit _result) (Default|MousePosonWorld (Variables|Default|GetBP%20Player%20Controller%20Infernale) "TraceTypeQuery1" 0 "None"))
  (if _hit
    (bind _asbp_grbase (Utilities|Casting|CastToBP_GRBase (.HitActor (Collision|BreakHitResult _result))))
    (Actor|DestroyActor _asbp_grbase)))

(event Custom|DebugBuildBase
  (params (Activated :type Boolean))
  ;[1 1 1] DebugBuildBase
  (if Activated
    (CallFunction|DebugBuildBaseStart)
    (CallFunction|ChangeBuildMode "CreateBase")
    (else
      (CallFunction|DebugBuildBaseEnd)
      (CallFunction|ChangeBuildMode "None"))))

(event Custom|DebugBuildBaseStart
  (bind _bp_player_controller_infernale (Variables|Default|GetBP%20Player%20Controller%20Infernale))
  (EventDispatchers|BindEventtoMousePrimaryStart _bp_player_controller_infernale (delegate Custom|BuildBasePrimary))
  (EventDispatchers|BindEventtoMouseSecondaryStart _bp_player_controller_infernale (delegate Custom|BuildBaseSecondary)))

(event Custom|DebugBuildBaseEnd
  (bind _bp_player_controller_infernale (Variables|Default|GetBP%20Player%20Controller%20Infernale))
  ;[1 1 1] DebugBuildBaseEnd
  (EventDispatchers|UnbindEventfromMousePrimaryStart _bp_player_controller_infernale (delegate Custom|BuildBasePrimary))
  (EventDispatchers|UnbindEventfromLookTriggered _bp_player_controller_infernale (delegate Custom|LookBuild))
  (EventDispatchers|UnbindEventfromMousePrimaryEnd _bp_player_controller_infernale (delegate Custom|MousePrimaryEnd_Build))
  (EventDispatchers|UnbindEventfromMouseSecondaryStart _bp_player_controller_infernale (delegate Custom|BuildBaseSecondary))
  (Class|GRInfernalePawn|SubscribetoLookEvents (Variables|/Script/InfernaleTesting.GRPlayerControllerInfernale|GetInfernalePawn _bp_player_controller_infernale)))

(event Custom|MouseSecondaryStart_Event_0
  ;[1 1 1] DebugBuildStart
  (bind (_hit _result) (Default|MousePosonWorld (Variables|Default|GetBP%20Player%20Controller%20Infernale) "TraceTypeQuery1" 0 "None"))
  (if _hit
    (bind _asbp_grbuild_spot (Utilities|Casting|CastToBP_GRBuildSpot (.HitActor (Collision|BreakHitResult _result))))
    (Actor|DestroyActor _asbp_grbuild_spot)))

(event Custom|BuildBasePrimary
  (bind _bp_player_controller_infernale (Variables|Default|GetBP%20Player%20Controller%20Infernale))
  (bind _bp_player_controller_infernale_2 (Variables|Default|GetBP%20Player%20Controller%20Infernale))
  (bind (_hit _result) (Default|MousePosonWorld (Variables|Default|GetBP%20Player%20Controller%20Infernale) "TraceTypeQuery1" 0 "None"))
  (if _hit
    (bind _asbp_grbase (Utilities|Casting|CastToBP_GRBase (.HitActor (Collision|BreakHitResult _result)))
      (:then
        (Variables|Default|SetBase _asbp_grbase)
        (Variables|Default|SetBuildSpot 0)
        (Class|GRInfernalePawn|UnsubscribefromLookEvents (Variables|/Script/InfernaleTesting.GRPlayerControllerInfernale|GetInfernalePawn _bp_player_controller_infernale) :!label _label)
        (EventDispatchers|BindEventtoLookTriggered _bp_player_controller_infernale_2 (delegate Custom|LookBuild))
        (EventDispatchers|AssignMousePrimaryEnd _bp_player_controller_infernale_2 (delegate Custom|MousePrimaryEnd_Build)))
      (:CastFailed
        (bind (_hit_2 _result_2 _pos) (Default|MousePosonWorld (Variables|Default|GetBP%20Player%20Controller%20Infernale) "TraceTypeQuery3" 0 "None" :!label _label_2))
        (if _hit_2
          ;[1 1 1] Mult will change this
          (bind _returnvalue (Game|SpawnActorfromClass "/Game/Blueprints/0_GrayRoom/AlexMess/Grayroom_Flux/Blueprint/BP_GRBase.BP_GRBase_C" (Math|Transform|MakeTransform _pos) "Undefined" "MultiplyWithRoot" 0 0))
          (bind _output_get (Variables|Default|SetBase _returnvalue))
          (Default|UpdateTeam _output_get (Math|Conversions|ToByte(Integer) (Variables|/Game/Blueprints/0_GrayRoom/InfernaleAssets/Blueprint/UI/WBP_GRDebugMenu.WBP_GRDebugMenu_C|GetTeam (Variables|/Game/Blueprints/0_GrayRoom/InfernaleAssets/Blueprint/GameMode/Game/BP_GRPlayerControllerInfernale.BP_GRPlayerControllerInfernale_C|GetDebugMenu _bp_player_controller_infernale))))
          (goto _label))))
    (else
      (goto _label_2))))

(event Custom|OnPrimaryStart
  (bind _bp_player_controller_infernale (Variables|Default|GetBP%20Player%20Controller%20Infernale))
  (bind (_hit _result) (Default|MousePosonWorld (Variables|Default|GetBP%20Player%20Controller%20Infernale) "TraceTypeQuery1" 0 "None"))
  (if _hit
    (bind _asbp_grbuild_spot (Utilities|Casting|CastToBP_GRBuildSpot (.HitActor (Collision|BreakHitResult _result)))
      (:then
        (Variables|Default|SetBuildSpot _asbp_grbuild_spot)
        (Class|GRInfernalePawn|UnsubscribefromLookEvents (Variables|/Script/InfernaleTesting.GRPlayerControllerInfernale|GetInfernalePawn (Variables|Default|GetBP%20Player%20Controller%20Infernale)) :!label _label)
        (EventDispatchers|BindEventtoLookTriggered _bp_player_controller_infernale (delegate Custom|Looked))
        (EventDispatchers|AssignMousePrimaryEnd _bp_player_controller_infernale (delegate Custom|MousePrimaryEnd_Event)))
      (:CastFailed
        (bind (_hit_2 _result_2 _pos) (Default|MousePosonWorld (Variables|Default|GetBP%20Player%20Controller%20Infernale) "TraceTypeQuery3" 0 "None" :!label _label_2))
        (if _hit_2
          ;[1 1 1] Mult will change this
          (bind _returnvalue (Game|SpawnActorfromClass "/Game/Blueprints/0_GrayRoom/InfernaleAssets/Blueprint/Build/BP_GRBuildSpot.BP_GRBuildSpot_C" (Math|Transform|MakeTransform _pos) "Undefined" "MultiplyWithRoot" 0 0))
          (Variables|Default|SetBuildSpot _returnvalue)
          (goto _label))))
    (else
      (goto _label_2))))

(event Custom|MousePrimaryEnd_Event
  ;[1 1 1] MousePrimaryEnd_Event
  (CallFunction|DebugBuildSpotFinish)
  (EventDispatchers|UnbindEventfromMousePrimaryEnd (Variables|Default|GetBP%20Player%20Controller%20Infernale) (delegate Custom|MousePrimaryEnd_Event)))

(event Custom|DebugBuildSpot
  (params (Activated :type Boolean))
  ;[1 1 1] DebugBuildSpot
  (if Activated
    (CallFunction|DebugBuildStart)
    (CallFunction|ChangeBuildMode "None")
    (else
      (CallFunction|DebugBuildSpotEnd)
      (CallFunction|ChangeBuildMode "DebugCreateSpot"))))

(event Custom|DebugBuildSpotFinish
  ;[1 1 1] DebugBuildSpotFinish
  (EventDispatchers|UnbindEventfromLookTriggered (Variables|Default|GetBP%20Player%20Controller%20Infernale) (delegate Custom|Looked))
  (Class|GRInfernalePawn|SubscribetoLookEvents (Variables|/Script/InfernaleTesting.GRPlayerControllerInfernale|GetInfernalePawn (Variables|Default|GetBP%20Player%20Controller%20Infernale))))

(event Custom|Looked
  (params (Look :type Vector%202D%20Structure))
  ;[1 1 1] Looked
  (bind _pos (Default|MousePosonWorld (Variables|Default|GetBP%20Player%20Controller%20Infernale) "TraceTypeQuery3" 0 "None"))
  (Transformation|SetActorLocation (Variables|Default|GetBuildSpot) _pos false false))

(event Custom|DebugBuildSpotEnd
  (bind _bp_player_controller_infernale (Variables|Default|GetBP%20Player%20Controller%20Infernale))
  ;[1 1 1] DebugBuildSpotEnd
  (EventDispatchers|UnbindEventfromMousePrimaryStart _bp_player_controller_infernale (delegate Custom|OnPrimaryStart))
  (EventDispatchers|UnbindEventfromLookTriggered _bp_player_controller_infernale (delegate Custom|Looked))
  (EventDispatchers|UnbindEventfromMousePrimaryEnd _bp_player_controller_infernale (delegate Custom|MousePrimaryEnd_Event))
  (EventDispatchers|UnbindEventfromMouseSecondaryStart _bp_player_controller_infernale (delegate Custom|MouseSecondaryStart_Event_0))
  (Class|GRInfernalePawn|SubscribetoLookEvents (Variables|/Script/InfernaleTesting.GRPlayerControllerInfernale|GetInfernalePawn _bp_player_controller_infernale)))

(event Custom|BuildBaseFinish
  ;[1 1 1] BuildBaseFinish
  (EventDispatchers|UnbindEventfromLookTriggered (Variables|Default|GetBP%20Player%20Controller%20Infernale) (delegate Custom|LookBuild))
  (Class|GRInfernalePawn|SubscribetoLookEvents (Variables|/Script/InfernaleTesting.GRPlayerControllerInfernale|GetInfernalePawn (Variables|Default|GetBP%20Player%20Controller%20Infernale))))

(event Custom|LookBuild
  (params (Look :type Vector%202D%20Structure))
  ;[1 1 1] Looked
  (bind _pos (Default|MousePosonWorld (Variables|Default|GetBP%20Player%20Controller%20Infernale) "TraceTypeQuery3" 0 "None"))
  (Transformation|SetActorLocation (Variables|Default|GetBase) _pos false false))

(event Custom|MousePrimaryEnd_Build
  ;[1 1 1] MousePrimaryEnd_Event
  (CallFunction|BuildBaseFinish)
  (EventDispatchers|UnbindEventfromMousePrimaryEnd (Variables|Default|GetBP%20Player%20Controller%20Infernale) (delegate Custom|MousePrimaryEnd_Build)))

(event Custom|DebugBuildStart
  (bind _bp_player_controller_infernale (Variables|Default|GetBP%20Player%20Controller%20Infernale))
  ;[1 1 1] DebugBuildStart
  (EventDispatchers|BindEventtoMousePrimaryStart _bp_player_controller_infernale (delegate Custom|OnPrimaryStart))
  (EventDispatchers|AssignMouseSecondaryStart _bp_player_controller_infernale (delegate Custom|MouseSecondaryStart_Event_0)))

(event Custom|MouseSecondaryStart_Event
  ;[1 1 1] BeginPlay
  (CallFunction|SecondaryStart))

(event Custom|SecondaryStart
  ;[1 1 1] SecondaryStart (EditMode)
  (switch Utilities|FlowControl|Switch|SwitchonEBuildModeGR (Variables|Default|GetCurrentMode)
    (:None
      (bind (_hit _result) (Default|MousePosonWorld (Variables|Default|GetBP%20Player%20Controller%20Infernale) "TraceTypeQuery1" 0 "ForDuration"))
      (if _hit
        ;;[1 1 1] Does implement interface?
        (bind _asbp_grbuild_spot (Utilities|Casting|CastToBP_GRBuildSpot (.HitActor (Collision|BreakHitResult _result))))
        (if (Utilities|IsValid (Variables|Default|GetBuildSpot))
          (if (== (Variables|Default|GetBuildSpot) _asbp_grbuild_spot)
            (CallFunction|StopEditing)
            (else
              (CallFunction|StopEditing)
              (bind _output_get (Variables|Default|SetBuildSpot _asbp_grbuild_spot :!label _label))
              (Default|StartEdit _output_get)))
          (else
            (goto _label)))))))

(event EventBeginPlay
  ;[1 1 1] BeginPlay
  (bind _output_get (Variables|Default|SetBP%20Player%20Controller%20Infernale (.AsBP%20GRPlayer%20Controller%20Infernale (Utilities|Casting|CastToBP_GRPlayerControllerInfernale (Components|GetOwner)))))
  (EventDispatchers|AssignMouseSecondaryStart _output_get (delegate Custom|MouseSecondaryStart_Event)))

(fn StopEditing
  (Utilities|IsValid (Variables|Default|GetBuildSpot)
    (:Is%20Valid
      (Default|StopEdit (Variables|Default|GetBuildSpot))
      (Variables|Default|SetBuildSpot 0))
    (:Is%20Not%20Valid
      _))
  (return))