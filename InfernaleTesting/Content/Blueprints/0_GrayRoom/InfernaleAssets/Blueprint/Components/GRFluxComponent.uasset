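; Player controller component for drawing and editing fluxes, the spline routes that army units follow from bases.
; Mouse events route through Build mode, which selects bases and creates fluxes at clicked points, and Edit mode, entered on node selection.
; Edit mode reroutes end nodes, inserts and drags nodes while updating units, and removes nodes or, on a timed hold, whole fluxes.
; Tick runs that timer and snaps a preview node onto selected splines near the cursor.
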(event Custom|FluxModeStart
  (bind _bp_player_controller_infernale (Variables|Default|GetBP%20Player%20Controller%20Infernale))
  ;[1 1 1] FluxModeStart
  (CallFunction|ChangeMode "Build")
  (EventDispatchers|BindEventtoMousePrimaryStart _bp_player_controller_infernale (delegate Custom|MousePrimaryEnd_Event))
  (EventDispatchers|BindEventtoMousePrimaryEnd _bp_player_controller_infernale (delegate Custom|MouseSecondaryEnd_Event)))

(event Custom|FluxModeEnd
  (bind _bp_player_controller_infernale (Variables|Default|GetBP%20Player%20Controller%20Infernale))
  ;[1 1 1] FluxModeEnd
  (EventDispatchers|UnbindEventfromMousePrimaryStart _bp_player_controller_infernale (delegate Custom|MousePrimaryEnd_Event))
  (EventDispatchers|UnbindEventfromMouseSecondaryStart _bp_player_controller_infernale (delegate Custom|MouseSecondaryEnd_Event))
  (CallFunction|ChangeMode "None"))

(event Custom|ExitLastMode
  ;[1 1 1] ChangeMode
  (switch Utilities|FlowControl|Switch|SwitchonEFluxModeGR (Variables|Default|GetCurrentMode)
    (:Edit
      (CallFunction|DeselectAllFluxes)
      (CallFunction|AddNodeVisual false))))

(event Custom|SecondaryStartBuild
  ;[1 1 1] SecondaryStartBuild
  (if (Utilities|Array|IsNotEmpty (Variables|Default|GetSelectedBasesOrigin))
    (bind (_hit _result _pos) (Default|MousePosonWorld (Variables|Default|GetBP%20Player%20Controller%20Infernale) "TraceTypeQuery1" 0 "None"))
    (if _hit
      (for _array_element (Variables|Default|GetSelectedBasesOrigin)
        (Default|CreateFluxPos _array_element _pos)))
    (else
      (Development|PrintString "No base selected"))))

(event Custom|PrimaryStartBuild
  ;[1 1 1] PrmaryStarBuild
  (bind _clickedonbase (CallFunction|AddBasetoSelection))
  (if (not _clickedonbase)
    (CallFunction|CheckforNode true)))

(event Custom|NodeSelected
  (params (Selected :type Boolean) (Node :type BP%20GR%20Flux%20Node%20Object%20Reference) (Flux :type BP%20GR%20Flux%20Drawer%20Object%20Reference))
  (bind _struct_grfluxnode (Utilities|Struct|MakeSTRUCT_GRFluxNode Node Flux))
  (bind (_fluxnode _fluxdrawer) (Utilities|Struct|BreakSTRUCT_GRFluxNode _struct_grfluxnode))
  ;[1 1 1] NodeSelected
  (if Selected
    (if (CallFunction|FluxNodeAlreadySelected _struct_grfluxnode)
      (CallFunction|DeselectNodeandFlux _struct_grfluxnode)
      (else
        (CallFunction|DeselectNodeandFlux _struct_grfluxnode)
        (Utilities|Array|AddUnique (Variables|Default|GetSelectedFluxes) _struct_grfluxnode)
        (Default|OnFluxSelected (Variables|/Game/Blueprints/0_GrayRoom/AlexMess/Grayroom_Flux/Blueprint/BP_GRFluxDrawer.BP_GRFluxDrawer_C|GetOrigin _fluxdrawer) _fluxdrawer)
        (CallFunction|ChangeMode "Edit")
        (Development|PrintString "Hello")))))

(event Custom|DeselectNodeAndFlux
  (params (Flux :type STRUCT%20GR%20Flux%20Node%20Structure))
  (bind (_fluxnode _fluxdrawer) (Utilities|Struct|BreakSTRUCT_GRFluxNode Flux))
  ;[1 1 1] DeselectNodeAndFlux
  (if (CallFunction|FluxNodeAlreadySelected Flux)
    (Utilities|IsValid _fluxnode
      (:Is%20Valid
        (Default|OnDeselected _fluxnode))
      (:Is%20Not%20Valid
        _))
    (Utilities|IsValid _fluxdrawer
      (:Is%20Valid
        (Default|OnFluxDeselected (Variables|/Game/Blueprints/0_GrayRoom/AlexMess/Grayroom_Flux/Blueprint/BP_GRFluxDrawer.BP_GRFluxDrawer_C|GetOrigin _fluxdrawer) _fluxdrawer)))))

(event Custom|EditSecondaryCancel
  (bind _bp_player_controller_infernale (Variables|Default|GetBP%20Player%20Controller%20Infernale))
  ;[1 1 1] SecondaryStartEdit
  (EventDispatchers|UnbindEventfromMouseSecondaryEnd _bp_player_controller_infernale (delegate Custom|EditSecondaryCancel))
  (EventDispatchers|UnbindEventfromMouseSecondaryTriggered _bp_player_controller_infernale (delegate Custom|SecondaryTriggeredEdit))
  (Variables|Default|SetCurrentTime 0.0)
  (Variables|Default|SetRemoving false)
  (CallFunction|TryRemoveNode))

(event Custom|SecondaryTriggeredEdit
  ;[1 1 1] SecondaryStartEdit
  (bind (_hit _result) (Default|MousePosonWorld (Variables|Default|GetBP%20Player%20Controller%20Infernale) "TraceTypeQuery1" 0 "ForDuration"))
  (if _hit
    (Utilities|Casting|CastToBP_GRFluxNode (.HitActor (Collision|BreakHitResult _result))
      (:CastFailed
        _)))
  (CallFunction|EditSecondaryCancel))

(event Custom|TryRemoveNode
  (bind _bp_player_controller_infernale (Variables|Default|GetBP%20Player%20Controller%20Infernale))
  (bind (_hitresult _returnvalue) (Game|Player|GetHitResultUnderCursorbyChannel _bp_player_controller_infernale "TraceTypeQuery1" true))
  (if _returnvalue
    (bind _asbp_grflux_node (Utilities|Casting|CastToBP_GRFluxNode (.HitActor (Collision|BreakHitResult _hitresult)))
      (:then
        (if (not (or (Variables|/Game/Blueprints/0_GrayRoom/AlexMess/Grayroom_Flux/Blueprint/BP_GRFluxNode.BP_GRFluxNode_C|GetIsEnd _asbp_grflux_node) (Variables|/Game/Blueprints/0_GrayRoom/AlexMess/Grayroom_Flux/Blueprint/BP_GRFluxNode.BP_GRFluxNode_C|GetIsStart _asbp_grflux_node)))
          (Default|RemoveNode _asbp_grflux_node)
          (Development|PrintString "Remove")))
      (:CastFailed
        (Development|PrintString "...")))
    (else
      (Development|PrintString "Nop"))))

(event Custom|PrimaryStartEdit
  ;[1 1 1] PrimaryStartEdit
  (if (Variables|Default|GetAddNodeValid)
    (CallFunction|AddNode)
    (else
      (bind _clickedonbase (CallFunction|AddBasetoSelection))
      (if _clickedonbase
        (CallFunction|ChangeMode "Build")
        (else
          (bind (_wasnode _pos) (CallFunction|CheckforNode true))
          (if (not _wasnode)
            (CallFunction|RerouteNodes _pos)))))))

(event Custom|RerouteNodes
  (params (Pos :type Vector))
  ;[1 1 1] RerouteNodes
  (for _array_element (Variables|Default|GetSelectedFluxes)
    (if (Variables|/Game/Blueprints/0_GrayRoom/AlexMess/Grayroom_Flux/Blueprint/BP_GRFluxNode.BP_GRFluxNode_C|GetIsEnd (.FluxNode (Utilities|Struct|BreakSTRUCT_GRFluxNode _array_element)))
      (Default|UpdateLocation (.FluxNode (Utilities|Struct|BreakSTRUCT_GRFluxNode _array_element)) (.FluxDrawer (Utilities|Struct|BreakSTRUCT_GRFluxNode _array_element)) Pos)
      (Development|PrintString (Utilities|String|ToString(Vector) Pos)))))

(event Custom|FluxMode
  (params (Activated :type Boolean))
  ;[1 1 1] FluxMode
  (if Activated
    (CallFunction|FluxModeStart)
    (else
      (CallFunction|FluxModeEnd))))

(event Custom|Deselect%20All%20Fluxes
  ;[1 1 1] ChangeMode
  (for _array_element (Variables|Default|GetSelectedFluxes)
    (CallFunction|DeselectNodeandFlux _array_element)
    (Utilities|Array|RemoveItem (Variables|Default|GetSelectedFluxes) _array_element)))

(event Custom|AddNode
  (bind _bp_player_controller_infernale (Variables|Default|GetBP%20Player%20Controller%20Infernale))
  (bind _editfluxid (Variables|Default|GetEditFluxID))
  (if (and (!= _editfluxid -1) (< _editfluxid (Utilities|Array|Length (Variables|Default|GetSelectedFluxes))))
    (EventDispatchers|AssignMousePrimaryEnd _bp_player_controller_infernale (delegate Custom|MousePrimaryEnd_Event_0))
    (EventDispatchers|AssignMousePrimaryTriggered _bp_player_controller_infernale (delegate Custom|MousePrimaryTriggered_Event))
    (Variables|Default|SetIsDrag true)
    (CallFunction|CreateNode)
    (Rendering|SetVisibility (Variables|/Game/Blueprints/0_GrayRoom/AlexMess/Grayroom_Flux/Blueprint/BP_GRFluxNode.BP_GRFluxNode_C|GetScene (Variables|Default|GetEditNode)) false true)))

(event Custom|AddNodeVisual
  (params (Valid :type Boolean))
  (Variables|Default|SetAddNodeValid Valid)
  (Rendering|SetVisibility (Variables|/Game/Blueprints/0_GrayRoom/AlexMess/Grayroom_Flux/Blueprint/BP_GRFluxNode.BP_GRFluxNode_C|GetScene (Variables|Default|GetEditNode)) Valid true))

(event Custom|MousePrimaryEnd_Event_0
  (bind _bp_player_controller_infernale (Variables|Default|GetBP%20Player%20Controller%20Infernale))
  (EventDispatchers|UnbindEventfromMousePrimaryEnd _bp_player_controller_infernale (delegate Custom|MousePrimaryEnd_Event_0))
  (EventDispatchers|UnbindEventfromMousePrimaryTriggered _bp_player_controller_infernale (delegate Custom|MousePrimaryTriggered_Event))
  (CallFunction|DragNode)
  (Variables|Default|SetIsDrag false))

(event Custom|MousePrimaryTriggered_Event
  (CallFunction|DragNode))

(event Custom|DragNode
  (bind _selectedfluxes (Variables|Default|GetSelectedFluxes))
  (bind _editfluxid (Variables|Default|GetEditFluxID))
  (bind _bp_player_controller_infernale (Variables|Default|GetBP%20Player%20Controller%20Infernale))
  (bind _hitresult (Game|Player|GetHitResultUnderCursorbyChannel _bp_player_controller_infernale "TraceTypeQuery1" true))
  (bind _output (Utilities|Array|Get(acopy) _selectedfluxes _editfluxid))
  (bind _fluxdrawer (Utilities|Struct|BreakSTRUCT_GRFluxNode _output))
  (bind _impactpoint (Collision|BreakHitResult _hitresult))
  (bind (_x _y) (Math|Vector|BreakVector _impactpoint))
  (bind _units (Variables|/Game/Blueprints/0_GrayRoom/AlexMess/Grayroom_Flux/Blueprint/BP_GRFluxDrawer.BP_GRFluxDrawer_C|GetUnits _fluxdrawer))
  (Utilities|IsValid (Variables|Default|GetNewNode)
    (:Is%20Valid
      (Default|UpdateLocation (Variables|Default|GetNewNode) _fluxdrawer (Math|Vector|MakeVector _x _y 0.0))
      (for _index (range 0 (Utilities|Array|Length _units))
        (Utilities|IsValid (Utilities|Array|Get(acopy) _units _index)
          (:Is%20Valid
            (Default|CallUpdateArmyUnits (Utilities|Array|Get(acopy) _units _index)))
          (:Is%20Not%20Valid
            (Utilities|Array|RemoveItem _units (Utilities|Array|Get(acopy) _units _index))))))))

(event Custom|CreateNode
  (bind _editfluxid (Variables|Default|GetEditFluxID))
  (bind _selectedfluxes (Variables|Default|GetSelectedFluxes))
  (bind _output (Utilities|Array|Get(acopy) _selectedfluxes _editfluxid))
  (bind _fluxdrawer (Utilities|Struct|BreakSTRUCT_GRFluxNode _output))
  (bind _units (Variables|/Game/Blueprints/0_GrayRoom/AlexMess/Grayroom_Flux/Blueprint/BP_GRFluxDrawer.BP_GRFluxDrawer_C|GetUnits _fluxdrawer))
  (Default|AddNode _fluxdrawer (.ImpactPoint (Collision|BreakHitResult (.HitResult (Game|Player|GetHitResultUnderCursorbyChannel (Variables|Default|GetBP%20Player%20Controller%20Infernale) "TraceTypeQuery1" true)))))
  (for _index (range 0 (Utilities|Array|Length _units))
    (Utilities|IsValid (Utilities|Array|Get(acopy) _units _index)
      (:Is%20Valid
        (Default|CallUpdateArmyUnits (Utilities|Array|Get(acopy) _units _index)))
      (:Is%20Not%20Valid
        (Utilities|Array|RemoveItem _units (Utilities|Array|Get(acopy) _units _index)))))
  (bind _asbp_grflux_node (Utilities|Casting|CastToBP_GRFluxNode (.HitActor (Collision|BreakHitResult (.HitResult (Game|Player|GetHitResultUnderCursorbyChannel (Variables|Default|GetBP%20Player%20Controller%20Infernale) "TraceTypeQuery1" true)))))
    (:then
      (Variables|Default|SetNewNode _asbp_grflux_node))
    (:CastFailed
      (CallFunction|MousePrimaryEndEvent0))))

(event Custom|ClearSelectedBases
  ;[1 1 1] ClearSelectedBases
  (for _array_element (Variables|Default|GetSelectedBasesOrigin)
    (Default|OnDeselected _array_element))
  (Utilities|Array|Clear (Variables|Default|GetSelectedBasesOrigin))
  (for _array_element_2 (Variables|Default|GetSelectedBasesTarget)
    (Default|OnDeselected _array_element_2))
  (Utilities|Array|Clear (Variables|Default|GetSelectedBasesTarget)))

(event Custom|MousePrimaryEnd_Event
  ;[1 1 1] FluxModeStart
  (CallFunction|OnPrimaryStart))

(event Custom|MouseSecondaryEnd_Event
  ;[1 1 1] FluxModeStart
  (CallFunction|OnSecondaryStart))

(event Custom|OnPrimaryStart
  (Development|PrintString "Primary")
  (switch Utilities|FlowControl|Switch|SwitchonEFluxModeGR (Variables|Default|GetCurrentMode)
    (:Build
      (CallFunction|PrimaryStartBuild))
    (:Edit
      (CallFunction|PrimaryStartEdit))))

(event Custom|OnSecondaryStart
  (switch Utilities|FlowControl|Switch|SwitchonEFluxModeGR (Variables|Default|GetCurrentMode)
    (:Build
      (CallFunction|SecondaryStartBuild))
    (:Edit
      (CallFunction|SecondaryStartEdit))))

(event Custom|SecondaryStartEdit
  (bind _bp_player_controller_infernale (Variables|Default|GetBP%20Player%20Controller%20Infernale))
  ;[1 1 1] SecondaryStartEdit
  (EventDispatchers|BindEventtoMouseSecondaryEnd _bp_player_controller_infernale (delegate Custom|EditSecondaryCancel))
  (EventDispatchers|BindEventtoMouseSecondaryTriggered _bp_player_controller_infernale (delegate Custom|SecondaryTriggeredEdit))
  (CallFunction|DeselectAllFluxes)
  (bind _wasnode (CallFunction|CheckforNode false))
  (if _wasnode
    (Variables|Default|SetCurrentTime 0.0)
    (Variables|Default|SetRemoving true)
    (Variables|Default|SetEditFluxID -1)
    (Variables|Default|SetAddNodeValid false)))

(event Custom|ChangeMode
  (params (Mode :type EFluxModeGR%20Enum :default "Build"))
  ;[1 1 1] ChangeMode
  (if (Utilities|Enum|NotEqual(Enum) (Variables|Default|GetCurrentMode) Mode)
    (CallFunction|ClearSelectedBases)
    (CallFunction|ExitLastMode)
    (bind _output_get (Variables|Default|SetCurrentMode Mode))
    (switch Utilities|FlowControl|Switch|SwitchonEFluxModeGR _output_get)))

(event EventTick
  (params (DeltaSeconds :type Float%20%28single-precision%29))
  (bind _selectedfluxes (Variables|Default|GetSelectedFluxes))
  (bind _output (Utilities|Array|Get(acopy) _selectedfluxes))
  (bind _fluxdrawer (Utilities|Struct|BreakSTRUCT_GRFluxNode _output))
  (if (Variables|Default|GetRemoving)
    (bind _output_get (Variables|Default|SetCurrentTime (+ DeltaSeconds (Variables|Default|GetCurrentTime))))
    (if (>= _output_get (Variables|Default|GetRemoveTime))
      (Variables|Default|SetRemoving false)
      (Utilities|IsValid _fluxdrawer
        (:Is%20Valid
          (Default|DestroyFluxRef (Variables|/Game/Blueprints/0_GrayRoom/AlexMess/Grayroom_Flux/Blueprint/BP_GRFluxDrawer.BP_GRFluxDrawer_C|GetOrigin _fluxdrawer) _fluxdrawer)
          (Development|PrintString "Cancel"))
        (:Is%20Not%20Valid
          _))
      (CallFunction|DeselectAllFluxes))
    (elif (Math|Boolean|ANDBoolean (Utilities|Enum|Equal(Enum) (Variables|Default|GetCurrentMode) "Edit") (not (Variables|Default|GetIsDrag)) (not (Variables|Default|GetRemoving)))
      (bind (_closestid _closestlen _position) (CallFunction|ChecktoAddNode))
      (bind _output_get_2 (Variables|Default|SetEditFluxID _closestid))
      (CallFunction|AddNodeVisual (!= _output_get_2 -1))
      (if (!= _output_get_2 -1)
        (Transformation|SetActorLocation (Variables|Default|GetEditNode) (- _position "0.000000,0.000000,50.000000") false false))
      (else
        (Rendering|SetVisibility (Variables|/Game/Blueprints/0_GrayRoom/AlexMess/Grayroom_Flux/Blueprint/BP_GRFluxNode.BP_GRFluxNode_C|GetScene (Variables|Default|GetEditNode)) false true)))))

(event EventBeginPlay
  ;[1 1 1] BeginPlay
  (Variables|Default|SetBP%20Player%20Controller%20Infernale (.AsBP%20GRPlayer%20Controller%20Infernale (Utilities|Casting|CastToBP_GRPlayerControllerInfernale (Components|GetOwner))))
  (bind _returnvalue (Game|SpawnActorfromClass "/Game/Blueprints/0_GrayRoom/AlexMess/Grayroom_Flux/Blueprint/BP_GRFluxNode.BP_GRFluxNode_C" (Math|Transform|MakeTransform "0, 0, 0") "Undefined" "MultiplyWithRoot" 0 0))
  (bind _output_get (Variables|Default|SetEditNode _returnvalue))
  (Collision|SetActorEnableCollision _output_get false)
  (Rendering|SetVisibility (Variables|/Game/Blueprints/0_GrayRoom/AlexMess/Grayroom_Flux/Blueprint/BP_GRFluxNode.BP_GRFluxNode_C|GetScene _output_get) false true))

(fn AddBasetoSelection
  (bind _selectedbasesorigin (Variables|Default|GetSelectedBasesOrigin))
  (bind (_hit _result) (Default|MousePosonWorld (Variables|Default|GetBP%20Player%20Controller%20Infernale) "TraceTypeQuery1" 0 "ForDuration"))
  (if _hit
    (bind _asbp_grbase (Utilities|Casting|CastToBP_GRBase (.HitActor (Collision|BreakHitResult _result)))
      (:then
        (if (Utilities|Array|ContainsItem (Variables|Default|GetSelectedBasesOrigin) _asbp_grbase)
          (Utilities|Array|RemoveItem _selectedbasesorigin _asbp_grbase)
          (Default|OnDeselected _asbp_grbase)
          (return true false)
          (else
            (Utilities|Array|AddUnique _selectedbasesorigin _asbp_grbase)
            (Default|OnSelected _asbp_grbase)
            (return true true))))
      (:CastFailed
        _)))
  (return false false))

(fn CheckforNode
  (params (Select :type Boolean))
  (bind (_hit _result _pos) (Default|MousePosonWorld (Variables|Default|GetBP%20Player%20Controller%20Infernale) "TraceTypeQuery1" 0 "ForDuration"))
  (if _hit
    (bind _asbp_grflux_node (Utilities|Casting|CastToBP_GRFluxNode (.HitActor (Collision|BreakHitResult _result)))
      (:then
        (if Select
          (Default|OnSelected _asbp_grflux_node))
        (return true _pos))
      (:CastFailed
        _)))
  (return false (.ImpactPoint (Collision|BreakHitResult _result))))

(fn FluxNodeAlreadySelected
  (params (FluxNode :type STRUCT%20GR%20Flux%20Node%20Structure))
  (bind (_fluxnode _fluxdrawer) (Utilities|Struct|BreakSTRUCT_GRFluxNode FluxNode))
  (for _array_element (Variables|Default|GetSelectedFluxes)
    (if (and (== (.FluxNode (Utilities|Struct|BreakSTRUCT_GRFluxNode _array_element)) _fluxnode) (== (.FluxDrawer (Utilities|Struct|BreakSTRUCT_GRFluxNode _array_element)) _fluxdrawer))
      (return true)))
  (return false))

(fn ChecktoAddNode
  (if (Utilities|Array|IsNotEmpty (Variables|Default|GetSelectedFluxes))
    (LocalVariables|SetClosestLength 0.0)
    (LocalVariables|SetClosestIDloc -1)
    (bind (_hit _result _pos) (Default|MousePosonWorld (Variables|Default|GetBP%20Player%20Controller%20Infernale) "TraceTypeQuery3" 0 "None"))
    (if _hit
      (for (_array_element _array_index) (Variables|Default|GetSelectedFluxes)
        (if (and (<= (Math|Vector|Distance(Vector) _pos (Spline|FindLocationClosesttoWorldLocation (Variables|/Game/Blueprints/0_GrayRoom/AlexMess/Grayroom_Flux/Blueprint/BP_GRFluxDrawer.BP_GRFluxDrawer_C|GetSpline (.FluxDrawer (Utilities|Struct|BreakSTRUCT_GRFluxNode _array_element))) _pos "World")) (Variables|Default|GetMaxRangeForGrab)) (or (> (Math|Vector|Distance(Vector) _pos (Spline|FindLocationClosesttoWorldLocation (Variables|/Game/Blueprints/0_GrayRoom/AlexMess/Grayroom_Flux/Blueprint/BP_GRFluxDrawer.BP_GRFluxDrawer_C|GetSpline (.FluxDrawer (Utilities|Struct|BreakSTRUCT_GRFluxNode _array_element))) _pos "World")) (LocalVariables|GetClosestLength)) (Math|Float|NearlyEqual(Float) (LocalVariables|GetClosestLength) -1.0 1e-06)))
          (LocalVariables|SetClosestIDloc _array_index)
          (LocalVariables|SetClosestLength (Math|Vector|Distance(Vector) _pos (Spline|FindLocationClosesttoWorldLocation (Variables|/Game/Blueprints/0_GrayRoom/AlexMess/Grayroom_Flux/Blueprint/BP_GRFluxDrawer.BP_GRFluxDrawer_C|GetSpline (.FluxDrawer (Utilities|Struct|BreakSTRUCT_GRFluxNode _array_element))) _pos "World")))
          (LocalVariables|SetLocOnSpline (Spline|FindLocationClosesttoWorldLocation (Variables|/Game/Blueprints/0_GrayRoom/AlexMess/Grayroom_Flux/Blueprint/BP_GRFluxDrawer.BP_GRFluxDrawer_C|GetSpline (.FluxDrawer (Utilities|Struct|BreakSTRUCT_GRFluxNode _array_element))) _pos "World"))))))
  (return (LocalVariables|GetClosestIDloc) (LocalVariables|GetClosestLength) (LocalVariables|GetLocOnSpline)))