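; Player controller for the Infernale gray-room game mode that opens a debug menu and provides cursor and screen-space helpers.
; BeginPlay adds the menu, sets Game and UI input, runs "show splines" and binds a still-empty primary-click handler.
; MousePosOnWorld line-traces from the pawn along the deprojected cursor direction, while WorldPosToScreen returns center-relative normalized viewport coordinates.
; GetBases returns Base, which BeginPlay only ever sets to None.
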(event Custom|OnPrimaryStart)

(event EventBeginPlay
  (bind _returnvalue (UserInterface|CreateWidget "/Game/Blueprints/0_GrayRoom/InfernaleAssets/Blueprint/UI/WBP_GRDebugMenu.WBP_GRDebugMenu_C" self))
  (bind _output_get (Variables|UI|SetDebugMenu _returnvalue))
  (UserInterface|Viewport|AddtoViewport _output_get 0)
  (Input|SetInputModeGameandUI self _output_get "DoNotLock" false false)
  (EventDispatchers|BindEventtoMousePrimaryStart (delegate Custom|OnPrimaryStart))
  (bind _outactors (Actor|GetAllActorsOfClass 0))
  (if (Utilities|Array|IsNotEmpty _outactors)
    (Variables|Default|SetBase 0))
  (Development|ExecuteConsoleCommand "show splines" 0))

(fn ConstructionScript)

(fn WorldPostoScreen
  (params (WorldPos :type Vector))
  (bind (_sizex _sizey) (HUD|GetViewportSize))
  (bind _self self)
  (bind _screenposition (Class|GameplayStatics|ProjectWorldtoScreen _self WorldPos false))
  (bind (_x _y) (Math|Vector2D|BreakVector2D _screenposition))
  (return (Math|Vector2D|MakeVector2D (- (/ _x _sizex) 0.5) (- (/ _y _sizey) 0.5))))

(fn MousePosonWorld
  (params (Channel :type ETraceTypeQuery%20Enum :default "TraceTypeQuery1") (ActorsToIgnore :type Array%20of%20Actor%20Object%20References) (Debug :type EDrawDebugTrace%20Enum :default "None"))
  (bind _infernalepawn (Variables|Default|GetInfernalePawn))
  (bind _rootcomponent (Variables|/Script/Engine.Actor|GetRootComponent _infernalepawn))
  (bind _returnvalue (Transformation|GetWorldLocation _rootcomponent))
  (bind (_outhit _returnvalue_2) (Collision|LineTraceByChannel _returnvalue (* (- _returnvalue (.WorldLocation (Game|Player|ConvertMouseLocationToWorldSpace self))) 5e+04 -1.0) Channel false ActorsToIgnore Debug))
  (return _returnvalue_2 _outhit (.ImpactPoint (Collision|BreakHitResult _outhit))))

(fn GetBases
  (return (Variables|Default|GetBase)))