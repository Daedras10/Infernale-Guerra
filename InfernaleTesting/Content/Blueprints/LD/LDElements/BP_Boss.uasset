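; Boss altar level element: players sacrifice units to summon a Primal Monster, which yields Domination and Souls when killed.
; Event handlers for charge, awake, attack, death and capture drive a BP_BossSub child actor, arena decal fill, dissolve, VFX, sounds and team banners.
; Hovering swaps power widgets, shows a tooltip and highlights links to main buildings.
; It also triggers advisor checks, reward popups and a camera-offset power-scaling indicator.
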(event Custom|Hovered_Event
  (params (PlayerControllerInfernale :type Player%20Controller%20Infernale%20Object%20Reference) (bVal :type Boolean))
  (bind _result (Utilities|Text|FormatText "<img id=\"Altar\" width=\"32\" height=\"32\" stretch=\"ScaleToFit\"/><HoverTooltip_HellRed>Sacrifice </><img id=\"Units\" width=\"32\" height=\"32\" stretch=\"ScaleToFit\"/><HoverTooltip_UnitPower> UNITS</><HoverTooltip_Generic>, kill the summoned powerful </><img id=\"PrimalMonster\" width=\"32\" height=\"32\" stretch=\"ScaleToFit\"/> <HoverTooltip_MonsterPower>PRIMAL MONSTER</><HoverTooltip_Generic>,</> 
<HoverTooltip_Generic>and snatch a decisive one-time burst of </><img id=\"Domination\" width=\"24\" height=\"24\" stretch=\"ScaleToFit\"/><HoverTooltip_Domination> DOMINATION POINTS</><HoverTooltip_Generic> and </><img id=\"Souls\" width=\"24\" height=\"24\" stretch=\"ScaleToFit\"/><HoverTooltip_Souls> SOULS</><HoverTooltip_Generic>!</>"))
  (bind _self self)
  (bind _bawake (Variables|Default|GetbAwake))
  (bind _powerwidget (Variables|Default|GetPowerWidget))
  (bind _powerwidget_2 (Variables|Default|GetPowerWidget))
  (bind _uicomponent (Variables|/Script/InfernaleTesting.PlayerControllerInfernale|GetUIComponent PlayerControllerInfernale))
  (bind _cylinder (Variables|Default|GetCylinder))
  (bind _asbp_uicomponent (Utilities|Casting|CastToBP_UIComponent _uicomponent))
  (bind _hud_sandbox (Variables|/Game/Blueprints/Component/PlayerController/BP_UIComponent.BP_UIComponent_C|GetHUD%20Sandbox _asbp_uicomponent))
  (if (not (== (Variables|Default|GetisHovered) bVal))
    (Utilities|IsValid (Variables|Default|GetHUD%20Widget) :!label _label
      (:Is%20Valid
        (Default|HoveredTooltip (Variables|Default|GetHUD%20Widget) bVal _result _self 0.5))
      (:Is%20Not%20Valid
        (Utilities|IsValid _hud_sandbox
          (:Is%20Valid
            (Default|HoveredTooltip _hud_sandbox bVal _result _self 0.5))
          (:Is%20Not%20Valid
            (Variables|Default|SetHUD%20Widget (Variables|/Game/Blueprints/Component/PlayerController/BP_UIComponent.BP_UIComponent_C|GetHUD%20Widget (.AsBP%20UIComponent (Utilities|Casting|CastToBP_UIComponent (Variables|/Script/InfernaleTesting.PlayerControllerInfernale|GetUIComponent (.AsBP%20Player%20Controller%20Infernale (Utilities|Casting|CastToBP_PlayerControllerInfernale (Game|GetPlayerController 0))))))))
            (Utilities|FlowControl|Delay 0.1)
            (goto _label)))))
    (if (Variables|Default|GetisHovered)
      (bind _output_get (Variables|Default|SetisHovered bVal))
      (Rendering|SetVisibility _cylinder false false)
      (if _bawake
        (UserInterface|SetWidget _powerwidget_2 (Variables|Default|GetLow_Boss_Widget))
        (else
          (UserInterface|SetWidget _powerwidget_2 (Variables|Default|GetLow_Altar_Widget))))
      (else
        (Variables|Default|SetisHovered bVal)
        (Rendering|SetVisibility _cylinder true false)
        (if _bawake
          (UserInterface|SetWidget _powerwidget (Variables|Default|GetHigh_Boss_Widget))
          (else
            (UserInterface|SetWidget _powerwidget (Variables|Default|GetHigh_Altar_Widget))))))
    (for _array_element (Variables|Default|GetLinkedMainBuildings)
      (bind _asbp_main_building (Utilities|Casting|CastToBP_MainBuilding _array_element))
      (Default|ShowLinktoBoss _asbp_main_building _output_get))))

(event Custom|SetVFXOnOff
  (params (VFX :type Niagara%20Component%20Object%20Reference) (Switch :type Boolean))
  ;[0 0 0] SetVFXOnOff
  (if Switch
    (Components|Activation|Activate VFX false)
    (else
      (Components|Activation|Deactivate VFX))))

(event Custom|BossIdleSounds
  (Utilities|FlowControl|Delay (Math|Random|RandomFloatinRange 3.0 1e+01) :!label _label)
  (Class|SoundsDataAsset|PlaySound (Variables|Default|GetSounds%20Assets) "Boss" (Utilities|String|Append "BossIdle" (Utilities|String|ToString(Integer) (Math|Random|RandomIntegerinRange 1 7))) (Transformation|GetActorLocation))
  (if (not (Variables|Default|GetbDead))
    (goto _label)))

(event Custom|CheckConseillerBossAwake
  (Networking|SwitchHasAuthority
    (:Authority
      (for _array_element (Variables|/Game/UI/InGame/WBP_DebugHUD.WBP_DebugHUD_C|GetFloatToTextEntry (Variables|/Game/Blueprints/Component/PlayerController/BP_UIComponent.BP_UIComponent_C|GetHUD%20Widget (Variables|/Game/Blueprints/GameMode/Infernale/BP_PlayerControllerInfernale.BP_PlayerControllerInfernale_C|GetBP_UIComponent (.AsBP%20Player%20Controller%20Infernale (Utilities|Casting|CastToBP_PlayerControllerInfernale (Game|GetPlayerController 0))))))
        (if (Utilities|Enum|Equal(Enum) (.Index (Utilities|Struct|BreakBPS_FloatToTextEntry _array_element)) "Billy")
          (if (not (Variables|Default|GetConseillerDoOnce))
            (CallFunction|CheckConseillerBossAwakeMulticast)))))))

(event Custom|CheckConseillerBossAwakeMulticast
  (bind _returnvalue (Game|GetPlayerController 0))
  (bind _asbp_player_controller_infernale (Utilities|Casting|CastToBP_PlayerControllerInfernale _returnvalue))
  (bind _bp_uicomponent (Variables|/Game/Blueprints/GameMode/Infernale/BP_PlayerControllerInfernale.BP_PlayerControllerInfernale_C|GetBP_UIComponent _asbp_player_controller_infernale))
  (bind _hud_widget (Variables|/Game/Blueprints/Component/PlayerController/BP_UIComponent.BP_UIComponent_C|GetHUD%20Widget _bp_uicomponent))
  (bind _floattotextentry (Variables|/Game/UI/InGame/WBP_DebugHUD.WBP_DebugHUD_C|GetFloatToTextEntry _hud_widget))
  (for (_array_element _array_index) _floattotextentry
    (if (Utilities|Enum|Equal(Enum) (.Index (Utilities|Struct|BreakBPS_FloatToTextEntry _array_element)) "Billy")
      (bind _structout (Utilities|Struct|SetmembersinBPS_FloatToTextEntry _array_element false))
      (Utilities|Array|SetArrayElem _floattotextentry _array_index _structout))))

(event Custom|CheckForConseiller
  (bind _returnvalue (Game|GetPlayerController 0))
  (bind _asbp_player_controller_infernale (Utilities|Casting|CastToBP_PlayerControllerInfernale _returnvalue))
  (if (== (.Value (Utilities|Map|Find (Variables|Default|GetTeamCaptureData) (.Team (Utilities|Struct|BreakOwner (Class|PlayerControllerInfernale|GetOwnerInfo _asbp_player_controller_infernale))))) 0.0)
    (Default|CheckConseillerOwner (Variables|/Game/Blueprints/GameMode/Infernale/BP_PlayerControllerInfernale.BP_PlayerControllerInfernale_C|GetBP_UIComponent _asbp_player_controller_infernale) "Machin")))

(event EventVisualDamagedBP
  (params (NewHealth :type Float%20%28single-precision%29) (DamageAmount :type Float%20%28single-precision%29) (Percent :type Float%20%28single-precision%29))
  (CallFunction|ChangeBarCharge Percent "(R=1.000000,G=0.000000,B=0.014042,A=1.000000)")
  (Default|ChangeHealthValue (.AsWBP%20Boss%20Bar (Utilities|Casting|CastToWBP_BossBar (UserInterface|GetWidget (Variables|Default|GetBossHealth)))) Percent))

(event EventTick
  (params (DeltaSeconds :type Float%20%28single-precision%29))
  (bind _bosszonecontested (Variables|Default|GetBossZoneContested))
  (bind _output_get (Variables|Default|SetDisolveTarget (+ (Variables|Default|GetDisolveTarget) (* DeltaSeconds (* (/ (Variables|Default|GetSpawnChargeInPercent) 1e+02) (Variables|Default|GetMaxCutoff))))))
  (bind _asbp_boss_sub (Utilities|Casting|CastToBP_BossSub (Variables|/Script/Engine.ChildActorComponent|GetChildActor (Variables|Default|GetChildActor))))
  (Default|ChangeDisolveValue _asbp_boss_sub _output_get)
  (if (Variables|Default|GetbIsContested)
    (CallFunction|SetVFXonOff _bosszonecontested true)
    (else
      (CallFunction|SetVFXonOff _bosszonecontested false))))

(event EventToggleDetectionDecal
  (params (Hide :type Boolean))
  (if (Variables|Default|GetbAwake)
    (if Hide
      (Rendering|Components|Decal|SetDecalColor (Variables|Default|GetDetectionDecal) (Class|KismetMathLibrary|LinearColorWhite)))
    (Development|SetHiddeninGame (Variables|Default|GetDetectionDecal) Hide false)
    (else
      (Development|SetHiddeninGame (Variables|Default|GetDetectionDecal) true false))))

(event EventTriggerDetectionVFX
  (params (Scaling :type EFluxPowerScaling%20Enum :default "VeryLow") (Power :type Integer))
  (bind _scalingindicator (Variables|Default|GetScalingIndicator))
  (Development|SetHiddeninGame (Variables|Default|GetScalingIndicator) false false)
  (bind _returnvalue (UserInterface|CreateWidget "/Game/UI/InGame/WBP_PowerScaling.WBP_PowerScaling_C" (Game|GetPlayerController 0)))
  (UserInterface|SetWidget _scalingindicator _returnvalue)
  (Default|Init _returnvalue Scaling "EntityTypeBoss" self "NatureTeam" Power)
  (Transformation|AddWorldOffset _scalingindicator (CallFunction|GetOffsetScalingIndicator _scalingindicator) false false))

(event EventDisableDetectionVFX
  (bind _scalingindicator (Variables|Default|GetScalingIndicator))
  (Development|SetHiddeninGame _scalingindicator true false)
  (UserInterface|SetWidget _scalingindicator 0)
  (Transformation|SetRelativeLocation _scalingindicator "0, 0, 0" false false))

(event EventSetDetectionDecalColor
  (params (Color :type Color%20Structure))
  (Rendering|Components|Decal|SetDecalColor (Variables|Default|GetDetectionDecal) (Math|Conversions|ToLinearColor(Color) Color)))

(event EventOnSpawnChargeChangedBP
  (params (Charge :type Float%20%28single-precision%29))
  (bind _returnvalue (/ Charge 1e+02))
  (bind _returnvalue_2 (Math|Float|Clamp(Float) _returnvalue))
  (bind _output_get (Variables|Default|SetSpawnChargeInPercent _returnvalue_2))
  (CallFunction|ChangeBarCharge _output_get "(R=1.000000,G=0.000000,B=0.014042,A=1.000000)")
  (Variables|Default|SetHeightCutoffValue (* _returnvalue_2 (Variables|Default|GetMaxCutoff)))
  (Class|SoundsDataAsset|PlaySound (Variables|Default|GetSounds%20Assets) "Boss" (Utilities|String|Append "Unit Sacrificed onto Altar" (Utilities|String|ToString(Integer) (Math|Random|RandomIntegerinRange 1 7))) (Transformation|GetActorLocation))
  (CallFunction|CheckforConseiller)
  (Utilities|FlowControl|Delay 1.0)
  (Class|SoundsDataAsset|PlaySound (Variables|Default|GetSounds%20Assets) "Boss" (Utilities|String|Append "Unit Sacrificed onto Altar" (Utilities|String|ToString(Integer) (Math|Random|RandomIntegerinRange 1 7))) (Transformation|GetActorLocation)))

(event EventOnAttackChangedBP
  (params (bAttackingVal :type Boolean))
  (Variables|/Game/Blueprints/LD/LDElements/BP_BossSub.BP_BossSub_C|SetAttack (Variables|Default|GetAs%20BP%20Boss%20Sub) bAttackingVal))

(event EventOnAwakeChangedBP
  (params (bAwakeVal :type Boolean))
  (bind _bossmid (Variables|Default|GetBossMID))
  (Class|SoundsDataAsset|PlaySound (Variables|Default|GetSounds%20Assets) "Boss" "Boss Awakening" (Transformation|GetActorLocation))
  (UserInterface|SetWidget (Variables|Default|GetPowerWidget) (Variables|Default|GetLow_Boss_Widget))
  (CallFunction|SetVFXonOff (Variables|Default|GetSacrificeZone) false)
  (CallFunction|BossIdleSounds)
  (Variables|/Game/Blueprints/LD/LDElements/BP_BossSub.BP_BossSub_C|SetAwake (Variables|Default|GetAs%20BP%20Boss%20Sub) bAwakeVal)
  (Rendering|Material|SetScalarParameterValue _bossmid "general emissive" 2.0 :!class /Script/Engine.MaterialInstanceDynamic)
  (Rendering|Material|SetScalarParameterValue _bossmid "IsBreathing" 0.0 :!class /Script/Engine.MaterialInstanceDynamic)
  (Actor|Tick|SetActorTickEnabled false)
  (bind _asbp_boss_sub (Utilities|Casting|CastToBP_BossSub (Variables|/Script/Engine.ChildActorComponent|GetChildActor (Variables|Default|GetChildActor))))
  (Default|ChangeDisolveValue _asbp_boss_sub 4.5e+03)
  (Rendering|SetVisibility (Variables|Default|GetBossHealth) true false)
  (CallFunction|CheckConseillerBossAwake))

(event EventOnDeadChangedBP
  (params (bDeadVal :type Boolean))
  (Variables|/Game/Blueprints/LD/LDElements/BP_BossSub.BP_BossSub_C|SetDead (Variables|Default|GetAs%20BP%20Boss%20Sub) bDeadVal)
  (Class|SoundsDataAsset|PlaySound (Variables|Default|GetSounds%20Assets) "Boss" "Boss Death" (Transformation|GetActorLocation))
  (Rendering|SetVisibility (Variables|Default|GetPowerWidget) false false)
  (Rendering|Material|SetScalarParameterValue (Variables|Default|GetBossMID) "IsBreathing" 0.0 :!class /Script/Engine.MaterialInstanceDynamic)
  (CallFunction|SetVFXonOff (Variables|Default|GetBossIsKilled) true))

(event EventBeginPlay
  (bind _cylinder (Variables|Default|GetCylinder))
  (Actor|Tick|SetActorTickEnabled false)
  (Variables|Default|SetSounds%20Assets (.SoundsAssets (Utilities|Struct|BreakDataAssetsSettings (Utilities|Array|Get(acopy) (Variables|/Script/InfernaleTesting.GameSettingsDataAsset|GetDataAssetsSettings (Class|FunctionLibraryInfernale|GetGameSettingsDataAsset))))))
  (UserInterface|SetWidget (Variables|Default|GetPowerWidget) (Variables|Default|GetLow_Altar_Widget))
  (bind _asbp_boss_sub (Utilities|Casting|CastToBP_BossSub (Variables|/Script/Engine.ChildActorComponent|GetChildActor (Variables|Default|GetChildActor)) :!label _label)
    (:then
      (bind _output_get (Variables|Default|SetAs%20BP%20Boss%20Sub _asbp_boss_sub))
      (bind _returnvalue (Rendering|Material|CreateDynamicMaterialInstance (Variables|/Game/Blueprints/LD/LDElements/BP_BossSub.BP_BossSub_C|GetSkeletalMesh _output_get) 0 (Rendering|Material|GetMaterial (Variables|/Game/Blueprints/LD/LDElements/BP_BossSub.BP_BossSub_C|GetSkeletalMesh _output_get) 0) "None" :!class /Script/Engine.PrimitiveComponent))
      (bind _output_get_2 (Variables|Default|SetBossMID _returnvalue))
      (Rendering|Material|SetScalarParameterValue _output_get_2 "general emissive" 0.0 :!class /Script/Engine.MaterialInstanceDynamic)
      (bind _returnvalue_2 (Rendering|Material|CreateDynamicMaterialInstance (Variables|Default|GetDecalArena) :!class /Script/Engine.DecalComponent))
      (bind _output_get_3 (Variables|Default|SetDecalArenaMID _returnvalue_2))
      (Rendering|Material|SetScalarParameterValue _output_get_3 "pourcent" 0.0 :!class /Script/Engine.MaterialInstanceDynamic)
      (CallFunction|SetVFXonOff (Variables|Default|GetSacrificeZone) true)
      (Rendering|Material|SetOverlayMaterial _cylinder "/Game/_Draft/Philemon/MOI_Boss.MOI_Boss" :!class /Script/Engine.MeshComponent)
      (Rendering|SetVisibility _cylinder false false)
      (Variables|Default|SetHUD%20Widget (Variables|/Game/Blueprints/Component/PlayerController/BP_UIComponent.BP_UIComponent_C|GetHUD%20Widget (.AsBP%20UIComponent (Utilities|Casting|CastToBP_UIComponent (Variables|/Script/InfernaleTesting.PlayerControllerInfernale|GetUIComponent (.AsBP%20Player%20Controller%20Infernale (Utilities|Casting|CastToBP_PlayerControllerInfernale (Game|GetPlayerController 0))))))))
      (EventDispatchers|AssignHovered (delegate Custom|Hovered_Event))
      (bind _asbp_boss_sub_2 (Utilities|Casting|CastToBP_BossSub (Variables|/Script/Engine.ChildActorComponent|GetChildActor (Variables|Default|GetChildActor))))
      (Default|ChangeDisolveValue _asbp_boss_sub_2 0.0)
      (Development|SetHiddeninGame (Variables|Default|GetDetectionDecal) true false))
    (:CastFailed
      (Utilities|FlowControl|Delay 0.2)
      (goto _label))))

(event EventOnCaptureCompletedBP
  (params (NewOwner :type Owner%20Structure))
  (bind _neutralcamprewards (Variables|Default|GetNeutralCampRewards))
  (CallFunction|SetVFXonOff (Variables|Default|GetBossIsKilled) false)
  (CallFunction|SetBanners NewOwner)
  (if (Utilities|Enum|Equal(Enum) (.Team (Utilities|Struct|BreakOwner (Variables|/Script/InfernaleTesting.PlayerStateInfernale|GetOwnerInfo (.AsBP%20Player%20State%20Infernale (Utilities|Casting|CastToBP_PlayerStateInfernale (Game|GetPlayerState 0)))))) (.Team (Utilities|Struct|BreakOwner NewOwner)))
    (CallFunction|CreatePopUp self (Utilities|Text|ToText(Float) (.RewardValue (Utilities|Struct|BreakNeutralCampRewardData (Utilities|Array|Get(acopy) _neutralcamprewards 1))) "HalfToEven") "/Game/UI/Textures/T_DominationIcon.T_DominationIcon" 5.0)
    (Utilities|FlowControl|Delay 1.0)
    (CallFunction|CreatePopUp self (Utilities|Text|ToText(Float) (.RewardValue (Utilities|Struct|BreakNeutralCampRewardData (Utilities|Array|Get(acopy) _neutralcamprewards))) "HalfToEven") "/Game/UI/Textures/T_SoulsSimplified.T_SoulsSimplified" 5.0)
    (Utilities|FlowControl|Delay 1.0)))

(event EventUpdateCaptureBarBP
  (params (Capture :type Float%20%28single-precision%29) (Vector :type Vector%20%28by%20ref%29 :default "0, 0, 0"))
  (CallFunction|ChangeBarCharge Capture (Math|Conversions|ToLinearColor(Vector) Vector))
  (if (<= Capture 0.5)
    (bind _returnvalue (Class|SoundsDataAsset|GetSoundType (Variables|Default|GetSounds%20Assets) "Boss" (Utilities|String|Append "Boss Capturing Low" (Utilities|String|ToString(Integer) (Math|Random|RandomIntegerinRange 1 5)))))
    (Audio|SpawnSoundatLocation (.Sound (Utilities|Struct|BreakSoundType _returnvalue)) "0, 0, 0" "90.000000,0.000000,0.000000" (* (.Volume (Utilities|Struct|BreakSoundType _returnvalue)) (Variables|/Script/InfernaleTesting.GameInstanceInfernale|GetMasterXMusicVolume (.AsBP%20Game%20Instance%20Infernale (Utilities|Casting|CastToBP_GameInstanceInfernale (Game|GetGameInstance))))) 1.0 0.0 0 0)
    (else
      (bind _returnvalue_2 (Class|SoundsDataAsset|GetSoundType (Variables|Default|GetSounds%20Assets) "Boss" (Utilities|String|Append "Boss Capturing High" (Utilities|String|ToString(Integer) (Math|Random|RandomIntegerinRange 1 5)))))
      (Audio|SpawnSoundatLocation (.Sound (Utilities|Struct|BreakSoundType _returnvalue_2)) (Transformation|GetActorLocation) "90.000000,0.000000,0.000000" (* 0.0 (.Volume (Utilities|Struct|BreakSoundType _returnvalue_2))) 1.0 0.0 0 0))))

(fn ConstructionScript)

(fn ChangeBarCharge
  (params (Value :type Float%20%28single-precision%29) (Color :type Linear%20Color%20Structure))
  (bind _decalarenamid (Variables|Default|GetDecalArenaMID))
  (Rendering|Material|SetVectorParameterValue _decalarenamid "Emissive Color" Color :!class /Script/Engine.MaterialInstanceDynamic)
  (Rendering|Material|SetScalarParameterValue _decalarenamid "pourcent" Value :!class /Script/Engine.MaterialInstanceDynamic)
  (Rendering|Material|SetScalarParameterValue (Variables|Default|GetBossMID) "IsBreathing" 1.0 :!class /Script/Engine.MaterialInstanceDynamic))

(fn SetBanners
  (params (NewOwner :type Owner%20Structure))
  (bind _team (Utilities|Struct|BreakOwner NewOwner))
  (bind _banners (LocalVariables|GetBanners))
  (Utilities|Array|Add _banners (Variables|Default|GetBanner))
  (Utilities|Array|Add _banners (Variables|Default|GetBanner1))
  (Utilities|Array|Add _banners (Variables|Default|GetSM_BannerNoPole))
  (switch Utilities|FlowControl|Switch|SwitchonETeam _team
    (:Team1
      (LocalVariables|SetTeamScalarValue 0.0))
    (:Team2
      (LocalVariables|SetTeamScalarValue 0.25))
    (:Team3
      (LocalVariables|SetTeamScalarValue 0.5))
    (:Team4
      (LocalVariables|SetTeamScalarValue 0.75)))
  (for _array_element (LocalVariables|GetBanners)
    (Development|SetHiddeninGame _array_element false false)
    (Rendering|SetVisibility _array_element true false)
    (Rendering|Material|SetMaterial _array_element 0 "/Game/Character/Glutonny/Materials/MI_TeamBannerEnviroNoPole.MI_TeamBannerEnviroNoPole")
    (bind _returnvalue (Rendering|Material|CreateDynamicMaterialInstance _array_element 0 (Rendering|Material|GetMaterial _array_element 0) "None" :!class /Script/Engine.PrimitiveComponent))
    (Rendering|Material|SetScalarParameterValue _returnvalue "Team" (LocalVariables|GetTeamScalarValue) :!class /Script/Engine.MaterialInstanceDynamic)
    (Rendering|Material|SetVectorParameterValue _returnvalue "FirstTeamColor" (.SpecifiedColor (Utilities|Struct|BreakSlateColor (CallFunction|GetTeamColor _team))) :!class /Script/Engine.MaterialInstanceDynamic)
    (Rendering|Material|SetVectorParameterValue _returnvalue "SecondTeamColor" (.SpecifiedColor (Utilities|Struct|BreakSlateColor (CallFunction|GetTeamSecondColor _team))) :!class /Script/Engine.MaterialInstanceDynamic)))

(fn GetOffsetScalingIndicator
  (params (Widget :type Widget%20Component%20Object%20Reference))
  (bind _returnvalue (Game|Player|GetPlayerPawn 0))
  (bind _returnvalue_2 (Transformation|GetWorldLocation Widget))
  (bind (_x _y) (Math|Vector|BreakVector _returnvalue_2))
  (bind _asbp_infernale_pawn (Utilities|Casting|CastToBP_InfernalePawn _returnvalue))
  (bind _cameracomponent (Variables|/Script/InfernaleTesting.InfernalePawn|GetCameraComponent _asbp_infernale_pawn))
  (bind _returnvalue_3 (Transformation|GetWorldLocation _cameracomponent))
  (bind (_x_2 _y_2) (Math|Vector|BreakVector _returnvalue_3))
  (return (* (Math|Vector|Normalize (Math|Vector|MakeVector (- _x_2 _x) (- _y_2 _y) 0.0)) (Variables|/Game/UI/InGame/WBP_PowerScaling.WBP_PowerScaling_C|GetOffsetWidget (.AsWBP%20Power%20Scaling (Utilities|Casting|CastToWBP_PowerScaling (UserInterface|GetWidget Widget)))))))