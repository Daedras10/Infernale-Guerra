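; Small neutral monster camp that players slay for repeatable souls, handling the visual and audio side of damage, death and respawn.
; Visual events shrink the golems with damage, swap materials, show reward popups to the killing team and drive a radial respawn bar.
; Golems animate through static mesh and material swaps, alternating dancing and circling until attacked, with Tick restoring idle afterwards.
; Also handles hover highlight and tooltip, detection decal and power-scaling widget.
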(event Custom|Hovered_Event
  (params (PlayerControllerInfernale :type Player%20Controller%20Infernale%20Object%20Reference) (bVal :type Boolean))
  (bind _result (Utilities|Text|FormatText "<HoverTooltip_Generic>Fast-respawning </><img id=\"Monster\" width=\"32\" height=\"32\" stretch=\"ScaleToFit\"/><HoverTooltip_MonsterPower>MONSTERS</><HoverTooltip_Generic>, slay for repeatable income of </><img id=\"Souls\" width=\"24\" height=\"24\" stretch=\"ScaleToFit\"/><HoverTooltip_Souls>SOULS</>"))
  (bind _iconressources (Variables|Default|GetIconRessources))
  (bind _uicomponent (Variables|/Script/InfernaleTesting.PlayerControllerInfernale|GetUIComponent PlayerControllerInfernale))
  (bind _asbp_uicomponent (Utilities|Casting|CastToBP_UIComponent _uicomponent))
  (bind _hud_sandbox (Variables|/Game/Blueprints/Component/PlayerController/BP_UIComponent.BP_UIComponent_C|GetHUD%20Sandbox _asbp_uicomponent))
  (if (not (== (Variables|Default|GetisHovered) bVal))
    (Utilities|IsValid (Variables|Default|GetHUD%20Widget) :!label _label
      (:Is%20Valid
        (Default|HoveredTooltip (Variables|Default|GetHUD%20Widget) bVal _result self 0.5))
      (:Is%20Not%20Valid
        (Utilities|IsValid _hud_sandbox
          (:Is%20Valid
            (Default|HoveredTooltip _hud_sandbox bVal _result self 0.5))
          (:Is%20Not%20Valid
            (Variables|Default|SetHUD%20Widget (Variables|/Game/Blueprints/Component/PlayerController/BP_UIComponent.BP_UIComponent_C|GetHUD%20Widget (.AsBP%20UIComponent (Utilities|Casting|CastToBP_UIComponent (Variables|/Script/InfernaleTesting.PlayerControllerInfernale|GetUIComponent (.AsBP%20Player%20Controller%20Infernale (Utilities|Casting|CastToBP_PlayerControllerInfernale (Game|GetPlayerController 0))))))))
            (Utilities|FlowControl|Delay 0.1)
            (goto _label)))))
    (if (Variables|Default|GetIsHovered)
      (Variables|Default|SetisHovered bVal)
      (for _array_element (CallFunction|SetHighlighMesh)
        (Rendering|Material|SetOverlayMaterial _array_element 0 :!class /Script/Engine.MeshComponent)
        (UserInterface|SetWidget _iconressources (Variables|Default|GetLowWidget)))
      (else
        (Variables|Default|SetisHovered bVal)
        (for _array_element_2 (CallFunction|SetHighlighMesh)
          (Rendering|Material|SetOverlayMaterial _array_element_2 "/Game/_Draft/Philemon/MOI_NeutralCamp.MOI_NeutralCamp" :!class /Script/Engine.MeshComponent)
          (UserInterface|SetWidget _iconressources (Variables|Default|GetHighWidget)))))))

(event Custom|LoopIdleAnimation
  (bind _arrayofmesh (Variables|Default|GetArrayOfMesh))
  (bind _isattacked (Variables|Default|GetisAttacked))
  (bind _returnvalue (not _isattacked))
  (Variables|Default|SetIdleStarted true)
  (if (and (Utilities|Array|IsNotEmpty _arrayofmesh) (not (Variables|Default|GetisAttacked)))
    (for _array_element _arrayofmesh
      (Rendering|Material|SetMaterial _array_element 0 "/Game/Character/GolemGrunt/Material/MI_GolemGrunt_Idle.MI_GolemGrunt_Idle")
      (Components|StaticMesh|SetStaticMesh _array_element "/Game/Character/GolemGrunt/SK_Mob_IdleDance.SK_Mob_IdleDance"))
    (Utilities|FlowControl|Delay 2.0)
    (if _returnvalue
      (Variables|Default|SetisTurning true)
      (for _array_element_2 (Variables|Default|GetArrayOfMesh)
        (Rendering|Material|SetMaterial _array_element_2 0 "/Game/Character/GolemGrunt/Material/MI_Golem_IdleWalk.MI_Golem_IdleWalk")
        (Components|StaticMesh|SetStaticMesh _array_element_2 "/Game/Character/GolemGrunt/SM_GruntGolemIdleWalk.SM_GruntGolemIdleWalk"))
      (Utilities|FlowControl|Delay 2.0)
      (if _returnvalue
        (Variables|Default|SetisTurning false)
        (CallFunction|LoopIdleAnimation)
        (else
          (Variables|Default|SetIdleStarted false)))
      (else
        (Variables|Default|SetIdleStarted false)))))

(event Custom|SoulsCollect
  ;[1 1 1] VFX Souls collect
  (bind _returnvalue (Niagara|SpawnSystematLocation "/Game/Effects/NeutralCamp/NS_CampIsAttackedSmall.NS_CampIsAttackedSmall" (Transformation|GetWorldLocation (Variables|Transformation|GetRootComponent))))
  (bind _output_get (Variables|Default|SetNS_SoulsCollect _returnvalue))
  (Class|NiagaraComponent|SetVariableBool _output_get "IsAttacked" false))

(event Custom|NeutralCampAttackLoop
  (Utilities|FlowControl|Delay 0.75 :!label _label)
  (Class|SoundsDataAsset|PlaySound (.soundsassets (Utilities|Array|Get(acopy) (Variables|/Script/InfernaleTesting.GameSettingsDataAsset|GetDataAssetsSettings (Class|FunctionLibraryInfernale|GetGameSettingsDataAsset)))) "Monsters" (Utilities|String|Append "Monsters Attacking" (Utilities|String|ToString(Integer) (Math|Random|RandomIntegerinRange 1 2))) (Transformation|GetActorLocation))
  (if (Variables|Default|GetisAttacked)
    (goto _label)))

(event EventToggleDetectionDecal
  (params (Hide :type Boolean))
  (if Hide
    (Rendering|Components|Decal|SetDecalColor (Variables|Default|GetDetectionDecal) (Class|KismetMathLibrary|LinearColorWhite)))
  (Development|SetHiddeninGame (Variables|Default|GetDetectionDecal) Hide false))

(event EventOnDeathEffectVFXTrigger
  (params (Location :type Vector :default "0, 0, 0") (Depleter :type Owner%20Structure))
  (bind _gamesettings (Variables|Default|GetGameSettings))
  (bind _debugsettings (Variables|/Script/InfernaleTesting.GameSettingsDataAsset|GetDebugSettings _gamesettings))
  (bind _showvfxdebug (Utilities|Struct|BreakDebugSettings _debugsettings))
  ;[1 1 1] On Death Effect VFX
  (Development|PrintString "CampSmall OnDeathVFX" _showvfxdebug _showvfxdebug))

(event EventOnAttackPerformedBP
  (params (AttackHitInfo :type Attack%20Hit%20Info%20Structure%20%28by%20ref%29))
  (bind _ns_soulscollect (Variables|Default|GetNS_SoulsCollect))
  ;[1 1 1] On Attack Performed
  (Rendering|Material|SetMaterial (Variables|Default|GetArrayOfMesh) 0 "/Game/Character/GolemGrunt/Material/MI_GolemGrunt_Attack.MI_GolemGrunt_Attack")
  (Utilities|IsValid _ns_soulscollect
    (:Is%20Valid
      (Class|NiagaraComponent|SetVariableBool _ns_soulscollect "IsAttacked" true))
    (:Is%20Not%20Valid
      _))
  (Variables|Default|SetisAttacked true)
  (Variables|Default|SetIdleStarted false)
  (Variables|Default|SetLastAttackTime 0.0))

(event EventTriggerDetectionVFX
  (params (Scaling :type EFluxPowerScaling%20Enum :default "VeryLow") (Power :type Integer))
  (bind _scalingindicator (Variables|Default|GetScalingIndicator))
  (Development|SetHiddeninGame (Variables|Default|GetScalingIndicator) false false)
  (bind _returnvalue (UserInterface|CreateWidget "/Game/UI/InGame/WBP_PowerScaling.WBP_PowerScaling_C" (Game|GetPlayerController 0)))
  (UserInterface|SetWidget _scalingindicator _returnvalue)
  (Default|Init _returnvalue Scaling "EntityTypeNeutralCamp" self "NatureTeam" Power)
  (Transformation|AddWorldOffset _scalingindicator (CallFunction|GetOffsetScalingIndicator _scalingindicator) false false))

(event EventDisableDetectionVFX
  (bind _scalingindicator (Variables|Default|GetScalingIndicator))
  (Development|SetHiddeninGame _scalingindicator true false)
  (UserInterface|SetWidget _scalingindicator 0)
  (Transformation|SetRelativeLocation _scalingindicator "0, 0, 0" false false))

(event EventOnCampRespawnVFXTrigger
  (params (Location :type Vector :default "0, 0, 0"))
  (bind _gamesettings (Variables|Default|GetGameSettings))
  (bind _debugsettings (Variables|/Script/InfernaleTesting.GameSettingsDataAsset|GetDebugSettings _gamesettings))
  (bind _showvfxdebug (Utilities|Struct|BreakDebugSettings _debugsettings))
  ;[1 1 1] On Respawn VFX
  (Development|PrintString "CampSmall OnRespawnVFX" _showvfxdebug _showvfxdebug))

(event EventVisualDamagedBP
  (params (NewHealth :type Float%20%28single-precision%29) (DamageAmount :type Float%20%28single-precision%29) (Percent :type Float%20%28single-precision%29))
  (CallFunction|SetScale Percent)
  (Utilities|FlowControl|DoOnce false
    (:Completed
      (Rendering|Material|SetMaterial (Variables|Default|GetMonster4) 0 "/Game/Character/GolemGrunt/Material/MI_GolemGrunt_Attack.MI_GolemGrunt_Attack")
      (Variables|Default|SetisAttacked true))))

(event EventVisualDeathBP
  (params (Depleter :type Owner%20Structure))
  (Variables|Default|SetisTurning false)
  (Variables|Default|SetisAttacked false)
  (Class|SoundsDataAsset|PlaySound (Variables|Default|GetSounds%20Assets) "Monsters" "Monsters Dying" (Transformation|GetActorLocation))
  (Rendering|SetVisibility (Variables|Default|GetIconRessources) false false)
  (Rendering|Material|SetMaterial (Variables|Default|GetMonster4) 0 "/Game/Character/GolemGrunt/Material/M_GruntGolem_Texture_GD.M_GruntGolem_Texture_GD")
  (Widget|SetVisibility (Variables|Default|GetWBP%20Radial%20Progress%20Bar) "HitTestInvisible")
  (if (Utilities|Enum|Equal(Enum) (.Team (Utilities|Struct|BreakOwner (Variables|/Script/InfernaleTesting.PlayerStateInfernale|GetOwnerInfo (.AsBP%20Player%20State%20Infernale (Utilities|Casting|CastToBP_PlayerStateInfernale (Game|GetPlayerState 0)))))) (.Team (Utilities|Struct|BreakOwner Depleter)))
    (bind _array_element (Utilities|Array|ForEachLoopwithBreak (Variables|/Script/InfernaleTesting.NeutralCampDataAsset|GetRewardData (Variables|Default|GetNeutralCampDataAsset)))
      (:LoopBody
        (switch Utilities|FlowControl|Switch|SwitchonENeutralCampReward (.RewardType (Utilities|Struct|BreakNeutralCampRewardData _array_element))
          (:ENeutralMobRewardSouls
            (CallFunction|CreatePopUp self (Utilities|Text|ToText(Float) (.RewardValue (Utilities|Struct|BreakNeutralCampRewardData _array_element)) "HalfToEven") "/Game/UI/Textures/T_SoulsSimplified.T_SoulsSimplified" 5.0)
            (Utilities|FlowControl|Delay 0.5))
          (:ENeutralMobRewardDomination
            (CallFunction|CreatePopUp self (Utilities|Text|ToText(Float) (.RewardValue (Utilities|Struct|BreakNeutralCampRewardData _array_element)) "HalfToEven") "/Game/UI/Textures/T_DominationIcon.T_DominationIcon" 5.0)))))))

(event EventVisualRespawnBP
  (Widget|SetVisibility (Variables|Default|GetWBP%20Radial%20Progress%20Bar) "Hidden")
  (CallFunction|SetScale 1.0)
  (if (Variables|Default|GetFirstSpawned)
    (Class|SoundsDataAsset|PlaySound (Variables|Default|GetSounds%20Assets) "Monsters" "Monsters Appearing" (Transformation|GetActorLocation))
    (else
      (Variables|Default|SetFirstSpawned true)))
  (Rendering|SetVisibility (Variables|Default|GetIconRessources) true false)
  (for _array_element (Variables|Default|GetArrayOfMesh)
    (Rendering|Material|SetMaterial _array_element 0 "/Game/Character/GolemGrunt/Material/MI_GolemGrunt_Idle.MI_GolemGrunt_Idle")
    (Components|StaticMesh|SetStaticMesh _array_element "/Game/Character/GolemGrunt/SK_Mob_IdleDance.SK_Mob_IdleDance"))
  (CallFunction|LoopIdleAnimation)
  (Utilities|FlowControl|DoOnce false) ; enters at Reset
)

(event EventVisualRespawnTimeBP
  (params (TimeRemaining :type Float%20%28single-precision%29) (TotalTime :type Float%20%28single-precision%29))
  (bind _returnvalue (/ 0.0 1e+02))
  (bind _returnvalue_2 (Math|Float|Clamp(Float) _returnvalue))
  (Default|UpdatePercent (Variables|Default|GetWBP%20Radial%20Progress%20Bar) (/ TimeRemaining TotalTime))
  (Variables|Default|SetSpawnChargeInPercent _returnvalue_2)
  (Actor|Tick|SetActorTickEnabled true)
  (Variables|Default|SetHeightCutoffValue (* _returnvalue_2 (Variables|Default|GetMaxCutoff))))

(event EventBeginPlay
  (bind _returnvalue (UserInterface|CreateWidget "/Game/UI/InGame/WBP_PermanentTooltip_Monster_Small_High.WBP_PermanentTooltip_Monster_Small_High_C"))
  (Variables|Default|SetHighWidget _returnvalue)
  (bind _returnvalue_2 (UserInterface|CreateWidget "/Game/UI/InGame/WBP_PermanentTooltip_Monster_Small_Low.WBP_PermanentTooltip_Monster_Small_Low_C"))
  (bind _output_get (Variables|Default|SetLowWidget _returnvalue_2))
  (UserInterface|SetWidget (Variables|Default|GetIconRessources) _output_get)
  (CallFunction|SoulsCollect)
  (Variables|Default|SetArrayOfMesh (Utilities|Array|MakeArray (Variables|Default|GetMonster7) (Variables|Default|GetMonster8) (Variables|Default|GetMonster5) (Variables|Default|GetMonster4) (Variables|Default|GetMonster3) (Variables|Default|GetMonster2)))
  (CallFunction|LoopIdleAnimation)
  (Variables|Default|SetSounds%20Assets (.SoundsAssets (Utilities|Struct|BreakDataAssetsSettings (Utilities|Array|Get(acopy) (Variables|/Script/InfernaleTesting.GameSettingsDataAsset|GetDataAssetsSettings (Class|FunctionLibraryInfernale|GetGameSettingsDataAsset))))))
  (Rendering|SetVisibility (Variables|Default|GetIconRessources) true false)
  (bind _output_get_2 (Variables|Default|SetWBP%20Radial%20Progress%20Bar (.AsWBP%20Radial%20Progress%20Bar (Utilities|Casting|CastToWBP_RadialProgressBar (UserInterface|GetWidget (Variables|Default|GetWidget))))))
  (Widget|SetVisibility _output_get_2 "Hidden")
  (EventDispatchers|AssignHovered (delegate Custom|Hovered_Event))
  (Development|SetHiddeninGame (Variables|Default|GetDetectionDecal) true false))

(event EventTick
  (params (DeltaSeconds :type Float%20%28single-precision%29))
  (bind _ns_soulscollect (Variables|Default|GetNS_SoulsCollect))
  (bind _output_get (Variables|Default|SetLastAttackTime (+ (Variables|Default|GetLastAttackTime) DeltaSeconds)))
  (if (> _output_get 3.0)
    (if (Variables|Default|GetIdleStarted)
      _
      (else
        (Variables|Default|SetisAttacked false)
        (CallFunction|LoopIdleAnimation)
        (Utilities|IsValid _ns_soulscollect
          (:Is%20Valid
            (Class|NiagaraComponent|SetVariableBool _ns_soulscollect "IsAttacked" false))
          (:Is%20Not%20Valid
            _))))
    (if (and (Variables|Default|GetisTurning) (not (Variables|Default|GetisAttacked)))
      (Class|NeutralCamp|RotateStaticMeshesAroundPoint (Variables|Default|GetArrayOfMesh) (Transformation|GetActorLocation) 15.0 DeltaSeconds)
      (bind _output_get_2 (Variables|Default|SetDisolveTarget (+ (Variables|Default|GetDisolveTarget) (* 0.0 (* (/ (Variables|Default|GetChargeAddedPerTick) 1e+02) (Variables|Default|GetMaxCutoff))))))
      (Rendering|Material|SetScalarParameterValueonMaterials (Variables|Default|GetMonster4) "CutoffHeight" _output_get_2))))

(event EventSetDetectionDecalColor
  (params (Color :type Color%20Structure))
  (Rendering|Components|Decal|SetDecalColor (Variables|Default|GetDetectionDecal) (Math|Conversions|ToLinearColor(Color) Color)))

(fn ConstructionScript
  (CallFunction|SetScale 1.0)
  (Variables|Default|SetPowerValue (Variables|Default|GetMonsterPower)))

(fn SetScale
  (params (Percent :type Float%20%28double-precision%29))
  (bind _basescale (Variables|Default|GetBaseScale))
  (bind _returnvalue (* Percent _basescale))
  (bind _returnvalue_2 (Math|Vector|MakeVector _returnvalue _returnvalue _returnvalue))
  (for _array_element (Variables|Default|GetArrayOfMesh)
    (Transformation|SetRelativeScale3D _array_element (select (Math|Float|NearlyEqual(Float) (Math|Vector|VectorLength _returnvalue_2) 0.0 1e-06) "0.001000,0.001000,0.001000" _returnvalue_2))))

(fn SetHighlighMesh
  (return (Utilities|Array|MakeArray (Variables|Default|GetMonster3) (Variables|Default|GetMonster2) (Variables|Default|GetPillar) (Variables|Default|GetMonster5) (Variables|Default|GetMonster8) (Variables|Default|GetMonster7) (Variables|Default|GetMonster4))))

(fn GetOffsetScalingIndicator
  (params (Widget :type Widget%20Component%20Object%20Reference))
  (bind _returnvalue (Game|Player|GetPlayerPawn 0))
  (bind _returnvalue_2 (Transformation|GetWorldLocation Widget))
  (bind (_x _y) (Math|Vector|BreakVector _returnvalue_2))
  (bind _asbp_infernale_pawn (Utilities|Casting|CastToBP_InfernalePawn _returnvalue))
  (bind _cameracomponent (Variables|/Script/InfernaleTesting.InfernalePawn|GetCameraComponent _asbp_infernale_pawn))
  (bind _returnvalue_3 (Transformation|GetWorldLocation _cameracomponent))
  (bind (_x_2 _y_2) (Math|Vector|BreakVector _returnvalue_3))
  (return (* (Math|Vector|Normalize (Math|Vector|MakeVector (- _x_2 _x) (- _y_2 _y) 0.0)) (Variables|/Game/UI/InGame/WBP_PowerScaling.WBP_PowerScaling_C|GetOffsetWidget (.AsWBP%20Power%20Scaling (Utilities|Casting|CastToWBP_PowerScaling (UserInterface|GetWidget Widget)))))))