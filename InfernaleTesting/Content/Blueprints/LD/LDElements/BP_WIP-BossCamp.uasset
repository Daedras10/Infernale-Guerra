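; BP_WIP-BossCamp is a work-in-progress boss camp level element that gives visual feedback for damage, death and respawn.
; Damage events uniformly scale the Cube by remaining health relative to the DamageableComponent's max, times BaseScale.
; Death reveals a radial progress bar widget that respawn-time events update with the remaining-time fraction.
; Respawn hides the bar and restores full scale, which the construction script also applies.
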(event EventVisualDamagedBP
  (params (NewHealth :type Float%20%28single-precision%29) (DamageAmount :type Float%20%28single-precision%29))
  (CallFunction|SetScale (/ NewHealth (Variables|/Script/InfernaleTesting.DamageableComponent|GetMaxHealth (Variables|Default|GetDamageableComponent)))))

(event EventVisualDeathBP
  (Widget|SetVisibility (Variables|Default|GetWBP%20Radial%20Progress%20Bar) "HitTestInvisible"))

(event EventVisualRespawnBP
  (Widget|SetVisibility (Variables|Default|GetWBP%20Radial%20Progress%20Bar) "Hidden")
  (CallFunction|SetScale 1.0))

(event EventVisualRespawnTimeBP
  (params (TimeRemaining :type Float%20%28single-precision%29) (TotalTime :type Float%20%28single-precision%29))
  (Default|UpdatePercent (Variables|Default|GetWBP%20Radial%20Progress%20Bar) (/ TimeRemaining TotalTime)))

(event EventBeginPlay
  (bind _output_get (Variables|Default|SetWBP%20Radial%20Progress%20Bar (.AsWBP%20Radial%20Progress%20Bar (Utilities|Casting|CastToWBP_RadialProgressBar (UserInterface|GetWidget (Variables|Default|GetWidget))))))
  (Widget|SetVisibility _output_get "Hidden"))

(fn ConstructionScript
  (CallFunction|SetScale 1.0))

(fn SetScale
  (params (Percent :type Float%20%28double-precision%29))
  (bind _basescale (Variables|Default|GetBaseScale))
  (bind _returnvalue (* Percent _basescale))
  (Transformation|SetRelativeScale3D (Variables|Default|GetCube) (Math|Vector|MakeVector _returnvalue _returnvalue _returnvalue)))