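; Soul Beacon: a capturable level element that rewards souls to its owning team for units dying in its zone.
; This Blueprint handles presentation: bobbing mesh, hover tooltip and highlight, capture/loss notifications, reward pop-ups and a power-scaling indicator.
; Ownership changes recolor the mesh, Niagara effects, decal and tagged zone banners to the team.
; Tick feeds capture progress and main contester color into a radial material.
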(event Custom|Hovered_Event
  (params (PlayerControllerInfernale :type Player%20Controller%20Infernale%20Object%20Reference) (bVal :type Boolean))
  (bind _result (Utilities|Text|FormatText "<HoverTooltip_Generic>Capture the </><img id=\"SoulBeacon\" width=\"24\" height=\"24\" stretch=\"ScaleToFit\"/><HoverTooltip_Souls>SOUL BEACON</><HoverTooltip_Generic>, and reap the </><img id=\"Souls\" width=\"24\" height=\"24\" stretch=\"ScaleToFit\"/><HoverTooltip_Souls> SOULS</><HoverTooltip_Generic> of every </><img id=\"Units\" width=\"32\" height=\"32\" stretch=\"ScaleToFit\"/><HoverTooltip_UnitPower> UNITS</><HoverTooltip_Generic> dying of combat in its associated zone.</>"))
  (bind _decalmid (Variables|Default|GetDecalMID))
  (bind _debugsb_bp (Variables|Default|GetDebugSB_BP))
  (bind _uicomponent (Variables|/Script/InfernaleTesting.PlayerControllerInfernale|GetUIComponent PlayerControllerInfernale))
  (bind _asbp_uicomponent (Utilities|Casting|CastToBP_UIComponent _uicomponent))
  (bind _hud_sandbox (Variables|/Game/Blueprints/Component/PlayerController/BP_UIComponent.BP_UIComponent_C|GetHUD%20Sandbox _asbp_uicomponent))
  (if bVal
    (Rendering|Material|SetScalarParameterValue _decalmid "IsHide" 0.0 :!class /Script/Engine.MaterialInstanceDynamic)
    (Rendering|Material|SetScalarParameterValue _decalmid "IsHovered" 0.3 :!class /Script/Engine.MaterialInstanceDynamic)
    (else
      (switch Utilities|FlowControl|Switch|SwitchonETeam (.Team (Utilities|Struct|BreakOwner (Variables|Default|GetOwnerWithTeam)))
        (:NatureTeam
          (Rendering|Material|SetScalarParameterValue _decalmid "IsHide" 1.0 :!class /Script/Engine.MaterialInstanceDynamic))
        (:Team1
          (Rendering|Material|SetScalarParameterValue _decalmid "IsHide" 0.0 :!class /Script/Engine.MaterialInstanceDynamic :!label _label)
          (Development|PrintString "HIDDDEENN" _debugsb_bp _debugsb_bp))
        (:Team2
          (goto _label))
        (:Team3
          (goto _label))
        (:Team4
          (goto _label)))
      (Rendering|Material|SetScalarParameterValue _decalmid "IsHovered" 0.0 :!class /Script/Engine.MaterialInstanceDynamic)))
  (if (not (== (Variables|Default|GetisHovered) bVal))
    (Utilities|IsValid (Variables|Default|GetHUD%20Widget) :!label _label_2
      (:Is%20Valid
        (Default|HoveredTooltip (Variables|Default|GetHUD%20Widget) bVal _result self 0.5))
      (:Is%20Not%20Valid
        (Utilities|IsValid _hud_sandbox
          (:Is%20Valid
            (Default|HoveredTooltip _hud_sandbox bVal _result self 0.5))
          (:Is%20Not%20Valid
            (Variables|Default|SetHUD%20Widget (Variables|/Game/Blueprints/Component/PlayerController/BP_UIComponent.BP_UIComponent_C|GetHUD%20Widget (.AsBP%20UIComponent (Utilities|Casting|CastToBP_UIComponent (Variables|/Script/InfernaleTesting.PlayerControllerInfernale|GetUIComponent (.AsBP%20Player%20Controller%20Infernale (Utilities|Casting|CastToBP_PlayerControllerInfernale (Game|GetPlayerController 0))))))))
            (Utilities|FlowControl|Delay 0.1)
            (goto _label_2)))))
    (if (Variables|Default|GetIsHovered)
      (Variables|Default|SetisHovered bVal)
      (Rendering|Material|SetOverlayMaterial (Variables|Default|GetMesh) 0 :!class /Script/Engine.MeshComponent)
      (else
        (Variables|Default|SetisHovered bVal)
        (Rendering|Material|SetOverlayMaterial (Variables|Default|GetMesh) "/Game/_Draft/Philemon/MOI_SoulBeacon.MOI_SoulBeacon" :!class /Script/Engine.MeshComponent)))))

(event Custom|NewOwnerVisualMulticast
  (params (Actor :type Actor%20Object%20Reference) (OldOwner :type Owner%20Structure) (NewOwner :type Owner%20Structure))
  (bind _soulbeaconneutral (Variables|Default|GetSoulBeaconNeutral))
  (CallFunction|CaptureEvent NewOwner)
  (Variables|Default|SetOldOwner NewOwner)
  (CallFunction|NewVisuals (.Team (Utilities|Struct|BreakOwner NewOwner)))
  (Utilities|IsValid _soulbeaconneutral
    (:Is%20Valid
      (if (Components|Activation|IsActive _soulbeaconneutral)
        (Components|DestroyComponent (Variables|Default|GetSoulBeaconNeutral))
        (if (not (Components|Activation|IsActive (Variables|Default|GetNS_SoulBeacon)))
          (Components|Activation|Activate (Variables|Default|GetNS_SoulBeacon) false))))))

(event Custom|Activate
  (bind _debugsb_bp (Variables|Default|GetDebugSB_BP))
  (bind _returnvalue (Class|SoulBeacon|CanActivate))
  (if (not _returnvalue)
    (Development|PrintString "didnt activate" _debugsb_bp _debugsb_bp)))

(event Custom|CaptureEvent
  (params (Owner :type Owner%20Structure%20%28by%20ref%29))
  (bind _returnvalue (Game|GetPlayerController 0))
  (bind _returnvalue_2 (Game|GetPlayerController 0))
  (bind _returnvalue_3 (Game|GetGameInstance))
  (bind _self self)
  (bind _returnvalue_4 (Actor|GetComponentbyClass _returnvalue "/Game/Blueprints/Component/PlayerController/BP_UIComponent.BP_UIComponent_C"))
  (bind _asbp_game_instance_infernale (Utilities|Casting|CastToBP_GameInstanceInfernale _returnvalue_3))
  (bind _asbp_player_controller_infernale (Utilities|Casting|CastToBP_PlayerControllerInfernale _returnvalue_2))
  (bind _personalplayerinfo (Variables|/Script/InfernaleTesting.GameInstanceInfernale|GetPersonalPlayerInfo _asbp_game_instance_infernale))
  (bind _bp_uicomponent (Variables|/Game/Blueprints/GameMode/Infernale/BP_PlayerControllerInfernale.BP_PlayerControllerInfernale_C|GetBP_UIComponent _asbp_player_controller_infernale))
  (bind _notificationtray (Variables|/Game/Blueprints/Component/PlayerController/BP_UIComponent.BP_UIComponent_C|GetNotificationTray _returnvalue_4))
  (bind _playerownerinfo (Utilities|Struct|BreakPlayerInfo _personalplayerinfo))
  (bind _hud_widget (Variables|/Game/Blueprints/Component/PlayerController/BP_UIComponent.BP_UIComponent_C|GetHUD%20Widget _bp_uicomponent))
  (bind _player (Utilities|Struct|BreakOwner _playerownerinfo))
  (bind _floattotextentry (Variables|/Game/UI/InGame/WBP_DebugHUD.WBP_DebugHUD_C|GetFloatToTextEntry _hud_widget))
  (if (Pawn|IsLocalPlayerController (Game|GetPlayerController 0))
    (if (Utilities|Enum|Equal(Enum) (.Player (Utilities|Struct|BreakOwner Owner)) _player)
      (Default|AddNotification _notificationtray "Soul Beacon Captured" "/Game/UI/Textures/T_SoulsSimplified.T_SoulsSimplified" _self)
      (Class|SoundsDataAsset|PlaySound (.soundsassets (Utilities|Array|Get(acopy) (Variables|/Script/InfernaleTesting.GameSettingsDataAsset|GetDataAssetsSettings (Class|FunctionLibraryInfernale|GetGameSettingsDataAsset)))) "Soul Beacon" "Soul Beacon Captured" (Transformation|GetActorLocation (Game|Player|GetPlayerPawn 0)))
      (for (_array_element _array_index) _floattotextentry
        (if (Utilities|Enum|Equal(Enum) (.Index (Utilities|Struct|BreakBPS_FloatToTextEntry _array_element)) "Francis")
          (if (.AND (Utilities|Struct|BreakBPS_FloatToTextEntry _array_element))
            (bind _structout (Utilities|Struct|SetmembersinBPS_FloatToTextEntry _array_element false))
            (Utilities|Array|SetArrayElem _floattotextentry _array_index _structout))))
      (elif (Utilities|Enum|Equal(Enum) _player (.Player (Utilities|Struct|BreakOwner (Variables|Default|GetOldOwner))))
        (Default|AddNotification _notificationtray "Soul Beacon Lost" "/Game/UI/Textures/T_SoulsSimplified.T_SoulsSimplified" _self)))))

(event Custom|StartAnims
  (bind _mesh (Variables|Default|GetMesh))
  ;[1 0 0.5375] ANIMATION SOUL BEACON
  (Variables|Default|SetInitMeshLocation (Transformation|GetWorldLocation _mesh))
  (bind _up_and_down (Timeline|Timeline PlayFromStart)
    (:Update
      (Transformation|SetWorldLocation _mesh (Math|Vector|MakeVector (.x (Variables|Default|GetInitMeshLocation)) (.y (Variables|Default|GetInitMeshLocation)) (+ (.z (Variables|Default|GetInitMeshLocation)) _up_and_down)) false false))
    (:Finished
      (Utilities|FlowControl|DelayUntilNextTick)
      (Timeline|Timeline PlayFromStart))))

(event EventOnCapturingBP)

(event EventSetDetectionDecalColor
  (params (Color :type Color%20Structure))
  ;[1 1 1] Detection Decal Color
  (Rendering|Components|Decal|SetDecalColor (Variables|Default|GetDetectionDecal) (Math|Conversions|ToLinearColor(Color) Color)))

(event EventTriggerDetectionVFX
  (params (Scaling :type EFluxPowerScaling%20Enum :default "VeryLow") (Power :type Integer))
  (bind _scalingindicator (Variables|Default|GetScalingIndicator))
  (Development|SetHiddeninGame (Variables|Default|GetScalingIndicator) false false)
  (bind _returnvalue (UserInterface|CreateWidget "/Game/UI/InGame/WBP_PowerScaling.WBP_PowerScaling_C" (Game|GetPlayerController 0)))
  (UserInterface|SetWidget _scalingindicator _returnvalue)
  (Default|Init _returnvalue "Average" "EntityTypeNone" self (.Team (Utilities|Struct|BreakOwner (Class|PlayerControllerInfernale|GetOwnerInfo (.AsBP%20Player%20Controller%20Infernale (Utilities|Casting|CastToBP_PlayerControllerInfernale (Game|GetPlayerController 0)))))) Power)
  (Transformation|AddWorldOffset _scalingindicator (CallFunction|GetOffsetScalingIndicator _scalingindicator) false false))

(event EventDisableDetectionVFX
  (bind _scalingindicator (Variables|Default|GetScalingIndicator))
  (Development|SetHiddeninGame _scalingindicator true false)
  (UserInterface|SetWidget _scalingindicator 0)
  (Transformation|SetRelativeLocation _scalingindicator "0, 0, 0" false false))

(event EventOnStalemateBP)

(event EventBeginPlay
  (bind _detectiondecal (Variables|Default|GetDetectionDecal))
  (bind _output_get (Variables|Default|SetSounds%20Assets (.SoundsAssets (Utilities|Struct|BreakDataAssetsSettings (Utilities|Array|Get(acopy) (Variables|/Script/InfernaleTesting.GameSettingsDataAsset|GetDataAssetsSettings (Class|FunctionLibraryInfernale|GetGameSettingsDataAsset)))))))
  (bind _returnvalue (Class|SoundsDataAsset|GetSoundType _output_get "Soul Beacon" "Soul Beacon Button Clicked"))
  (Audio|Components|Audio|SetSound (Variables|Default|GetAmbiantSound) (.sound _returnvalue))
  (CallFunction|NewVisuals "NatureTeam")
  (Components|Activation|Activate (Variables|Default|GetSoulBeaconNeutral) false)
  (EventDispatchers|AssignHovered self (delegate Custom|Hovered_Event))
  (CallFunction|StartAnims)
  (Development|SetHiddeninGame _detectiondecal true false)
  (Rendering|Components|Decal|SetDecalColor _detectiondecal (Class|KismetMathLibrary|LinearColorWhite))
  (bind _returnvalue_2 (Rendering|Material|CreateDynamicMaterialInstance (Variables|Default|GetCaptureAmount) 0 "/Game/Effects/Soulbeacon/Materials/MI_CaptureRadialZone.MI_CaptureRadialZone" "None" :!class /Script/Engine.PrimitiveComponent))
  (Variables|Default|SetCaptureZoneMat _returnvalue_2)
  (Class|SoundsDataAsset|PlaySound (.soundsassets (Utilities|Array|Get(acopy) (Variables|/Script/InfernaleTesting.GameSettingsDataAsset|GetDataAssetsSettings (Class|FunctionLibraryInfernale|GetGameSettingsDataAsset)))) "Soul Beacon" "Soul Beacon Ambiant Sounds" (Transformation|GetWorldLocation (Variables|Default|GetCaptureAmount))))

(event EventNewOwnerVisuals
  (params (Actor :type Actor%20Object%20Reference) (OldOwner :type Owner%20Structure) (NewOwner :type Owner%20Structure))
  (CallFunction|NewOwnerVisualMulticast Actor OldOwner NewOwner))

(event EventTick
  (params (DeltaSeconds :type Float%20%28single-precision%29))
  (bind _capturezonemat (Variables|Default|GetCaptureZoneMat))
  (Rendering|Material|SetScalarParameterValue _capturezonemat "pourcent" (/ (Variables|Default|GetCaptureAmountSoulBeacon) 1e+02) :!class /Script/Engine.MaterialInstanceDynamic)
  (Rendering|Material|SetVectorParameterValue _capturezonemat "TeamColor" (.SpecifiedColor (Utilities|Struct|BreakSlateColor (CallFunction|GetTeamColor (.Team (Utilities|Struct|BreakOwner (Variables|Default|GetMainContesterSoulBeacon)))))) :!class /Script/Engine.MaterialInstanceDynamic))

(event EventRewardBP
  (params (RewardType :type ESoulBeaconRewardType%20Enum :default "RewardAmalgam"))
  (if (Utilities|Enum|Equal(Enum) (.Team (Utilities|Struct|BreakOwner (Variables|/Script/InfernaleTesting.PlayerStateInfernale|GetOwnerInfo (.AsBP%20Player%20State%20Infernale (Utilities|Casting|CastToBP_PlayerStateInfernale (Game|GetPlayerState 0)))))) (.Team (Utilities|Struct|BreakOwner (Variables|Default|GetOwnerWithTeam))))
    (bind _newparam (CallFunction|GetRewardValue RewardType "/Game/DataAssets/DA_SoulBeaconRewards.DA_SoulBeaconRewards"))
    (CallFunction|CreatePopUp self (Utilities|Text|ToText(Integer) _newparam) "/Game/UI/Textures/T_SoulsSimplified.T_SoulsSimplified" 5.0)))

(event EventToggleDetectionDecal
  (params (Hide :type Boolean))
  (bind _returnvalue (Game|GetPlayerController 0))
  (bind _ownerwithteam (Variables|Default|GetOwnerWithTeam))
  (bind _team (Utilities|Struct|BreakOwner _ownerwithteam))
  (bind _asbp_player_controller_infernale (Utilities|Casting|CastToBP_PlayerControllerInfernale _returnvalue))
  (bind _returnvalue_2 (Class|PlayerControllerInfernale|GetOwnerInfo _asbp_player_controller_infernale))
  (bind _team_2 (Utilities|Struct|BreakOwner _returnvalue_2))
  (bind _returnvalue_3 (Utilities|Enum|Equal(Enum) _team _team_2))
  (bind _returnvalue_4 (or Hide _returnvalue_3))
  ;[1 1 1] Toggle Detection Decal
  (if _returnvalue_4
    (Rendering|Components|Decal|SetDecalColor (Variables|Default|GetDetectionDecal) (Class|KismetMathLibrary|LinearColorWhite)))
  (Development|SetHiddeninGame (Variables|Default|GetDetectionDecal) _returnvalue_4 false))

(event EventOnUncontestedBP)

(event EventOnCapturedVFXTrigger
  (params (Location :type Vector :default "0, 0, 0"))
  ;[1 1 1] Capture VFX
)

(fn ConstructionScript
  (Rendering|Components|Decal|SetDecalMaterial (Variables|Default|GetDecalMarks) (Variables|Default|GetDecalNumberMaterial)))

(fn NewVisuals
  (params (Team :type ETeam%20Enum :default "NatureTeam"))
  (bind _teamvector (CallFunction|GetTeamVectorColor Team))
  (bind _mesh (Variables|Default|GetMesh))
  (bind _returnvalue (Math|Conversions|ToLinearColor(Vector) _teamvector))
  (bind _returnvalue_2 (Rendering|Material|CreateDynamicMaterialInstance _mesh 1 (Rendering|Material|GetMaterial _mesh 0) "None" :!class /Script/Engine.PrimitiveComponent))
  (Rendering|Material|SetVectorParameterValue _returnvalue_2 "Color emissive" _returnvalue :!class /Script/Engine.MaterialInstanceDynamic)
  (Niagara|SetNiagaraVariable(LinearColor) (Variables|Default|GetNS_SoulBeacon) "MainColor" _returnvalue)
  (bind _returnvalue_3 (Rendering|Material|CreateDynamicMaterialInstance (Variables|Default|GetDecalMarks) :!class /Script/Engine.DecalComponent))
  (Rendering|Material|SetVectorParameterValue _returnvalue_3 "TeamColor" _returnvalue :!class /Script/Engine.MaterialInstanceDynamic)
  (Variables|Default|SetDecalMID _returnvalue_3)
  (Niagara|SetNiagaraVariable(LinearColor) (Variables|Default|GetCaptureZone) "TeamColor" _returnvalue)
  (switch Utilities|FlowControl|Switch|SwitchonETeam Team
    (:NatureTeam
      _)
    (:Team1
      (Rendering|Material|SetScalarParameterValue (Variables|Default|GetDecalMID) "IsHide" 0.0 :!class /Script/Engine.MaterialInstanceDynamic :!label _label))
    (:Team2
      (goto _label))
    (:Team3
      (goto _label))
    (:Team4
      (goto _label)))
  (CallFunction|SetBanners Team))

(fn GetRewardValue
  (params (Reward%20Type :type ESoulBeaconRewardType%20Enum :default "RewardAmalgam") (Reward%20Asset :type Soul%20Beacon%20Reward%20Asset%20Object%20Reference))
  (switch Utilities|FlowControl|Switch|SwitchonESoulBeaconRewardType Reward%20Type
    (:RewardAmalgam
      (return (Variables|/Script/InfernaleTesting.SoulBeaconRewardAsset|GetAmalgamReward Reward%20Asset)))
    (:RewardNeutral
      (return (Variables|/Script/InfernaleTesting.SoulBeaconRewardAsset|GetNeutralReward Reward%20Asset)))
    (:RewardBoss
      (return (Variables|/Script/InfernaleTesting.SoulBeaconRewardAsset|GetBossReward Reward%20Asset)))
    (:RewardBuilding
      (return (Variables|/Script/InfernaleTesting.SoulBeaconRewardAsset|GetBuildingReward Reward%20Asset)))
    (:RewardMainBuilding
      (return (Variables|/Script/InfernaleTesting.SoulBeaconRewardAsset|GetMainBuildingReward Reward%20Asset)))))

(fn SetBanners
  (params (NewTeam :type ETeam%20Enum :default "NatureTeam"))
  (if (Utilities|Enum|NotEqual(Enum) NewTeam "NatureTeam")
    (switch Utilities|FlowControl|Switch|SwitchonETeam NewTeam
      (:Team1
        (LocalVariables|SetTeamScalarValue 0.0))
      (:Team2
        (LocalVariables|SetTeamScalarValue 0.25))
      (:Team3
        (LocalVariables|SetTeamScalarValue 0.5))
      (:Team4
        (LocalVariables|SetTeamScalarValue 0.75)))
    (for _array_element (Variables|Default|GetZoneBanners)
      (Development|SetHiddeninGame (Variables|/Script/Engine.Actor|GetRootComponent _array_element) false false)
      (Rendering|SetVisibility (Variables|/Script/Engine.Actor|GetRootComponent _array_element) true false)
      (Rendering|Material|SetMaterial (Variables|/Script/Engine.StaticMeshActor|GetStaticMeshComponent _array_element) 0 "/Game/Character/Glutonny/Materials/MI_TeamBannerEnviroNoPole.MI_TeamBannerEnviroNoPole")
      (bind _returnvalue (Rendering|Material|CreateDynamicMaterialInstance (Variables|/Script/Engine.StaticMeshActor|GetStaticMeshComponent _array_element) 0 (Rendering|Material|GetMaterial (Variables|/Script/Engine.StaticMeshActor|GetStaticMeshComponent _array_element) 0) "None" :!class /Script/Engine.PrimitiveComponent))
      (Rendering|Material|SetScalarParameterValue _returnvalue "Team" (LocalVariables|GetTeamScalarValue) :!class /Script/Engine.MaterialInstanceDynamic)
      (Rendering|Material|SetVectorParameterValue _returnvalue "FirstTeamColor" (.SpecifiedColor (Utilities|Struct|BreakSlateColor (CallFunction|GetTeamColor NewTeam))) :!class /Script/Engine.MaterialInstanceDynamic)
      (Rendering|Material|SetVectorParameterValue _returnvalue "SecondTeamColor" (.SpecifiedColor (Utilities|Struct|BreakSlateColor (CallFunction|GetTeamSecondColor NewTeam))) :!class /Script/Engine.MaterialInstanceDynamic))
    (else
      (for _array_element_2 (Variables|Default|GetZoneBanners)
        (Rendering|Material|SetMaterial (Variables|/Script/Engine.StaticMeshActor|GetStaticMeshComponent _array_element_2) 0 "/Game/Environment/Props/GenericBanners/MI_BannerGeneric.MI_BannerGeneric")))))

(fn UpdateBannersEditor
  (Utilities|Array|Clear (Variables|Default|GetZoneBanners))
  (bind _outactors (Actor|GetAllActorsOfClasswithTag "/Script/Engine.StaticMeshActor" (Variables|Default|GetBannerTag)))
  (Utilities|Array|AppendArray (Variables|Default|GetZoneBanners) _outactors))

(fn GetOffsetScalingIndicator
  (params (Widget :type Widget%20Component%20Object%20Reference))
  (bind _returnvalue (Game|Player|GetPlayerPawn 0))
  (bind _returnvalue_2 (Transformation|GetWorldLocation Widget))
  (bind (_x _y) (Math|Vector|BreakVector _returnvalue_2))
  (bind _asbp_infernale_pawn (Utilities|Casting|CastToBP_InfernalePawn _returnvalue))
  (bind _cameracomponent (Variables|/Script/InfernaleTesting.InfernalePawn|GetCameraComponent _asbp_infernale_pawn))
  (bind _returnvalue_3 (Transformation|GetWorldLocation _cameracomponent))
  (bind (_x_2 _y_2) (Math|Vector|BreakVector _returnvalue_3))
  (return (* (Math|Vector|Normalize (Math|Vector|MakeVector (- _x_2 _x) (- _y_2 _y) 0.0)) (Variables|/Game/UI/InGame/WBP_PowerScaling.WBP_PowerScaling_C|GetOffsetWidget (.AsWBP%20Power%20Scaling (Utilities|Casting|CastToWBP_PowerScaling (UserInterface|GetWidget Widget)))))))