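; Building Blueprint that handles team-colored visual feedback and selection state.
; Owner changes multicast the new team's emissive color to the model and cone, which shows during flux selection.
; Hover dims the team color, and two chained timelines blink it red before darkening permanent buildings.
; Ending interaction clears the local souls-cost hover after a short delay; construction, lifetime and overclick hooks are empty, with timer-widget code disconnected.
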(event Custom|NewOwnerVisualMulticast
  (params (Actor :type Actor%20Object%20Reference) (OldOwner :type Owner%20Structure) (NewOwner :type Owner%20Structure))
  (bind _team (Utilities|Struct|BreakOwner NewOwner))
  (bind _model (Variables|Default|GetModel))
  (Rendering|Material|SetVectorParameterValueonMaterials _model "Color emissive" (CallFunction|GetTeamVectorColor _team))
  (Rendering|Material|SetMaterial (Variables|Default|GetSelectedCone) 0 (Rendering|Material|GetMaterial _model 0))
  (Development|PrintString (Utilities|String|EnumtoString _team) false false))

(event EventOnConstructionTimeRemainingBP
  (params (RemainingTime :type Float%20%28single-precision%29) (InitialDuration :type Float%20%28single-precision%29) (shouldHide :type Boolean)))

(event EventOnSelectedforFlux
  (Rendering|SetVisibility (Variables|Default|GetSelectedCone) true false))

(event EventHoveredBP
  (params (bHovered :type Boolean))
  (Rendering|Material|SetVectorParameterValueonMaterials (Variables|Default|GetModel) "Color" (* (CallFunction|GetTeamVectorColor (.Team (Utilities|Struct|BreakOwner (Variables|Default|GetOwnerWithTeam)))) (Math|Float|SelectFloat 0.55 1.0 bHovered))))

(event EventInteractedBP
  (params (Interacted :type Boolean))
  (if (not Interacted)
    (Utilities|FlowControl|Delay 0.1)
    (Class|UIComponent|SoulsCostHovered (Variables|/Game/Blueprints/GameMode/Infernale/BP_PlayerControllerInfernale.BP_PlayerControllerInfernale_C|GetBP_UIComponent (.AsBP%20Player%20Controller%20Infernale (Utilities|Casting|CastToBP_PlayerControllerInfernale (Game|GetPlayerController 0)))) false 0.0)))

(event EventOnDeselectedforFlux
  (Rendering|SetVisibility (Variables|Default|GetSelectedCone) false false))

(event EventNewOwnerVisuals
  (params (Actor :type Actor%20Object%20Reference) (OldOwner :type Owner%20Structure) (NewOwner :type Owner%20Structure))
  (CallFunction|NewOwnerVisualMulticast Actor OldOwner NewOwner))

(event EventBeginPlay
  (Class|Building|InteractedBP false))

(event EventOverclickVisualsBP)

(event EventOnLifeTimeRemainingBP
  (params (RemainingTime :type Float%20%28single-precision%29) (InitialDuration :type Float%20%28single-precision%29)))

(event EventUpgradeBuildingVisuals
  (if (Variables|Default|GetbIsPermanent)
    (Rendering|Material|SetVectorParameterValueonMaterials (Variables|Default|GetModel) "Color" (* (CallFunction|GetTeamVectorColor (.Team (Utilities|Struct|BreakOwner (Variables|Default|GetOwnerWithTeam)))) 0.3))))

(event EventBlinkEffect
  (bind _alpha (Timeline|BlinkIn PlayFromStart)
    (:Update
      (Variables|Default|SetDebugAlpha _alpha)
      (Rendering|Material|SetVectorParameterValueonMaterials (Variables|Default|GetModel) "Color" (Math|Vector|Lerp(Vector) (CallFunction|GetTeamVectorColor (.Team (Utilities|Struct|BreakOwner (Variables|Default|GetOwnerWithTeam)))) "1.000000,0.000000,0.000000" _alpha)))
    (:Finished
      (bind _alpha_2 (Timeline|BlinkOut PlayFromStart)
        (:Update
          (Rendering|Material|SetVectorParameterValueonMaterials (Variables|Default|GetModel) "Color" (Math|Vector|Lerp(Vector) (CallFunction|GetTeamVectorColor (.Team (Utilities|Struct|BreakOwner (Variables|Default|GetOwnerWithTeam)))) "1.000000,0.000000,0.000000" _alpha_2)))
        (:Finished
          (if (Variables|Default|GetbIsPermanent)
            (Rendering|Material|SetVectorParameterValueonMaterials (Variables|Default|GetModel) "Color" (* (CallFunction|GetTeamVectorColor (.Team (Utilities|Struct|BreakOwner (Variables|Default|GetOwnerWithTeam)))) 0.3))))))))

(fn ConstructionScript)

(fn GetAllActorswithColor
  (return (Utilities|Array|MakeArray (Variables|Default|GetSelectedCone))))