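; BP_BuildFlux is the Flux Building, a child building Blueprint that defers to its parent for BeginPlay and visual upgrades.
; On BeginPlay it creates a dynamic material on the model and sets FirstTeamColor to the third team color of the local player's team, read from player controller 0's PlayerState.
; The construction script clears AttackComponent.
; A randomized placement sound chain is present but unconnected.
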(event EventUpgradeBuildingVisuals
  (|CallParentFunction))

(event EventBeginPlay
  (bind _model (Variables|Default|GetModel))
  (|CallParentFunction)
  (bind _returnvalue (Rendering|Material|CreateDynamicMaterialInstance _model 0 (Rendering|Material|GetMaterial _model 0) "None" :!class /Script/Engine.PrimitiveComponent))
  (Rendering|Material|SetVectorParameterValue _returnvalue "FirstTeamColor" (.SpecifiedColor (Utilities|Struct|BreakSlateColor (CallFunction|GetTeamThirdColor (.Team (Utilities|Struct|BreakOwner (Variables|/Script/InfernaleTesting.PlayerStateInfernale|GetOwnerInfo (.AsBP%20Player%20State%20Infernale (Utilities|Casting|CastToBP_PlayerStateInfernale (Variables|/Script/Engine.Controller|GetPlayerState (.AsBP%20Player%20Controller%20Infernale (Utilities|Casting|CastToBP_PlayerControllerInfernale (Game|GetPlayerController 0)))))))))))) :!class /Script/Engine.MaterialInstanceDynamic))

(fn ConstructionScript
  (Variables|Default|SetAttackComponent 0))