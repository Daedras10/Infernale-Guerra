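; BP_BuildDefence is a defence building Blueprint that extends a parent building class with its own Cube and Cylinder meshes.
; On a visual upgrade, it runs the parent logic and then doubles the Cube's relative scale, so the growth compounds with each call.
; It overrides GetAllActorsWithColor to append the Cylinder and Cube to the parent's list of colored parts.
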(event EventUpgradeBuildingVisuals
  (bind _cube (Variables|Default|GetCube))
  (|CallParentFunction)
  (Transformation|SetRelativeScale3D _cube (* (Variables|/Script/Engine.SceneComponent|GetRelativeScale3D _cube) 2.0)))

(fn ConstructionScript)

(fn GetAllActorswithColor
  (bind _output_get (LocalVariables|SetArray (|CallParentFunction)))
  (Utilities|Array|AppendArray _output_get (Utilities|Array|MakeArray (Variables|Default|GetCylinder) (Variables|Default|GetCube)))
  (return (LocalVariables|GetArray)))