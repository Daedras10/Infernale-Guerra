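; BP_Breach is a team-owned breach point in the level, with team-colored mesh visuals and a linked UI.
; Ownership changes re-tint the mesh through material parameters via a multicast-named event.
; DisplayWidget shows the breach UI through the player controller's UI component and starts a delayed loop of timeline color blinks while visible.
; Hover, limited to the owning player on unlocked breaches, and lock state adjust color brightness; FacePosition is an empty stub.
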(event Custom|NewOwnerVisualMulticast
  (params (Actor :type Actor%20Object%20Reference) (OldOwner :type Owner%20Structure) (NewOwner :type Owner%20Structure))
  (CallFunction|NewVisualforTeam (.Team (Utilities|Struct|BreakOwner NewOwner))))

(event Custom|UIVisibleChanged
  (if (Variables|Default|GetUIVisible) :!label _label
    (CallFunction|BlinkEffect)
    (Utilities|FlowControl|Delay (Variables|Default|GetBlinkDelay))
    (goto _label)
    (else
      (Class|Breach|LockVisualBP (Variables|Default|GetbLocked))
      (Rendering|Material|SetVectorParameterValueonMaterials (Variables|Default|GetCylinder) "Color" (* (CallFunction|GetTeamVectorColor (.Team (Utilities|Struct|BreakOwner (Variables|Default|GetOwnerWithTeam)))) (Math|Float|SelectFloat 0.15 1.0 (Variables|Default|GetbHovered)))))))

(event Custom|BlinkEffect
  (bind _ownerwithteam (Variables|Default|GetOwnerWithTeam))
  (bind _team (Utilities|Struct|BreakOwner _ownerwithteam))
  (bind _teamvector (CallFunction|GetTeamVectorColor _team))
  (bind _alpha (Timeline|BlinkIn PlayFromStart)
    (:Update
      (Rendering|Material|SetVectorParameterValueonMaterials (Variables|Default|GetCylinder) "Color" (Math|Vector|Lerp(Vector) (CallFunction|GetTeamVectorColor (.Team (Utilities|Struct|BreakOwner (Variables|Default|GetOwnerWithTeam)))) "0, 0, 0" _alpha)))
    (:Finished
      (bind _alpha_2 (Timeline|BlinkOut PlayFromStart)
        (:Update
          (Rendering|Material|SetVectorParameterValueonMaterials (Variables|Default|GetCylinder) "Color" (Math|Vector|Lerp(Vector) _teamvector "0, 0, 0" _alpha_2))
          (Rendering|Material|SetVectorParameterValueonMaterials (Variables|Default|GetCylinder) "Color" _teamvector))))))

(event EventDisplayWidget
  (params (Display :type Boolean) (DisplayWidgetType :type EDisplayWidgetType%20Enum :default "DisplayWidgetNone"))
  ;[1 1 1] Event Display widget
  (Default|ShowBreach (Variables|/Game/Blueprints/GameMode/Infernale/BP_PlayerControllerInfernale.BP_PlayerControllerInfernale_C|GetBP_UIComponent (.AsBP%20Player%20Controller%20Infernale (Utilities|Casting|CastToBP_PlayerControllerInfernale (Game|GetPlayerController 0)))) Display self (Variables|Default|GetUseCategory))
  (Variables|Default|SetUIVisible Display)
  (CallFunction|UIVisibleChanged))

(event EventBeginPlay
  (bind _cylinder (Variables|Default|GetCylinder))
  (Rendering|SetVisibility (Variables|Default|GetWidget) false false)
  (Collision|SetCollisionEnabled (Variables|Default|GetWidget) "NoCollision")
  (bind _output_get (Variables|Default|SetBP%20Player%20Controller%20Infernale (.AsBP%20Player%20Controller%20Infernale (Utilities|Casting|CastToBP_PlayerControllerInfernale (Game|GetPlayerController 0)))))
  (bind _output_get_2 (Variables|Default|SetWBP%20Breach%20UI (.AsWBP%20Breach%20UI (Utilities|Casting|CastToWBP_BreachUI (UserInterface|GetWidget (Variables|Default|GetWidget))))))
  (Default|Init _output_get_2 self 0 _output_get)
  (Variables|Default|SetBaseWidgetLoc (Variables|/Script/Engine.SceneComponent|GetRelativeLocation (Variables|Default|GetWidget)))
  (Components|Timeline|SetPlayRate (Variables|Default|GetBlinkIn) (/ 1.0 (Variables|Default|GetBlinkInDuration)))
  (Components|Timeline|SetPlayRate (Variables|Default|GetBlinkOut) (/ 1.0 (Variables|Default|GetBlinkOutDuration)))
  (Variables|Default|SetAs%20BP%20Player%20Controller%20Infernale (.AsBP%20Player%20Controller%20Infernale (Utilities|Casting|CastToBP_PlayerControllerInfernale (Game|GetPlayerController 0))))
  (bind _returnvalue (Rendering|Material|CreateDynamicMaterialInstance _cylinder 0 (Rendering|Material|GetMaterial _cylinder 0) "None" :!class /Script/Engine.PrimitiveComponent))
  (Variables|Default|SetBreach%20MI _returnvalue))

(event EventOnHoverEnd
  (if (Utilities|Enum|Equal(Enum) (.Player (Utilities|Struct|BreakOwner (Variables|/Script/InfernaleTesting.PlayerStateInfernale|GetOwnerInfo (.AsBP%20Player%20State%20Infernale (Utilities|Casting|CastToBP_PlayerStateInfernale (Variables|/Script/Engine.Controller|GetPlayerState (Variables|Default|GetAs%20BP%20Player%20Controller%20Infernale))))))) (.Player (Utilities|Struct|BreakOwner (Variables|Default|GetOwnerWithTeam))))
    (if (not (Variables|Default|GetbLocked))
      (if (Variables|Default|GetUIVisible)
        _))))

(event EventNewOwnerVisuals
  (params (Actor :type Actor%20Object%20Reference) (OldOwner :type Owner%20Structure) (NewOwner :type Owner%20Structure))
  (CallFunction|NewOwnerVisualMulticast Actor OldOwner NewOwner))

(event EventFacePosition
  (params (Position :type Vector :default "0, 0, 0")))

(event EventOnHoverStart
  (if (Utilities|Enum|Equal(Enum) (.Player (Utilities|Struct|BreakOwner (Variables|/Script/InfernaleTesting.PlayerStateInfernale|GetOwnerInfo (.AsBP%20Player%20State%20Infernale (Utilities|Casting|CastToBP_PlayerStateInfernale (Variables|/Script/Engine.Controller|GetPlayerState (Variables|Default|GetAs%20BP%20Player%20Controller%20Infernale))))))) (.Player (Utilities|Struct|BreakOwner (Variables|Default|GetOwnerWithTeam))))
    (if (not (Variables|Default|GetbLocked))
      (Default|CallTmpHover true)
      (if (Variables|Default|GetbIsRealBreach)
        _))))

(event EventLockVisualBP
  (params (bLockedVal :type Boolean))
  (if bLockedVal
    (Rendering|Material|SetVectorParameterValueonMaterials (Variables|Default|GetCylinder) "Color" (* (CallFunction|GetTeamVectorColor (.Team (Utilities|Struct|BreakOwner (Variables|Default|GetOwnerWithTeam)))) (Math|Float|SelectFloat 0.15 1.0 bLockedVal)))
    (elif (Variables|Default|GetbHovered)
      (Rendering|Material|SetVectorParameterValueonMaterials (Variables|Default|GetCylinder) "Color" (* (CallFunction|GetTeamVectorColor (.Team (Utilities|Struct|BreakOwner (Variables|Default|GetOwnerWithTeam)))) (Math|Float|SelectFloat 0.15 1.0 (Variables|Default|GetbHovered))))
      (Default|CallTmpHover false))))

(event EventSetMeshBP
  (params (NewMesh :type Static%20Mesh%20Object%20Reference))
  (Components|StaticMesh|SetStaticMesh (Variables|Default|GetCylinder) NewMesh)
  (CallFunction|NewVisualforTeam (.Team (Utilities|Struct|BreakOwner (Variables|Default|GetOwnerWithTeam)))))

(fn ConstructionScript
  (CallFunction|NewVisualforTeam (.Team (Utilities|Struct|BreakOwner (Variables|Default|GetOwnerWithTeam)))))

(fn NewVisualforTeam
  (params (Team :type ETeam%20Enum :default "NatureTeam"))
  (bind _cylinder (Variables|Default|GetCylinder))
  (bind _returnvalue (Rendering|Material|CreateDynamicMaterialInstance _cylinder 0 (Rendering|Material|GetMaterial _cylinder 0) "None" :!class /Script/Engine.PrimitiveComponent))
  (Rendering|Material|SetVectorParameterValue _returnvalue "Emissive" (.SpecifiedColor (Utilities|Struct|BreakSlateColor (CallFunction|GetTeamThirdColor Team))) :!class /Script/Engine.MaterialInstanceDynamic)
  (Rendering|Material|SetVectorParameterValueonMaterials (Variables|Default|GetCylinder) "FirstTeamColor" (Math|Conversions|ToVector(LinearColor) (.SpecifiedColor (Utilities|Struct|BreakSlateColor (CallFunction|GetTeamColor Team))))))