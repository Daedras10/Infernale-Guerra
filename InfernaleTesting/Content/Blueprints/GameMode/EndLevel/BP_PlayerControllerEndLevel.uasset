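; Player controller for the end-of-match level that shows the end game screen.
; On BeginPlay it creates WBP_EndGame and passes it the victory info and the local player's team, both read from BP_GameInstanceInfernale.
; It then adds the widget to the viewport, switches to Game and UI input focused on it with the mouse locked, and shows the cursor.
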(event EventBeginPlay
  (bind _returnvalue (Game|GetGameInstance))
  (bind _asbp_game_instance_infernale (Utilities|Casting|CastToBP_GameInstanceInfernale _returnvalue))
  (bind _returnvalue_2 (UserInterface|CreateWidget "/Game/UI/InGame/EndGame/WBP_EndGame.WBP_EndGame_C" self))
  (bind _output_get (Variables|Default|SetWBP%20End%20Game _returnvalue_2))
  (Default|GameEnded _output_get (Variables|/Script/InfernaleTesting.GameInstanceInfernale|GetEndGameVictoryInfo _asbp_game_instance_infernale) (.Team (Utilities|Struct|BreakOwner (.PlayerOwnerInfo (Utilities|Struct|BreakPlayerInfo (Variables|/Script/InfernaleTesting.GameInstanceInfernale|GetPersonalPlayerInfo _asbp_game_instance_infernale))))))
  (UserInterface|Viewport|AddtoViewport _output_get 0)
  (Input|SetInputModeGameandUI self _output_get "LockAlways" true false)
  (Variables|Default|SetbShowMouseCursor true))

(fn ConstructionScript)