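; Main menu player controller that resets online session state and exposes a debug LAN-mode toggle.
; On BeginPlay it destroys any session, then calls Cleanup on the Infernale game instance whether that succeeds or fails.
; It polls each tick until the menu widget is valid, then shows or hides its LAN indicator from the game instance's UseLAN flag.
; Debug key M flips that flag and updates the indicator.
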(event EventBeginPlay
  (bind _wbpmenu (Variables|Default|GetWBPMenu))
  (bind _rt_lanmode (Variables|/Game/UI/DebugLobby/WBP_DebugLobby.WBP_DebugLobby_C|GetRT_LanMode _wbpmenu))
  (|DestroySession self
    (:OnSuccess
      _)
    (:OnFailure
      _))
  (Default|Cleanup (.AsBP%20Game%20Instance%20Infernale (Utilities|Casting|CastToBP_GameInstanceInfernale (Game|GetGameInstance))))
  (Utilities|IsValid (Variables|Default|GetWBPMenu) :!label _label
    (:Is%20Valid
      (if (Class|GameInstanceInfernale|UseLAN (.AsBP%20Game%20Instance%20Infernale (Utilities|Casting|CastToBP_GameInstanceInfernale (Game|GetGameInstance))))
        (Widget|SetVisibility _rt_lanmode "Visible")
        (else
          (Widget|SetVisibility _rt_lanmode "Hidden"))))
    (:Is%20Not%20Valid
      (Utilities|FlowControl|DelayUntilNextTick)
      (goto _label))))

(event Input|KeyboardEvents|DebugKeyM
  (params (Key :type Key%20Structure :default "None") (ActionValue :type Input%20Action%20Value%20Structure))
  (bind _returnvalue (Game|GetGameInstance))
  (bind _wbpmenu (Variables|Default|GetWBPMenu))
  (bind _asbp_game_instance_infernale (Utilities|Casting|CastToBP_GameInstanceInfernale _returnvalue))
  (bind _rt_lanmode (Variables|/Game/UI/DebugLobby/WBP_DebugLobby.WBP_DebugLobby_C|GetRT_LanMode _wbpmenu))
  (bind _returnvalue_2 (Class|GameInstanceInfernale|UseLAN _asbp_game_instance_infernale))
  (:Pressed
    (Class|GameInstanceInfernale|SetUseLAN _asbp_game_instance_infernale (not _returnvalue_2))
    (if _returnvalue_2
      (Widget|SetVisibility _rt_lanmode "Visible")
      (else
        (Widget|SetVisibility _rt_lanmode "Hidden")))))

(fn ConstructionScript)