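; Player controller for Infernale, bridging local input and UI with the server game mode for player data, JSON-load sync and game launch.
; Space highlights all flux actors (toggle or hold), Escape handles menus, C toggles HUD for permitted cheaters.
; Tab or a gate-timed double-click moves the pawn to the cursor.
; At game end, clients open the end level while the host waits for them to leave, then tears down the session.
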(event Custom|SwitchHUDVisibility
  (bind _output_get (Variables|Default|SetShowWidget (not (Variables|Default|GetShowWidget))))
  (Default|SwitchVisibilityOfAllWidgets (Variables|Default|GetBP_UIComponent) _output_get false))

(event Custom|RefreshOwning
  (params (PlayerInfo :type Array%20of%20Player%20Info%20Structures) (LaunchGame :type Boolean))
  (Utilities|FlowControl|DelayUntilNextTick)
  (Default|UpdatePlayerList (Variables|/Game/Blueprints/Component/PlayerController/BP_UIComponent.BP_UIComponent_C|GetHUD%20Sandbox (Variables|Default|GetBP_UIComponent)) PlayerInfo LaunchGame))

(event Custom|SyncPlayerDataServer
  (params (PlayerInfo :type Player%20Info%20Structure))
  (bind _asbp_game_mode_infernale (Utilities|Casting|CastToBP_GameModeInfernale (Game|GetGameMode)))
  (Default|SyncDataClient _asbp_game_mode_infernale PlayerInfo self))

(event Custom|SyncPlayerData
  (CallFunction|SyncPlayerDataServer (Variables|/Script/InfernaleTesting.GameInstanceInfernale|GetPersonalPlayerInfo (.AsBP%20Game%20Instance%20Infernale (Utilities|Casting|CastToBP_GameInstanceInfernale (Game|GetGameInstance))))))

(event Custom|RefreshServer
  (params (PlayerInfo :type Array%20of%20Player%20Info%20Structures) (LaunchGame :type Boolean))
  (CallFunction|RefreshOwning PlayerInfo LaunchGame))

(event Custom|ShowHideOptionsMenuCall
  (bind _output_get (Variables|Default|SetShowOptions (not (Variables|Default|GetShowOptions))))
  (Variables|Default|SetbIsEscapeMenuOpen (not (Variables|Default|GetShowOptions)))
  (Default|ShowHideOptionsMenu (Variables|Default|GetBP_UIComponent) _output_get))

(event Custom|LaunchGame
  (Variables|/Script/InfernaleTesting.GameInstanceInfernale|SetbIsPhilosophicallyAccurateGame (.AsBP%20Game%20Instance%20Infernale (Utilities|Casting|CastToBP_GameInstanceInfernale (Game|GetGameInstance))) true)
  (Class|PlayerControllerInfernale|EnableInputs false)
  (Widget|SetVisibility (Variables|/Game/Blueprints/Component/PlayerController/BP_UIComponent.BP_UIComponent_C|GetLoadingScreen (Variables|Default|GetBP_UIComponent)) "Visible")
  (Networking|SwitchHasAuthority
    (:Authority
      (bind _asbp_game_mode_infernale (Utilities|Casting|CastToBP_GameModeInfernale (Game|GetGameMode)))
      (Default|AskLaunchGame _asbp_game_mode_infernale))))

(event Custom|JsonFinishedSync
  (CallFunction|JsonFinshedSyncServer))

(event Custom|JsonFinshedSyncServer
  ;[1 1 1] JsonFinshedSyncServer
  (Default|JsonSyncServer (.AsBP%20Game%20Mode%20Infernale (Utilities|Casting|CastToBP_GameModeInfernale (Game|GetGameMode)))))

(event Custom|GoToEndLevel
  (bind _self self)
  ;[1 1 1] GoToEndLevel
  (Networking|SwitchHasAuthority
    (:Authority
      (if (< (Class|AdvancedSessionsLibrary|GetNumberOfNetworkPlayers) 2) :!label _label
        (Utilities|FlowControl|Delay 0.2)
        (|EndSession _self
          (:OnSuccess
            _)
          (:OnFailure
            _))
        (|DestroySession _self
          (:OnSuccess
            _)
          (:OnFailure
            _))
        (else
          (Utilities|FlowControl|Delay 0.1)
          (goto _label))))
    (:Remote
      _))
  (Game|OpenLevel(byObjectReference) "/Game/Maps/10_EndLevel.10_EndLevel"))

(event Custom|JsonFileDone_Event
  (CallFunction|JsonFinishedSync))

(event Input|EnhancedActionEvents|EnhancedInputActionIA_Tab
  (params (ActionValue :type Boolean) (ElapsedSeconds :type Float%20%28double-precision%29) (TriggeredSeconds :type Float%20%28double-precision%29) (InputAction :type Input%20Action%20Object%20Reference :default "/Game/Blueprints/0_GrayRoom/InfernaleAssets/Inputs/IA/IA_Tab.IA_Tab"))
  (bind (_hitresult _returnvalue) (Game|Player|GetHitResultUnderCursorbyChannel "TraceTypeQuery1" true))
  ;[0 0 0] Move To Location
  (if _returnvalue
    (Default|MovePawntoLocation (.AsBP%20Infernale%20Pawn (Utilities|Casting|CastToBP_InfernalePawn (Game|Player|GetPlayerPawn 0))) (.Location (Collision|BreakHitResult _hitresult)))))

(event EventBeginPlay
  (Class|PlayerControllerInfernale|SyncGameSettings)
  (if (Variables|Default|GetbDebugSplines)
    (Development|ExecuteConsoleCommand "show splines" self))
  (if (Pawn|IsLocalPlayerController)
    (bind _returnvalue (Settings|GetGameUserSettings))
    (Class|GameUserSettings|SetOverallScalabilityLevel _returnvalue 2)
    (Class|GameUserSettings|ApplySettings _returnvalue false)
    (if (Variables|/Script/InfernaleTesting.GameSettingsDataAsset|GetArthurDesoleMaisNique (Variables|Default|GetGameSettingsDataAsset))
      (Development|ExecuteConsoleCommand "DisableAllScreenMessages" 0))
    (Utilities|FlowControl|Delay 0.5)
    (Default|SwitchVisibilityOfAllWidgets (Variables|Default|GetBP_UIComponent) false true)
    (Class|WidgetBlueprintLibrary|SetFocustoGameViewport)
    (Networking|SwitchHasAuthority
      (:Authority
        (Class|VictoryManagerComponent|CallonVictoryPointsChanged (Variables|/Script/InfernaleTesting.GameModeInfernale|GetVictoryManagerComponent (.AsBP%20Game%20Mode%20Infernale (Utilities|Casting|CastToBP_GameModeInfernale (Game|GetGameMode))))))
      (:Remote
        _))
    (bind _returnvalue_2 (Actor|GetActorOfClass "/Game/Blueprints/DataGatherer/BP_DataGather.BP_DataGather_C"))
    (EventDispatchers|AssignJsonFileDone _returnvalue_2 (delegate Custom|JsonFileDone_Event))))

(event EventOnSpacePressedBP
  (Default|CallSpacePressed)
  (bind _output_get (Variables|Default|SetbHighlight (not (Variables|Default|GetbHighlight))))
  (bind _outactors (Actor|GetAllActorsOfClass "/Game/Blueprints/Flux/BP_Flux.BP_Flux_C"))
  (for _array_element _outactors
    (Default|HighlighTacticalMode _array_element _output_get)))

(event EventOnSpaceReleasedBP
  (if (Variables|/Script/InfernaleTesting.GameSettingsDataAsset|GetbUseHoldSpaceMode (Class|FunctionLibraryInfernale|GetGameSettingsDataAsset))
    (Default|CallSpaceReleased)
    (bind _output_get (Variables|Default|SetbHighlight false))
    (bind _outactors (Actor|GetAllActorsOfClass "/Game/Blueprints/Flux/BP_Flux.BP_Flux_C"))
    (for _array_element _outactors
      (Default|HighlighTacticalMode _array_element _output_get))))

(event EventOnEscapeStartedBP
  (bind _bp_uicomponent (Variables|Default|GetBP_UIComponent))
  (if (Class|UIComponent|ShouldCloseSomeMenus _bp_uicomponent)
    (Class|UIComponent|TryCloseMenu _bp_uicomponent)
    (else
      (bind _output_get (Variables|Default|SetShowOptions (not (Variables|Default|GetShowOptions))))
      (Variables|Default|SetbIsEscapeMenuOpen (not (Variables|Default|GetShowOptions)))
      (Default|ShowHideOptionsMenu _bp_uicomponent _output_get))))

(event EventLaunchNewGameBP
  (Class|PlayerControllerInfernale|EnableInputs false)
  (Widget|SetVisibility (Variables|/Game/Blueprints/Component/PlayerController/BP_UIComponent.BP_UIComponent_C|GetLoadingScreen (Variables|Default|GetBP_UIComponent)) "Visible")
  (Networking|SwitchHasAuthority
    (:Authority
      (bind _asbp_game_mode_infernale (Utilities|Casting|CastToBP_GameModeInfernale (Game|GetGameMode)))
      (Default|AskLaunchGame _asbp_game_mode_infernale))))

(event Input|KeyboardEvents|C
  (params (Key :type Key%20Structure :default "None"))
  (:Pressed
    (if (Class|PlayerControllerInfernale|IsAllowedtoCheatBP)
      (if (not (Variables|/Script/InfernaleTesting.GameSettingsDataAsset|GetbIsJuryMode (Class|FunctionLibraryInfernale|GetGameSettingsDataAsset)))
        (bind _output_get (Variables|Default|SetShowWidget (not (Variables|Default|GetShowWidget))))
        (Default|SwitchVisibilityOfAllWidgets (Variables|Default|GetBP_UIComponent) _output_get false)))))

(event Input|MouseEvents|LeftMouseButton
  (params (Key :type Key%20Structure :default "None"))
  (bind (_hitresult _returnvalue) (Game|Player|GetHitResultUnderCursorbyChannel "TraceTypeQuery1" true))
  ;[0 0 0] Move To Location
  (:Pressed
    (Utilities|FlowControl|Sequence
      (:then_0
        (Utilities|FlowControl|Gate true :!label _label
          (:Exit
            (if _returnvalue
              (Default|MovePawntoLocation (.AsBP%20Infernale%20Pawn (Utilities|Casting|CastToBP_InfernalePawn (Game|Player|GetPlayerPawn 0))) (.Location (Collision|BreakHitResult _hitresult)))))))
      (:then_1
        (goto _label Open))
      (:then_2
        (Utilities|FlowControl|Delay 0.2)
        (goto _label Close)))))

(fn ConstructionScript
  (Variables|Default|SetPlayerNetworkComponent (Variables|Default|GetBP_PlayerNetworkComponent))
  (Variables|Default|SetUIComponent (Variables|Default|GetBP_UIComponent)))

(fn OnRepBPPawn)