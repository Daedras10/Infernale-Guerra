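; Game mode for the start lobby that tracks connected player controllers, match settings and ready states.
; Setting changes and client syncs update its variables or the game instance's player info array, then RefreshData pushes the whole state to every controller.
; Client syncs also assign missing player IDs and pass the all-ready result as the launch flag.
; AskLaunchGame pre-launches controllers, copies settings into the game instance and server-travels after a short delay.
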(event Custom|AskLaunchGame
  (params (Map :type String))
  (bind _returnvalue (Game|GetGameInstance))
  (bind _asbp_game_instance_infernale (Utilities|Casting|CastToBP_GameInstanceInfernale _returnvalue))
  ;[0 0 0] AskLaunchGame
  (for _array_element (Variables|Default|GetPlayerController)
    (Default|PreLaunchGame _array_element))
  (Class|GameInstanceInfernale|SetPlayers _asbp_game_instance_infernale (Variables|Default|GetPlayers))
  (Class|GameInstanceInfernale|SetGameDuration _asbp_game_instance_infernale (CallFunction|GetGameDuration))
  (Class|GameInstanceInfernale|SetCustomGameMode _asbp_game_instance_infernale (Variables|Default|GetGameMode))
  (Class|GameInstanceInfernale|SetCustomTeamMode _asbp_game_instance_infernale (Variables|Default|GetTeamMode))
  (Class|GameInstanceInfernale|SetLastTravelScene _asbp_game_instance_infernale Map)
  (Utilities|FlowControl|Delay 0.5)
  (Class|GameInstanceInfernale|ServerTraveltoScene _asbp_game_instance_infernale Map))

(event Custom|UpdateTeamMode
  (params (Index :type Integer))
  ;[0 0 0] UpdateGameSettings
  (Variables|Default|SetTeamMode Index)
  (Development|PrintString "UpdateGameDur UpdateGameMode UpdateGameMap" false false "(R=1.000000,G=0.000000,B=0.102836,A=1.000000)" 2e+02)
  (CallFunction|RefreshData false))

(event Custom|UpdateGameMode
  (params (Index :type Integer))
  ;[0 0 0] UpdateGameSettings
  (Variables|Default|SetGameMode Index)
  (Development|PrintString "UpdateGameDur UpdateGameMode UpdateGameMap" false false "(R=1.000000,G=0.000000,B=0.102836,A=1.000000)" 2e+02)
  (CallFunction|RefreshData false))

(event Custom|UnsetReady
  (bind _returnvalue (Game|GetGameInstance))
  (bind _asbp_game_instance_infernale (Utilities|Casting|CastToBP_GameInstanceInfernale _returnvalue))
  (bind _opponentplayerinfo (Variables|/Script/InfernaleTesting.GameInstanceInfernale|GetOpponentPlayerInfo _asbp_game_instance_infernale))
  ;[0 0 0] UnsetReady
  (bind _structout (Utilities|Struct|SetmembersinPlayerInfo (Variables|/Script/InfernaleTesting.GameInstanceInfernale|GetPersonalPlayerInfo _asbp_game_instance_infernale) false))
  (Variables|/Script/InfernaleTesting.GameInstanceInfernale|SetPersonalPlayerInfo _asbp_game_instance_infernale _structout)
  (for (_array_element _array_index) _opponentplayerinfo
    (bind _structout_2 (Utilities|Struct|SetmembersinPlayerInfo _array_element false))
    (Utilities|Array|SetArrayElem _opponentplayerinfo _array_index _structout_2))
  (CallFunction|RefreshData false)
  (Variables|Default|SetAllPlayerReady? false))

(event Custom|OnPlayerConnected
  (params (PlayerController :type BP%20Player%20Controller%20Start%20Lobby%20Object%20Reference))
  ;[0 0 0] OnPlayerConnected
  (Math|Integer|IncrementInt (Variables|Default|GetPlayers)
    (:%20%20
      (Utilities|Array|Add (Variables|Default|GetPlayerController) PlayerController)
      (CallFunction|RefreshData false))))

(event Custom|SyncDataClient
  (params (PlayerInfo :type Player%20Info%20Structure) (PlayerController :type BP%20Player%20Controller%20Start%20Lobby%20Object%20Reference))
  (bind _returnvalue (Game|GetGameInstance))
  (bind _asbp_game_instance_infernale (Utilities|Casting|CastToBP_GameInstanceInfernale _returnvalue))
  (bind _opponentplayerinfo (Variables|/Script/InfernaleTesting.GameInstanceInfernale|GetOpponentPlayerInfo _asbp_game_instance_infernale))
  ;[0 0 0] SyncDataClient
  (bind _structout (Utilities|Struct|SetmembersinPlayerInfo PlayerInfo PlayerController))
  (if (.isInRoom (Utilities|Struct|BreakPlayerInfo _structout))
    (if (== (Utilities|Array|Length _opponentplayerinfo) 0)
      _
      (else
        (for (_array_element _array_index) _opponentplayerinfo
          (if (== (.PlayerController (Utilities|Struct|BreakPlayerInfo _structout)) (.playercontroller _array_element))
            (Variables|Default|SetisUnique? true)
            (Utilities|Array|SetArrayElem _opponentplayerinfo _array_index _structout))
          (if (not (.playerisready _array_element))
            (Variables|Default|SetAllPlayerReady? false)))))
    (Utilities|Array|AddUnique _opponentplayerinfo _structout)
    (else
      (Utilities|Array|RemoveItem _opponentplayerinfo (Utilities|Struct|MakePlayerInfo (.PlayerID (Utilities|Struct|BreakPlayerInfo _structout)) (.PlayerName (Utilities|Struct|BreakPlayerInfo _structout)) (.PlayerOwnerInfo (Utilities|Struct|BreakPlayerInfo _structout)) (.PlayerController (Utilities|Struct|BreakPlayerInfo _structout)) (.PlayerIsReady (Utilities|Struct|BreakPlayerInfo _structout)) true))))
  (CallFunction|ReorderPlayerIDsbyID _opponentplayerinfo)
  (Development|PrintString "SyncData" false false "(R=1.000000,G=0.000000,B=0.813568,A=1.000000)")
  (CallFunction|RefreshData (Variables|Default|GetAllPlayerReady?))
  (Variables|Default|SetAllPlayerReady? true))

(event Custom|AskRefresh
  (params (PlayerController :type BP%20Player%20Controller%20Start%20Lobby%20Object%20Reference) (LaunchGame :type Boolean))
  ;[0 0 0] AskRefresh
  (Default|RefreshServer PlayerController (Variables|Default|GetPlayers) (Variables|Default|GetGameMode) (Variables|Default|GetGameDuration) (Variables|Default|GetGameMap) (Variables|Default|GetTeamMode) (Variables|/Script/InfernaleTesting.GameInstanceInfernale|GetOpponentPlayerInfo (.AsBP%20Game%20Instance%20Infernale (Utilities|Casting|CastToBP_GameInstanceInfernale (Game|GetGameInstance)))) LaunchGame))

(event Custom|UpdateGameDuration
  (params (Index :type Integer))
  ;[0 0 0] UpdateGameSettings
  (Variables|Default|SetGameDuration Index)
  (Development|PrintString "UpdateGameDur UpdateGameMode UpdateGameMap" false false "(R=1.000000,G=0.000000,B=0.102836,A=1.000000)" 2e+02)
  (CallFunction|RefreshData false))

(event Custom|LeaveGame
  (params (LeavingPlayer :type BP%20Player%20Controller%20Start%20Lobby%20Object%20Reference))
  ;[0 0 0] LeaveGame
  (Default|CleanupInfo LeavingPlayer)
  (if (== LeavingPlayer (Game|GetPlayerController 0))
    (Default|LeaveSession LeavingPlayer)
    (else
      (Default|DestroySessionClient LeavingPlayer)
      (Utilities|Array|RemoveItem (Variables|Default|GetPlayerController) LeavingPlayer)
      (CallFunction|RefreshData false))))

(event Custom|UpdateGameMap
  (params (Index :type Integer))
  ;[0 0 0] UpdateGameSettings
  (Variables|Default|SetGameMap Index)
  (Development|PrintString "UpdateGameDur UpdateGameMode UpdateGameMap" false false "(R=1.000000,G=0.000000,B=0.102836,A=1.000000)" 2e+02)
  (CallFunction|RefreshData false))

(event Custom|RefreshData
  (params (LaunchGame :type Boolean))
  (bind _playercontroller (Variables|Default|GetPlayerController))
  ;[0 0 0] RefreshData
  (Development|PrintString (Utilities|String|ToString(Integer) (Utilities|Array|Length _playercontroller)) false false "(R=0.205152,G=1.000000,B=0.000000,A=1.000000)" 2e+02)
  (for _array_element _playercontroller
    (CallFunction|AskRefresh _array_element LaunchGame)))

(event EventOnLogout
  (params (ExitingController :type Controller%20Object%20Reference))
  ;[0 0 0] OnLogout
  (Development|PrintText (Utilities|Text|FormatText " {a} has left the game" ExitingController)))

(fn ConstructionScript)

(fn GetGameDuration
  (return (* (Utilities|Select :Index (Variables|Default|GetGameDuration) :Option%200 25.1 :Option%201 2e+01 :Option%202 15.0 :Option%203 1e+01 :Option%204 0.16667) 6e+01)))

(fn ReorderPlayerIDs
  (params (PlayerInfoArray :type Array%20of%20Player%20Info%20Structures))
  (bind _returnvalue (Utilities|Array|LastIndex PlayerInfoArray))
  (for _index (range 0 _returnvalue)
    (for _index_2 (range _index _returnvalue)
      (if (> (.playerid (Utilities|Array|Get(acopy) PlayerInfoArray _index_2)) (.playerid (Utilities|Array|Get(acopy) PlayerInfoArray _index)))
        (Utilities|Array|Swap PlayerInfoArray _index_2 _index))))
  (for (_array_element _array_index) PlayerInfoArray
    (bind _structout (Utilities|Struct|SetmembersinPlayerInfo _array_element _array_index))
    (Utilities|Array|SetArrayElem PlayerInfoArray _array_index _structout)
    (Default|UpdatePersonalInfoOwning (.AsBP%20Player%20Controller%20Start%20Lobby (Utilities|Casting|CastToBP_PlayerControllerStartLobby (.PlayerController (Utilities|Struct|BreakPlayerInfo _structout)))) _structout))
  (return))

(fn ReorderPlayerIDsbyID
  (params (PlayerInfoArray :type Array%20of%20Player%20Info%20Structures) (CurrentMode :type Integer))
  (switch int CurrentMode
    (:Default
      _)
    (:0
      _))
  (for (_array_element _array_index) PlayerInfoArray
    (if (< (.PlayerID (Utilities|Struct|BreakPlayerInfo _array_element)) 0)
      (bind _structout (Utilities|Struct|SetmembersinPlayerInfo _array_element _array_index (Utilities|Struct|MakeOwner (CallFunction|GetPlayerID _array_index) (CallFunction|GetTeamID _array_index))))
      (Utilities|Array|SetArrayElem PlayerInfoArray _array_index _structout)
      (Default|UpdatePersonalInfoOwning (.AsBP%20Player%20Controller%20Start%20Lobby (Utilities|Casting|CastToBP_PlayerControllerStartLobby (.PlayerController (Utilities|Struct|BreakPlayerInfo _structout)))) _structout))))