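; Player controller for the start lobby, linking each player's lobby UI to BP_GameModeStartLobby.
; On local begin play it creates player info with a random name, and NotifyServer retries until the game mode is found, then registers and creates lobby and loading widgets.
; Setting changes, launch and leave requests go to the game mode, while refreshes update the lobby widget and game instance.
; It also handles session teardown and editor self-test auto-ready.
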(event Custom|AskRefreshServer
  ;[0 0 0] AskRefreshServer
  (Default|AskRefresh (Variables|Default|GetAs%20BP%20Game%20Mode%20Start%20Lobby) self false))

(event Custom|RefreshServer
  (params (Players :type Integer) (GameMode :type Integer) (GameDuration :type Integer) (GameMap :type Integer) (TeamMode :type Integer) (PlayerInfo :type Array%20of%20Player%20Info%20Structures) (LaunchGame :type Boolean))
  ;[0 0 0] RefreshServer
  (CallFunction|RefreshOwning Players GameMode GameDuration GameMap TeamMode PlayerInfo LaunchGame))

(event Custom|LaunchGameServer
  (params (Map :type String))
  ;[0 0 0] LaunchGameServer
  (Default|AskLaunchGame (Variables|Default|GetAs%20BP%20Game%20Mode%20Start%20Lobby) Map)
  (|UpdateSession 0 4 0 false false false true false false))

(event Custom|Create%20TestDamienWidget
  ;[0 0 0] Create TestDamienWidget
  (bind _returnvalue (UserInterface|CreateWidget "/Game/_Draft/Damien/BP/Widgets/WBP_TestDamien.WBP_TestDamien_C" self))
  (Development|PrintString " CreateWidget in PlayerCOntroller Test Damien Created" false false)
  (UserInterface|Viewport|AddtoViewport _returnvalue 1))

(event Custom|SyncPlayerDataServer
  (params (PlayerInfo :type Player%20Info%20Structure))
  ;[0 0 0] SyncPlayerDataServer
  (bind _asbp_game_mode_start_lobby (Utilities|Casting|CastToBP_GameModeStartLobby (Game|GetGameMode)))
  (Default|SyncDataClient _asbp_game_mode_start_lobby PlayerInfo self))

(event Custom|NotifyServer
  ;[0 0 0] NotifyServer
  (bind _asbp_game_mode_start_lobby (Utilities|Casting|CastToBP_GameModeStartLobby (Game|GetGameMode) :!label _label)
    (:then
      (bind _output_get (Variables|Default|SetAs%20BP%20Game%20Mode%20Start%20Lobby _asbp_game_mode_start_lobby))
      (Default|OnPlayerConnected _output_get self)
      (CallFunction|CreateWidgets)
      (CallFunction|AskRefreshServer))
    (:CastFailed
      (Utilities|FlowControl|Delay 0.1)
      (goto _label))))

(event Custom|UpdatePersonalInfoOwning
  (params (PlayerInfo :type Player%20Info%20Structure))
  ;[0 0 0] UpdatePersonalInfoOwning
  (bind _structout (Utilities|Struct|SetmembersinPlayerInfo PlayerInfo self))
  (Variables|/Script/InfernaleTesting.GameInstanceInfernale|SetPersonalPlayerInfo (.AsBP%20Game%20Instance%20Infernale (Utilities|Casting|CastToBP_GameInstanceInfernale (Game|GetGameInstance))) _structout))

(event Custom|Cleanup%20info
  (bind _returnvalue (Game|GetGameInstance))
  (bind _asbp_game_instance_infernale (Utilities|Casting|CastToBP_GameInstanceInfernale _returnvalue))
  ;[0 0 0] Cleanup info
  (Variables|/Script/InfernaleTesting.GameInstanceInfernale|SetPersonalPlayerInfo _asbp_game_instance_infernale "")
  (Utilities|Array|Clear (Variables|/Script/InfernaleTesting.GameInstanceInfernale|GetOpponentPlayerInfo _asbp_game_instance_infernale)))

(event Custom|SyncPlayerData
  ;[0 0 0] SyncPlayerData
  (CallFunction|SyncPlayerDataServer (Variables|/Script/InfernaleTesting.GameInstanceInfernale|GetPersonalPlayerInfo (.AsBP%20Game%20Instance%20Infernale (Utilities|Casting|CastToBP_GameInstanceInfernale (Game|GetGameInstance))))))

(event Custom|DestroySessionClient
  ;[0 0 0] DestroySessionClient
  (|DestroySession self
    (:OnSuccess
      (Game|OpenLevel(byObjectReference) "/Game/Maps/01_HostJoin.01_HostJoin"))))

(event Custom|CreateStartGameWidget
  (bind _self self)
  ;[0 0 0] CreateStartGameWidget
  (bind _returnvalue (UserInterface|CreateWidget "/Game/UI/StartGameLobby/WBP_StartGameLobby.WBP_StartGameLobby_C" _self))
  (bind _output_get (Variables|Default|SetWBP_Lobby _returnvalue))
  (UserInterface|Viewport|AddtoViewport _output_get 0)
  (Default|Init _output_get _self))

(event Custom|CreateLoadingScreenWidget
  ;[0 0 0] CreateLoadingScreenWidget
  (bind _returnvalue (UserInterface|CreateWidget "/Game/UI/StartGameLobby/WBP_LoadingScreen.WBP_LoadingScreen_C" self))
  (bind _output_get (Variables|Default|SetLoadingScreen _returnvalue))
  (UserInterface|Viewport|AddtoViewport _output_get 1)
  (Widget|SetRenderOpacity _output_get 0.0)
  (Widget|SetVisibility _output_get "Hidden"))

(event Custom|CreateWidgets
  ;[0 0 0] CreateWidget
  (CallFunction|CreateStartGameWidget)
  (CallFunction|CreateLoadingScreenWidget)
  (CallFunction|TestingSetup))

(event Custom|TestingSetup
  ;[0 0 0] TestingSetup
  (Utilities|FlowControl|Delay 0.2)
  (if (and (Variables|/Script/InfernaleTesting.GameSettingsDataAsset|GetSelfTesting (Class|FunctionLibraryInfernale|GetGameSettingsDataAsset)) (Class|FunctionLibraryInfernale|InEditor))
    (Networking|SwitchHasAuthority
      (:Remote
        (Default|Ready (Variables|Default|GetWBP_Lobby))))))

(event Custom|CreatePersonalInfo
  (bind _asbp_game_instance_infernale (Utilities|Casting|CastToBP_GameInstanceInfernale (Game|GetGameInstance)))
  (bind _returnvalue (Class|NameDataAsset|GetRandomName (Variables|/Script/InfernaleTesting.GameSettingsDataAsset|GetNameDataAsset (Variables|/Script/InfernaleTesting.GameInstanceInfernale|GetGameSettingsDataAsset _asbp_game_instance_infernale))))
  (Variables|/Script/InfernaleTesting.GameInstanceInfernale|SetPersonalPlayerInfo _asbp_game_instance_infernale (Utilities|Struct|MakePlayerInfo -1 (Utilities|String|Replace _returnvalue "\"") (Utilities|Struct|MakeOwner "Player1" "Team1") self)))

(event Custom|UpdateGameDuration
  (params (Index :type Integer))
  ;[0 0 0] UpdateGameSettings
  (Default|UpdateGameDuration (Variables|Default|GetAs%20BP%20Game%20Mode%20Start%20Lobby) Index))

(event Custom|LeaveSession
  (bind _returnvalue (Game|GetGameInstance))
  (bind _asbp_game_instance_infernale (Utilities|Casting|CastToBP_GameInstanceInfernale _returnvalue))
  ;[0 0 0] LeaveSession
  (|DestroySession (Game|GetPlayerController 0)
    (:OnSuccess
      (Game|OpenLevel(byObjectReference) "/Game/Maps/01_HostJoin.01_HostJoin")
      (Variables|/Script/InfernaleTesting.GameInstanceInfernale|SetPersonalPlayerInfo _asbp_game_instance_infernale "")
      (Utilities|Array|Clear (Variables|/Script/InfernaleTesting.GameInstanceInfernale|GetOpponentPlayerInfo _asbp_game_instance_infernale)))))

(event Custom|PreLaunchGame
  ;[0 0 0] PreLaunchGame
  (Default|PreLaunchGame (Variables|Default|GetWBP_Lobby))
  (Default|CreateLoadingScreen (.AsBP%20Game%20Instance%20Infernale (Utilities|Casting|CastToBP_GameInstanceInfernale (Game|GetGameInstance)))))

(event Custom|UpdateGameMode
  (params (Index :type Integer))
  (bind _as_bp_game_mode_start_lobby (Variables|Default|GetAs%20BP%20Game%20Mode%20Start%20Lobby))
  ;[0 0 0] UpdateGameSettings
  (Default|UpdateGameMode _as_bp_game_mode_start_lobby Index)
  (Default|UnsetReady _as_bp_game_mode_start_lobby))

(event Custom|UpdateTeamMode
  (params (Index :type Integer))
  (bind _as_bp_game_mode_start_lobby (Variables|Default|GetAs%20BP%20Game%20Mode%20Start%20Lobby))
  ;[0 0 0] UpdateGameSettings
  (Default|UpdateTeamMode _as_bp_game_mode_start_lobby Index)
  (Default|UnsetReady _as_bp_game_mode_start_lobby))

(event Custom|RefreshOwning
  (params (Players :type Integer) (GameMode :type Integer) (GameDuration :type Integer) (GameMap :type Integer) (TeamMode :type Integer) (PlayerInfo :type Array%20of%20Player%20Info%20Structures) (LaunchGame :type Boolean))
  (bind _returnvalue (Game|GetGameInstance))
  (bind _asbp_game_instance_infernale (Utilities|Casting|CastToBP_GameInstanceInfernale _returnvalue))
  ;[0 0 0] RefreshOwning
  (Utilities|FlowControl|DelayUntilNextTick)
  (Default|SetPlayerQuantity (Variables|Default|GetWBP_Lobby) Players)
  (Class|GameInstanceInfernale|SetPlayers _asbp_game_instance_infernale Players)
  (Class|GameInstanceInfernale|SetCustomGameMode _asbp_game_instance_infernale GameMode)
  (Default|UpdateGameMode (Variables|Default|GetWBP_Lobby) GameMode)
  (Default|UpdateGameDuration (Variables|Default|GetWBP_Lobby) GameDuration)
  (Default|UpdateGameMap (Variables|Default|GetWBP_Lobby) GameMap)
  (Default|UpdateTeamMode (Variables|Default|GetWBP_Lobby) TeamMode)
  (Default|UpdatePlayerList (Variables|Default|GetWBP_Lobby) PlayerInfo LaunchGame)
  (Variables|/Script/InfernaleTesting.GameInstanceInfernale|SetOpponentPlayerInfo _asbp_game_instance_infernale PlayerInfo))

(event Custom|UpdateGameMap
  (params (Index :type Integer))
  (bind _as_bp_game_mode_start_lobby (Variables|Default|GetAs%20BP%20Game%20Mode%20Start%20Lobby))
  ;[0 0 0] UpdateGameSettings
  (Default|UpdateGameMap _as_bp_game_mode_start_lobby Index)
  (Default|UnsetReady _as_bp_game_mode_start_lobby))

(event Custom|LeaveGame
  (params (Leaving%20Player :type BP%20Player%20Controller%20Start%20Lobby%20Object%20Reference))
  ;[0 0 0] LeaveGame
  (Default|LeaveGame (Variables|Default|GetAs%20BP%20Game%20Mode%20Start%20Lobby) Leaving%20Player))

(event EventBeginPlay
  ;[0 0 0] BeginPlay
  (if (Pawn|IsLocalController)
    (CallFunction|CreatePersonalInfo)
    (CallFunction|NotifyServer)
    (Variables|Default|SetbShowMouseCursor true)
    (Variables|/Script/InfernaleTesting.GameInstanceInfernale|SetbIsPhilosophicallyAccurateGame (.AsBP%20Game%20Instance%20Infernale (Utilities|Casting|CastToBP_GameInstanceInfernale (Game|GetGameInstance))) (not (Variables|/Script/InfernaleTesting.GameSettingsDataAsset|GetbUsePreGameSandbox (Class|FunctionLibraryInfernale|GetGameSettingsDataAsset))))
    (Utilities|FlowControl|Delay 0.1)
    (CallFunction|SyncPlayerData)))

(fn ConstructionScript)