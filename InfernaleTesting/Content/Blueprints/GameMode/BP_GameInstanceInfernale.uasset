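; Game instance for Infernale that manages online sessions, level travel, player lobby info and music volume.
; Hosting destroys any existing session, advertises one tagged with game, secret code, Steam ID and host name, then opens the lobby as listen server; matching filter builders and invite handling support joining.
; Loading settings rescales active music by master volume, with dynamic ambience following a curve of amalgams on map.
; Loading-screen removal events are empty stubs.
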(event Custom|JoinSessionInfernale
  (params (SessionToJoin :type Blueprint%20Session%20Result%20Structure))
  ;[0 0 0] JoinSessionInfernale
  (|JoinSession (Game|GetPlayerController 0) SessionToJoin))

(event Custom|CreateSessionName
  (params (Secret :type String))
  (bind _returnvalue (Game|GetPlayerController 0))
  ;[0 0 0] Event CreateSession
  (|DestroySession _returnvalue
    (:OnSuccess
      _)
    (:OnFailure
      _))
  (|AdvancedSession (CallFunction|CreateNewSessionParams (CallFunction|GetInfernaleParamsCode Secret)) _returnvalue 4 0 (Class|GameInstanceInfernale|UseLAN) true false true true true false false false true false true
    (:OnSuccess
      (Development|PrintString (Utilities|String|ToString(Text) (Utilities|Text|FormatText "SessionStarted with key {key}" Secret)) false false)
      (Game|OpenLevel(byObjectReference) "/Game/Maps/03_Lobby.03_Lobby" true "listen"))))

(event Custom|Cleanup
  ;[0 0 0] Cleanup
  (Variables|Default|SetPersonalPlayerInfo (Utilities|Struct|MakePlayerInfo -1 "" "(Player=Nature,Team=NatureTeam)" 0 false false))
  (Utilities|Array|Clear (Variables|Default|GetOpponentPlayerInfo)))

(event Custom|CreateLoadingScreen
  (bind _returnvalue (UserInterface|CreateWidget "/Game/UI/StartGameLobby/WBP_LoadingScreen.WBP_LoadingScreen_C" (Game|GetPlayerController 0)))
  (UserInterface|Viewport|AddtoViewport _returnvalue 10000))

(event Custom|ResetReadyState
  (bind _opponentplayerinfo (Variables|Default|GetOpponentPlayerInfo))
  (for (_array_element _array_index) _opponentplayerinfo
    (bind _structout (Utilities|Struct|SetmembersinPlayerInfo _array_element false))
    (Utilities|Array|SetArrayElem _opponentplayerinfo _array_index _structout)
    (Development|PrintString (Utilities|String|ToString(Boolean) (.PlayerIsReady (Utilities|Struct|BreakPlayerInfo _array_element)))))
  (bind _structout_2 (Utilities|Struct|SetmembersinPlayerInfo (Variables|Default|GetPersonalPlayerInfo) false))
  (Variables|Default|SetPersonalPlayerInfo _structout_2))

(event Custom|RemoveLoadingScreen)

(event Custom|ChangeMusicVolume
  (bind _datagatherer (Variables|Default|GetDataGatherer))
  (bind _playersnapshots (Variables|/Script/InfernaleTesting.DataGathererActor|GetPlayerSnapshots _datagatherer))
  (Utilities|FlowControl|Sequence
    (:then_0
      (Utilities|IsValid (Variables|Default|GetMainMenuTheme)
        (:Is%20Valid
          (bind _returnvalue (Class|GameInstanceInfernale|GetSoundType "Music" "Main Theme"))
          (Audio|Components|Audio|SetVolumeMultiplier (Variables|Default|GetMainMenuTheme) (* (.Volume (Utilities|Struct|BreakSoundType _returnvalue)) (Variables|Default|GetMasterXMusicVolume)) :!class /Script/Engine.AudioComponent))))
    (:then_1
      (Utilities|IsValid (Variables|Default|GetLobbyTheme)
        (:Is%20Valid
          (bind _returnvalue_2 (Class|GameInstanceInfernale|GetSoundType "Music" "Lobby Theme"))
          (Audio|Components|Audio|SetVolumeMultiplier (Variables|Default|GetLobbyTheme) (* (.Volume (Utilities|Struct|BreakSoundType _returnvalue_2)) (Variables|Default|GetMasterXMusicVolume)) :!class /Script/Engine.AudioComponent))))
    (:then_2
      (for _array_element (Variables|Default|GetAmbientTheme_Constant)
        (Utilities|IsValid _array_element
          (:Is%20Valid
            (bind _returnvalue_3 (Class|SoundsDataAsset|GetSoundVolumefromSoundinType (Variables|Default|GetDA%20Sounds) (Variables|/Script/Engine.AudioComponent|GetSound _array_element) "Music"))
            (Audio|Components|Audio|SetVolumeMultiplier _array_element (* _returnvalue_3 (Variables|Default|GetMasterXMusicVolume)) :!class /Script/Engine.AudioComponent)))))
    (:then_3
      (for _array_element_2 (Variables|Default|GetAmbientTheme_Dynamic)
        (Utilities|IsValid _array_element_2
          (:Is%20Valid
            (Utilities|IsValid _datagatherer
              (:Is%20Valid
                (Audio|Components|Audio|SetVolumeMultiplier _array_element_2 (* (Math|Curves|GetFloatValue (Variables|Default|GetDynamicMelodyAmbientCurve) (Math|Conversions|ToFloat(Integer) (.AmalgamsOnMap (Utilities|Struct|BreakPlayerSnapshot (Utilities|Array|Get(acopy) _playersnapshots (- (Utilities|Array|Length _playersnapshots) 1)))))) (Variables|Default|GetMasterXMusicVolume)) :!class /Script/Engine.AudioComponent)))))))
    (:then_4
      (bind _returnvalue_4 (Class|GameInstanceInfernale|GetSoundType "Music" "Ambient Mid - Battle"))
      (for _array_element_3 (Variables|Default|GetBattleTheme_Instances)
        (Utilities|IsValid _array_element_3
          (:Is%20Valid
            (Audio|Components|Audio|SetVolumeMultiplier _array_element_3 (* (.Volume (Utilities|Struct|BreakSoundType _returnvalue_4)) (Variables|Default|GetMasterXMusicVolume)) :!class /Script/Engine.AudioComponent)))))
    (:then_5
      (Utilities|IsValid (Variables|Default|GetVictoryJingle)
        (:Is%20Valid
          (bind _returnvalue_5 (Class|GameInstanceInfernale|GetSoundType "Music" "Victory Jingle"))
          (Audio|Components|Audio|SetVolumeMultiplier (Variables|Default|GetVictoryJingle) (* (.Volume (Utilities|Struct|BreakSoundType _returnvalue_5)) (Variables|Default|GetMasterXMusicVolume)) :!class /Script/Engine.AudioComponent))))
    (:then_6
      (Utilities|IsValid (Variables|Default|GetPostGameTheme)
        (:Is%20Valid
          (bind _returnvalue_6 (Class|GameInstanceInfernale|GetSoundType "Music" "Postgame"))
          (Audio|Components|Audio|SetVolumeMultiplier (Variables|Default|GetPostGameTheme) (* (.Volume (Utilities|Struct|BreakSoundType _returnvalue_6)) (Variables|Default|GetMasterXMusicVolume)) :!class /Script/Engine.AudioComponent))))))

(event Custom|NisemonoBeginPlay
  ;[0 0 0] 偽物BeginPlay
  (EventDispatchers|AssignOnSetDataGatherer (delegate Custom|OnSetDataGatherer_Event))
  (EventDispatchers|AssignOnLoadedSettings (delegate Custom|OnLoadedSettings_Event))
  (Class|GameInstanceInfernale|LoadGameSettings))

(event Custom|OnSetDataGatherer_Event
  (params (DataGatherer :type BP%20Data%20Gather%20Object%20Reference))
  ;[0 0 0] 偽物BeginPlay
  (Variables|Default|SetDataGatherer DataGatherer))

(event Custom|OnLoadedSettings_Event
  ;[0 0 0] 偽物BeginPlay
  (CallFunction|ChangeMusicVolume))

(event Custom|TravelToScene
  (params (SceneName :type String) (Is%20Philosophically%20Accurate%20Game :type Boolean))
  ;[0 0 0] TravelToScene
  (Development|ExecuteConsoleCommand (Utilities|String|Append "servertravel " SceneName) (Game|GetPlayerController 0)))

(event EventBeginLoadingScreenBP)

(event EventOnSessionInviteAccepted
  (params (LocalPlayerNum :type Integer) (PersonInvited :type BP%20Unique%20Net%20Id%20Structure) (SessionToJoin :type Blueprint%20Session%20Result%20Structure%20%28by%20ref%29))
  (bind _returnvalue (Game|GetPlayerController 0))
  ;[0 0 0] EventOnSessionInviteAccepted
  (|DestroySession _returnvalue
    (:OnSuccess
      _)
    (:OnFailure
      _))
  (|JoinSession _returnvalue SessionToJoin))

(event EventCreateSession
  ;[0 0 0] Event CreateSession
)

(event EventEndLoadingScreenBP)

(fn GetInfernaleParams
  (return (Utilities|Array|MakeArray (Class|AdvancedSessionsLibrary|MakeLiteralSessionPropertyString "Game" "Infernale"))))

(fn GetInfernaleParamsFilters
  (Utilities|Array|Clear (LocalVariables|GetReturnFilters))
  (for _array_element (CallFunction|GetInfernaleParams)
    (Utilities|Array|Add (LocalVariables|GetReturnFilters) (Class|AdvancedSessionsLibrary|MakeLiteralSessionSearchProperty _array_element "Equals")))
  (return (LocalVariables|GetReturnFilters)))

(fn GetInfernaleParamsFilterswithCode
  (params (Secret :type String))
  (Utilities|Array|Clear (LocalVariables|GetReturnFilters))
  (for _array_element (CallFunction|GetInfernaleParamsCode Secret)
    (Utilities|Array|Add (LocalVariables|GetReturnFilters) (Class|AdvancedSessionsLibrary|MakeLiteralSessionSearchProperty _array_element "Equals")))
  (return (LocalVariables|GetReturnFilters)))

(fn GetInfernaleParamsCode
  (params (Secret :type String))
  (return (Utilities|Array|MakeArray (Class|AdvancedSessionsLibrary|MakeLiteralSessionPropertyString "Game" "Infernale") (Class|AdvancedSessionsLibrary|MakeLiteralSessionPropertyString "SecretCode" Secret))))

(fn CreateNewSessionwithName
  (bind _sessionname (|CallParentFunction))
  (CallFunction|CreateSessionName _sessionname)
  (return _sessionname))

(fn CreateNewSessionParams
  (params (SessionProperty :type Array%20of%20Session%20Property%20Key%20Pair%20Structures))
  (bind _returnvalue (Class|AdvancedSteamFriendsLibrary|GetLocalSteamIDfromSteam))
  (Utilities|Array|Add SessionProperty (Class|AdvancedSessionsLibrary|MakeLiteralSessionPropertyString "SteamID" (Class|AdvancedSessionsLibrary|UniqueNetIdtoString _returnvalue)))
  (Utilities|Array|Add SessionProperty (Class|AdvancedSessionsLibrary|MakeLiteralSessionPropertyString "SessionName" (select (Class|FunctionLibraryInfernale|InEditor) (Utilities|Platform|GetPlatformUserName) (Class|AdvancedIdentityLibrary|GetPlayerNickname _returnvalue))))
  (return SessionProperty))

(fn GetWidgetBP)