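; BP_UnitActor is a team-owned unit actor with a placeholder cube as its visual.
; An ownership visual refresh tints the cube with the owner's team color, and damage scales it down in proportion to remaining health.
; The construction script assigns the cube as DebugCube and registers it with the fog-of-war component, along with the Fogg mesh as its fog hole.
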(event EventRefreshVisualOwned
  (Rendering|Material|SetVectorParameterValueonMaterials (Variables|Default|GetCube) "Color" (CallFunction|GetTeamVectorColor (.Team (Utilities|Struct|BreakOwner (Variables|Default|GetOwnerInfo))))))

(event EventOnDamagedBP
  (params (NewHealth :type Float%20%28single-precision%29) (MaxHealth :type Float%20%28single-precision%29) (DamageAmount :type Float%20%28single-precision%29))
  (Transformation|SetRelativeScale3D (Variables|Default|GetCube) (* "0.625000,0.625000,0.625000" (/ NewHealth MaxHealth))))

(fn ConstructionScript
  (bind _fogofwarcomponent (Variables|Default|GetFogOfWarComponent))
  (Variables|Default|SetDebugCube (Variables|Default|GetCube))
  (Variables|/Script/InfernaleTesting.FogOfWarComponent|SetFogHoleMesh _fogofwarcomponent (Variables|Default|GetFogg))
  (Variables|/Script/InfernaleTesting.FogOfWarComponent|SetActorMeshes _fogofwarcomponent (Utilities|Array|MakeArray (Variables|Default|GetCube))))