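; Base Blueprint for Niagara-based unit visuals, pairing a main particle system with a team-colored torch effect.
; One-time owner and speed-multiplier events set the torch color and curve-driven, slightly randomized shape size.
; Activation requires both setups, polls each tick until WasInit passes, then starts the units and, 20% of the time, the torch.
; The torch gets a random offset on BeginPlay.
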(event Custom|SetSizeBySpeed
  (bind _sizebyspeedcurve (Variables|Default|GetSizeBySpeedCurve))
  (bind _speed_multiplier (Variables|Default|GetSpeed%20Multiplier))
  (bind _returnvalue (Math|Curves|GetVectorValue _sizebyspeedcurve _speed_multiplier))
  (bind (_x _y _z) (Math|Vector|BreakVector _returnvalue))
  (Class|NiagaraComponent|SetNiagaraVariableVec3 (Variables|Default|GetNiagaraComponent) "ActiveShapeSize" (Math|Vector|MakeVector (+ (Math|Random|RandomFloatinRange -1e+01 1e+01) _x) _y _z)))

(event EventBeginPlay
  (bind _torch (Variables|Default|GetTorch))
  (Transformation|AddLocalOffset _torch (Math|Vector|MakeVector (Math|Random|RandomFloatinRange -2e+01 2e+01) (Math|Random|RandomFloatinRange -1e+02 1e+02) 5e+01) false false)
  (Class|NiagaraComponent|SetTickBehavior _torch "ForceTickLast"))

(event EventSpeedMultiplierUpdatedBP
  (params (SpeedMultiplier :type Float%20%28single-precision%29))
  (Variables|Default|SetSpeed%20Multiplier SpeedMultiplier)
  (Utilities|FlowControl|DoOnce false
    (:Completed
      (CallFunction|SetSizebySpeed)
      (Variables|Default|SetUnitsWasInit true)
      (Variables|Default|SetActivated false))))

(event EventOwnerBP
  (params (OwnerInfo :type Owner%20Structure))
  (Utilities|FlowControl|DoOnce false
    (:Completed
      (Niagara|SetNiagaraVariable(LinearColor) (Variables|Default|GetTorch) "TeamColor" (.SpecifiedColor (Utilities|Struct|BreakSlateColor (CallFunction|GetTeamColor (.Team (Utilities|Struct|BreakOwner OwnerInfo))))))
      (Variables|Default|SetTorchWasInit true)
      (Variables|Default|SetActivated false))))

(event EventActivateBP
  (params (Activate :type Boolean))
  (if (Math|Boolean|ANDBoolean Activate (Variables|Default|GetTorchWasInit) (Variables|Default|GetUnitsWasInit))
    (if (not (Variables|Default|GetActivated))
      (bind _returnvalue (Class|NiagaraUnitasActor|WasInit :!label _label))
      (if _returnvalue
        (Variables|Default|SetActivated true)
        (Components|Activation|Activate (Variables|Default|GetNiagaraComponent) false)
        (if (Math|Random|RandomBoolwithWeight 0.2)
          (Components|Activation|Activate (Variables|Default|GetTorch) false))
        (else
          (Utilities|FlowControl|DelayUntilNextTick)
          (goto _label))))
    (elif (Variables|Default|GetActivated)
      (Variables|Default|SetActivated false)
      (Components|Activation|Deactivate (Variables|Default|GetNiagaraComponent)))))

(fn ConstructionScript)