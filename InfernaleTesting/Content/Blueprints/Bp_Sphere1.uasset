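; Trigger volume actor that blends a referenced SkyLight between outside and inside lighting as a Pawn enters or leaves its Capsule.
; Overlap events flip Target and print debug messages.
; Tick moves a clamped progress value toward the matching end at LerpSpeed, then lerps the light's intensity and color from it.
; Unconnected nodes for snapping progress instantly remain in the graph but never run.
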(event OnComponentBeginOverlap(Capsule)
  (params (OverlappedComponent :type Primitive%20Component%20Object%20Reference) (OtherActor :type Actor%20Object%20Reference) (OtherComp :type Primitive%20Component%20Object%20Reference) (OtherBodyIndex :type Integer) (bFromSweep :type Boolean) (SweepResult :type Hit%20Result%20Structure%20%28by%20ref%29))
  (Utilities|Casting|CastToPawn OtherActor
    (:then
      (Variables|Default|SetTarget 0.0)
      (Development|PrintString "Inside"))
    (:CastFailed
      (Development|PrintString (Utilities|GetDisplayName OtherActor)))))

(event OnComponentEndOverlap(Capsule)
  (params (OverlappedComponent :type Primitive%20Component%20Object%20Reference) (OtherActor :type Actor%20Object%20Reference) (OtherComp :type Primitive%20Component%20Object%20Reference) (OtherBodyIndex :type Integer))
  (Utilities|Casting|CastToPawn OtherActor)
  (Variables|Default|SetTarget 1.0)
  (Development|PrintString "Outside"))

(event EventTick
  (params (DeltaSeconds :type Float%20%28single-precision%29))
  (bind _skylight (Variables|Default|GetSkyLight))
  (bind _output_get (Variables|Default|SetCurrentProgress (Math|Float|Clamp(Float) (+ (* DeltaSeconds (Variables|Default|GetLerpSpeed) (select (== (Variables|Default|GetTarget) 0.0) 1.0 -1.0)) (Variables|Default|GetCurrentProgress)))))
  (Rendering|Components|Light|SetIntensity (Variables|/Script/Engine.SkyLight|GetLightComponent _skylight) (Math|Float|Lerp (Variables|Default|GetOutsideIntensity) (Variables|Default|GetInsideIntensity) _output_get))
  (Rendering|Components|Light|SetLightColor (Variables|/Script/Engine.SkyLight|GetLightComponent _skylight) (Math|Color|Lerp(LinearColor) (Variables|Default|GetOutsideColor) (Variables|Default|GetInsideColor) _output_get)))

(fn ConstructionScript)