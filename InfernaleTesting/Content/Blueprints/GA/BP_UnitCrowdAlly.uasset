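; Allied crowd unit actor that travels along the spline of a referenced ally spline actor and destroys itself at the end.
; On BeginPlay it shifts its Torch component by a random local X/Y offset, so units spread around the path.
; Tick calls MoveCrowd, whose timeline, rate-scaled by TimeToComplete, sets world location and local-space spline rotation plus a fixed 90-degree correction by distance along the spline.
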(event Custom|Move%20Crowd
  (bind _splineally_ref (Variables|Default|GetSplineAlly%20REF))
  (bind _spline (Variables|/Game/Blueprints/GA/BP_CrowdSplineAlly.BP_CrowdSplineAlly_C|GetSpline _splineally_ref))
  (Components|Timeline|SetPlayRate (Variables|Default|GetMoveCrowd) (/ 1.0 (Variables|Default|GetTime%20To%20Complete)))
  (bind _movetrack (Timeline|MoveCrowd Play)
    (:Update
      (Transformation|SetActorTransform (Math|Transform|MakeTransform (Spline|GetLocationatDistanceAlongSpline _spline (Math|Float|Lerp 0.0 (Spline|GetSplineLength (Variables|/Game/Blueprints/GA/BP_CrowdSplineAlly.BP_CrowdSplineAlly_C|GetSpline (Variables|Default|GetSplineAlly%20REF))) _movetrack) "World") (Math|Rotator|CombineRotators (Spline|GetRotationatDistanceAlongSpline _spline (Math|Float|Lerp 0.0 (Spline|GetSplineLength (Variables|/Game/Blueprints/GA/BP_CrowdSplineAlly.BP_CrowdSplineAlly_C|GetSpline (Variables|Default|GetSplineAlly%20REF))) _movetrack) "Local") "0.000000,-90.000000,0.000000") "1.000000,1.000000,1.000000"))
      (if (== _movetrack 1.0)
        (Actor|DestroyActor)))))

(event EventBeginPlay
  (Transformation|AddLocalOffset (Variables|Default|GetTorch) (Math|Vector|MakeVector (Math|Random|RandomFloatinRange -6e+02 6e+02) (Math|Random|RandomFloatinRange -1e+03 1e+03) 0.0) false false)
  (Class|NiagaraComponent|SetTickBehavior (Variables|Default|GetTorch) "ForceTickLast"))

(event EventTick
  (params (DeltaSeconds :type Float%20%28single-precision%29))
  (CallFunction|MoveCrowd))

(fn ConstructionScript)