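; Lava river actor that builds a deformed mesh flow along an editable spline.
; The construction script adds a spline mesh per segment, matching point tangents and scales, with a dynamic MI_LavaRiver_01 instance tinted by Color.
; BeginPlay starts a randomized looping timer on SpawnNiagaraOnSpline, but that event is empty.
; The Niagara bubble spawn at random offsets along the spline and the material Speed setter are both disconnected.
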(event Custom|SpawnNiagaraOnSpline)

(event EventBeginPlay
  (Utilities|Time|SetTimerbyFunctionName 0 "SpawnNiagaraOnSpline" (Math|Random|RandomFloatinRange 2.0 5.0) true))

(fn ConstructionScript
  (bind _lavaspline (Variables|Default|GetLavaSpline))
  (bind _lavaspline_2 (Variables|Default|GetLavaSpline))
  (bind _lavaspline_3 (Variables|Default|GetLavaSpline))
  (bind _returnvalue (Spline|GetTransformatSplinePoint _lavaspline_3 0 "Local" false))
  (bind (_x _y _z) (Math|Vector|BreakVector (.location _returnvalue)))
  (for _index (range 0 (- (Spline|GetNumberOfSplinePoints (Variables|Default|GetLavaSpline)) 2))
    (bind _returnvalue_2 (AddComponent|AddSplineMeshComponent false (Math|Transform|MakeTransform (Math|Vector|MakeVector _x _y (- _z 0.0)) "0, 0, 0" "1.000000,1.000000,1.000000")))
    (bind _returnvalue_3 (Rendering|Material|CreateDynamicMaterialInstance _returnvalue_2 0 "/Game/Effects/Environement/Lava/MI_LavaRiver_01.MI_LavaRiver_01" "None" :!class /Script/Engine.PrimitiveComponent))
    (Rendering|Material|SetVectorParameterValue _returnvalue_3 "Color" (Variables|Default|GetColor) :!class /Script/Engine.MaterialInstanceDynamic)
    (SplineMesh|SetForwardAxis _returnvalue_2 "X" true)
    (SplineMesh|SetStartScale _returnvalue_2 (Math|Conversions|ToVector2D(Vector) (Spline|GetScaleatSplinePoint _lavaspline_2 _index)) true :!class /Script/Engine.SplineMeshComponent)
    (SplineMesh|SetEndScale _returnvalue_2 (Math|Conversions|ToVector2D(Vector) (Spline|GetScaleatSplinePoint _lavaspline_2 (+ _index 1))) true :!class /Script/Engine.SplineMeshComponent)
    (SplineMesh|SetStartandEnd _returnvalue_2 (Spline|GetLocationatSplinePoint _lavaspline _index "Local") (Spline|GetTangentatSplinePoint _lavaspline _index "Local") (Spline|GetLocationatSplinePoint _lavaspline (+ _index 1) "Local") (Spline|GetTangentatSplinePoint _lavaspline (+ _index 1) "Local") true :!class /Script/Engine.SplineMeshComponent)))