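; BP_SplineBuilding is a construction-script tool for procedural buildings along a spline, with no active runtime logic.
; It derives wall and floor dimensions from bottom, middle, top and unique mesh bounds, scaled by UniformScale and WallHeight.
; It applies the closed-loop setting, then adds spline mesh components in a loop counted by spline length over bottom mesh Y size.
; The script shows no mesh assignment or placement for those components.
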(event EventBeginPlay)

(event Collision|EventActorBeginOverlap
  (params (OtherActor :type Actor%20Object%20Reference)))

(event EventTick
  (params (DeltaSeconds :type Float%20%28single-precision%29)))

(fn ConstructionScript
  (bind _bottommesh (Variables|Param|GetBottomMesh))
  (bind _uniformscale (Variables|Param|GetUniformScale))
  (bind _middlemesh (Variables|Param|GetMiddleMesh))
  (bind _returnvalue (StaticMesh|GetBounds _middlemesh))
  (bind _returnvalue_2 (StaticMesh|GetBounds _bottommesh))
  (bind _returnvalue_3 (* (.boxextent _returnvalue) 2.0 _uniformscale))
  (bind _returnvalue_4 (* (.boxextent _returnvalue_2) 2.0 _uniformscale))
  (bind (_x _y _z) (Math|Vector|BreakVector _returnvalue_3))
  (bind (_x_2 _y_2 _z_2) (Math|Vector|BreakVector _returnvalue_4))
  (Spline|SetClosedLoop (Variables|Default|GetSpline) (Variables|Param|GetCurveClosed) true)
  (Variables|Default|SetBottomMeshYLenght _y_2)
  (bind _output_get (Variables|Default|SetBottomMeshZSize _z_2))
  (bind _output_get_2 (Variables|Default|SetMiddleMeshZSize _z))
  (Variables|Default|SetWallThickness _y)
  (Variables|Default|SetWallSize _x)
  (Variables|Default|SetTopWallOffset (* (Variables|Default|GetMiddleMeshZSize) (Variables|Param|GetWallHeight)))
  (bind _output_get_3 (Variables|Default|SetTopMeshSize (* (.Z (Math|Vector|BreakVector (.boxextent (StaticMesh|GetBounds (Variables|Param|GetTopMesh))))) 2.0 _uniformscale)))
  (Variables|Default|SetFloorHeight (+ (+ (* _output_get_2 (Variables|Param|GetWallHeight)) _output_get) _output_get_3))
  (Variables|Default|SetUniqqueFloorHeight (* (.Z (Math|Vector|BreakVector (.boxextent (StaticMesh|GetBounds (Variables|Param|GetUniqueWall))))) 2.0 _uniformscale))
  (for _index (range 0 (Math|Float|Truncate (/ (Spline|GetSplineLength (Variables|Default|GetSpline)) (Variables|Default|GetBottomMeshYLenght))))
    (AddComponent|AddSplineMeshComponent false)))